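; BP_CaroLalz is an actor Blueprint with helper functions that appear to support movement relative to a flying player.
; GenerateRandomOffset builds a vector within RandomOffsetMinMax, symmetric on X and Z, while Y always equals its maximum because both bounds match.
; GetLR reports whether the actor is closer to the Right point than the Left.
; FlyingPlayerQuery returns only zeroed rotation, side points and speed, and no graph calls these functions.
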(fn `FlyingPlayerQuery`
  (returns (Rot :type "Rotator Structure") (Left :type "Vector Structure") (Right :type "Vector Structure") (Speed :type "Float (double-precision)"))
  (return (struct) (0.0 0.0 0.0) (0.0 0.0 0.0) 0.0))

(fn `GenerateRandomOffset`
  (returns (`New Offset` :type "Vector Structure"))
  (bind (_randomoffsetminmax_x _randomoffsetminmax_y _randomoffsetminmax_z) (`KismetMathLibrary.BreakVector` (`self.RandomOffsetMinMax`)))
  (return (`KismetMathLibrary.MakeVector` (`KismetMathLibrary.RandomFloatInRange` (* -1 _randomoffsetminmax_x) _randomoffsetminmax_x) (`KismetMathLibrary.RandomFloatInRange` (* 1 _randomoffsetminmax_y) _randomoffsetminmax_y) (`KismetMathLibrary.RandomFloatInRange` (* -1 _randomoffsetminmax_z) _randomoffsetminmax_z))))

(fn `GetLR`
  (params (Left :type "Vector Structure") (Right :type "Vector Structure"))
  (returns (`GoRight?` :type Boolean))
  (bind _returnvalue (`self.K2_GetActorLocation`))
  (return (> (`KismetMathLibrary.VSize` (- _returnvalue Left)) (`KismetMathLibrary.VSize` (- _returnvalue Right)))))

(fn `UserConstructionScript`)