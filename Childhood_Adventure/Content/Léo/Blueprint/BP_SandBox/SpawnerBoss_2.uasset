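; SpawnerBoss_2 is a spawner actor that creates the second-phase boss when its SpawnBoss event is called.
; A DoOnce gate limits it to one spawn of Boss_Phase_2_BP, placed at the Spawner component's location with the Arrow's rotation.
; The Boss2 variable is set to None afterwards rather than to the spawned actor.
; The Box end-overlap event is empty; logic to destroy Boss2 for a PlayerCapsule-tagged component is disconnected.
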(event `SpawnBoss`
  (`/Engine/EditorBlueprintResources/StandardMacros.DoOnce` false
    (:`Completed`
      (`|SpawnActorFromClass` "/Game/Léo/Blueprint/Boss_Phase_2/BP/Boss_Phase_2_BP.Boss_Phase_2_BP_C" (`KismetMathLibrary.MakeTransform` (`SceneComponent.K2_GetComponentLocation` (`self.Spawner`)) (`SceneComponent.K2_GetComponentRotation` (`self.Arrow`))) "Undefined" "OverrideRootScale" null null)
      (set `self.Boss 2` null))))

(event `self.Box.OnComponentEndOverlap`
  (params (OverlappedComponent :type "PrimitiveComponent Object Reference") (OtherActor :type "Actor Object Reference") (OtherComp :type "PrimitiveComponent Object Reference") (OtherBodyIndex :type Integer)))

(fn `UserConstructionScript`)