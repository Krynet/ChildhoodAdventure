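; Phase 1 boss actor that adapts to the damage types the player uses and activates the ground destroyer on death.
; Per-type hit counters escalate defenses in two tiers: larger homing volleys, more eye-bomber directions, or shockwaves and armor that divides punch damage.
; Events spawn its attacks, including lasers, chained observers and an ultimate.
; The Capacity_Selected blackboard flag blocks shockwaves, flagging NeedDefense when a punch threshold is reached.
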(event `LD_Deal_Damage`
  ;[1 1 1 0.269] Deal Damage & Update Boss Resistance
  (bind _output_get (set `self.BossLife` (- (`self.BossLife`) (`self.LD_Deal_Damage_Value`))))
  (`KismetSystemLibrary.PrintString` (`KismetStringLibrary.Conv_DoubleToString` _output_get)))

(event `Deal_Projectile_Damage`
  ;[1 1 1 0.269] Deal Damage & Update Boss Resistance
  ;;[1 1 1] Deal Homing Projectile Damage & Update Number Of Homing Projectile
  (`KismetSystemLibrary.PrintString` "Le boss prend 1 Degat via projectile")
  (if (`self.Defend_Projectile_1`)
    (if (`self.Defend_Projectile_2`)
      (set `self.BossLife` (- (`self.BossLife`) (`self.Projectile_Damage_Value`)))
      (`self.Boss_Life`)
      (else
        (bind _result (`/Engine/EditorBlueprintResources/StandardMacros.IncrementInt` (`self.Defend_Projectile_Count`))
          (:`  `
            (if (>= _result (`self.Defend_Projectile_Phase_2`))
              (`KismetSystemLibrary.PrintString` "Le boss prend 1 Degat via projectile")
              (set `self.Defend_Projectile_2` true)
              (set `self.Homing_Projectile_Max` 12))
            (set `self.BossLife` (- (`self.BossLife`) (`self.Projectile_Damage_Value`)))
            (`self.Boss_Life`)))))
    (else
      (bind _result_2 (`/Engine/EditorBlueprintResources/StandardMacros.IncrementInt` (`self.Defend_Projectile_Count`))
        (:`  `
          (if (>= _result_2 (`self.Defend_Projectile_Phase_1`))
            (`KismetSystemLibrary.PrintString` "Projectile Phase 1")
            (set `self.Defend_Projectile_1` true)
            (set `self.Homing_Projectile_Max` 8))
          (set `self.BossLife` (- (`self.BossLife`) (`self.Projectile_Damage_Value`)))
          (`self.Boss_Life`))))))

(event `self.ReceiveBeginPlay`
  ;[1 1 1] Init List
  (bind _returnvalue (`GameplayStatics.GetActorOfClass` "/Game/ThirdPersonBP/Blueprints/ThirdPersonCharacter.ThirdPersonCharacter_C"))
  (set `self.Player` _returnvalue)
  (set `self.Eyes_Bomber_Direction_2` (`|MakeArray` (`SceneComponent.K2_GetComponentRotation` (`self.Eyes_Bomber_Spawn_Direction_4`)) (`SceneComponent.K2_GetComponentRotation` (`self.Eyes_Bomber_Spawn_Direction_1`))))
  (set `self.Eyes_Bomber_Direction_4` (`|MakeArray` (`SceneComponent.K2_GetComponentRotation` (`self.Eyes_Bomber_Spawn_Direction_2`)) (`SceneComponent.K2_GetComponentRotation` (`self.Eyes_Bomber_Spawn_Direction_3`)) (`SceneComponent.K2_GetComponentRotation` (`self.Eyes_Bomber_Spawn_Direction_4`)) (`SceneComponent.K2_GetComponentRotation` (`self.Eyes_Bomber_Spawn_Direction_1`))))
  (set `self.Eyes_Bomber_Direction_8` (`|MakeArray` (`SceneComponent.K2_GetComponentRotation` (`self.Eyes_Bomber_Spawn_Direction_2`)) (`SceneComponent.K2_GetComponentRotation` (`self.Eyes_Bomber_Spawn_Direction_3`)) (`SceneComponent.K2_GetComponentRotation` (`self.Eyes_Bomber_Spawn_Direction_4`)) (`SceneComponent.K2_GetComponentRotation` (`self.Eyes_Bomber_Spawn_Direction_1`)) (`SceneComponent.K2_GetComponentRotation` (`self.Eyes_Bomber_Spawn_Direction_5`)) (`SceneComponent.K2_GetComponentRotation` (`self.Eyes_Bomber_Spawn_Direction_6`)) (`SceneComponent.K2_GetComponentRotation` (`self.Eyes_Bomber_Spawn_Direction_7`)) (`SceneComponent.K2_GetComponentRotation` (`self.Eyes_Bomber_Spawn_Direction_8`))))
  (set `self.Homing_Missile_Direction` (`|MakeArray` (`SceneComponent.K2_GetComponentRotation` (`self.Homing_Projectiles_Spawn_Direction_1`)) (`SceneComponent.K2_GetComponentRotation` (`self.Homing_Projectiles_Spawn_Direction_2`)) (`SceneComponent.K2_GetComponentRotation` (`self.Homing_Projectiles_Spawn_Direction_3`)))))

(event `Deal_Damage_Eyes_Bomber`
  ;[1 1 1 0.269] Deal Damage & Update Boss Resistance
  ;;[1 1 1] Deal Eyes Bomber Damage & Update Eyes Bomber List
  (`KismetSystemLibrary.PrintString` "Le boss prend 1 Degat via EyesBomber")
  (if (`self.Defend_Eyes_1`)
    (if (`self.Defend_Eyes_2`)
      (set `self.BossLife` (- (`self.BossLife`) (`self.Eyes_Damage_Value`)))
      (`self.Boss_Life`)
      (else
        (bind _result (`/Engine/EditorBlueprintResources/StandardMacros.IncrementInt` (`self.Defend_Eyes_Count`))
          (:`  `
            (if (>= _result (`self.Defend_Eyes_Phase_2`))
              (`KismetSystemLibrary.PrintString` "EyesBomber Phase 2")
              (set `self.Defend_Eyes_2` true))
            (set `self.BossLife` (- (`self.BossLife`) (`self.Eyes_Damage_Value`)))
            (`self.Boss_Life`)))))
    (else
      (bind _result_2 (`/Engine/EditorBlueprintResources/StandardMacros.IncrementInt` (`self.Defend_Eyes_Count`))
        (:`  `
          (if (>= _result_2 (`self.Defend_Eyes_Phase_1`))
            (`KismetSystemLibrary.PrintString` "EyesBomber Phase 1")
            (set `self.Defend_Eyes_1` true))
          (set `self.BossLife` (- (`self.BossLife`) (`self.Eyes_Damage_Value`)))
          (`self.Boss_Life`))))))

(event `Deal_Damage_CaC`
  (bind _punch_damage_value (`self.Punch_Damage_Value`))
  ;[1 1 1 0.269] Deal Damage & Update Boss Resistance
  ;;[1 1 1] Deal CaC Damage & Update Boss Armor
  (if (`self.Defend_Punch_1`)
    (if (`self.Defend_Punch_2`)
      (bind _output_get (set `self.Armor` 10.0))
      (bind _returnvalue (/ (`self.Punch_Damage_Value`) _output_get))
      (set `self.BossLife` (- (`self.BossLife`) _returnvalue))
      (`KismetSystemLibrary.PrintString` "CaC Degat")
      (`KismetSystemLibrary.PrintString` (`KismetStringLibrary.Conv_DoubleToString` _returnvalue))
      (`self.Boss_Life`)
      (else
        (bind _result (`/Engine/EditorBlueprintResources/StandardMacros.IncrementInt` (`self.Defend_Punch_Count`))
          (:`  `
            (if (>= _result (`self.Defend_Punch_Phase_2`))
              (if (`BlackboardComponent.GetValueAsBool` (`AIBlueprintHelperLibrary.GetBlackboard` null) "Capacity_Selected")
                (set `self.Need_Defense` true)
                (else
                  (`/Engine/EditorBlueprintResources/StandardMacros.DoOnce` false
                    (:`Completed`
                      (set `self.Defend_Punch_2` true)
                      (`KismetSystemLibrary.PrintString` "Armor Phase 2")
                      (`self.Launch_Shock_Wave`)
                      (bind _output_get_2 (set `self.Armor` 5.0 :!label _label))
                      (bind _returnvalue_2 (/ (`self.Punch_Damage_Value`) _output_get_2))
                      (set `self.BossLife` (- (`self.BossLife`) _returnvalue_2))
                      (`KismetSystemLibrary.PrintString` "CaC Degat")
                      (`KismetSystemLibrary.PrintString` (`KismetStringLibrary.Conv_DoubleToString` _returnvalue_2))
                      (`self.Boss_Life`)))))
              (else
                (goto _label)))))))
    (else
      (bind _result_2 (`/Engine/EditorBlueprintResources/StandardMacros.IncrementInt` (`self.Defend_Punch_Count`))
        (:`  `
          (if (>= _result_2 (`self.Defend_Punch_Phase_1`))
            (if (`BlackboardComponent.GetValueAsBool` (`AIBlueprintHelperLibrary.GetBlackboard` null) "Capacity_Selected")
              (set `self.Need_Defense` true)
              (else
                (`/Engine/EditorBlueprintResources/StandardMacros.DoOnce` false
                  (:`Completed`
                    (set `self.Defend_Punch_1` true)
                    (`KismetSystemLibrary.PrintString` "Armor Phase 1")
                    (`self.Launch_Shock_Wave`)
                    (set `self.Armor` 0.0 :!label _label_2)
                    (set `self.BossLife` (- (`self.BossLife`) _punch_damage_value))
                    (`KismetSystemLibrary.PrintString` "CaC Degat")
                    (`KismetSystemLibrary.PrintString` (`KismetStringLibrary.Conv_DoubleToString` _punch_damage_value))
                    (`self.Boss_Life`)))))
            (else
              (goto _label_2))))))))

(event `Launch_Eyes_Bomber`
  ;[1 1 1] Launch Eyes Event
  (if (`self.Defend_Eyes_1`)
    (if (`self.Defend_Eyes_2`)
      (`self.LaunchEyes_8`)
      (else
        (`self.LaunchEyes_4`)))
    (else
      (`self.LaunchEyes_2`))))

(event `Fire_homing_projectiles`
  ;[1 1 1] Homing Projectiles Event
  (`self.Launch_Homing_Projectile`
    (:`Repeat`
      (`KismetSystemLibrary.Delay` 0.2)
      (`self.Fire_homing_projectiles`))
    (:`End`
      (set `self.Homing_Projectile_Count` 0))))

(event `Launch_Shock_Wave`
  ;[1 1 1] Shock Wave Event
  (if (not (`BlackboardComponent.GetValueAsBool` (`AIBlueprintHelperLibrary.GetBlackboard` null) "Capacity_Selected"))
    (set `self.Is_In_Defense` true)
    (`|SpawnActorFromClass` "/Game/Léo/Blueprint/ShockWave/ShockWave_BP.ShockWave_BP_C" (`KismetMathLibrary.MakeTransform` (`SceneComponent.K2_GetComponentLocation` (`self.Shock_Wave_Spawn`))) "Undefined" "OverrideRootScale" null null)
    (`KismetSystemLibrary.Delay` 6.0)
    (set `self.Is_In_Defense` false)
    (set `self.Need_Defense` false)))

(event `Laser_Circle`
  ;[1 1 1] Laser Circle Event
  (`|SpawnActorFromClass` "/Game/Léo/Blueprint/LaserCircle/LaserCircle.LaserCircle_C" (`KismetMathLibrary.MakeTransform` (- (`self.K2_GetActorLocation`) (0.0 0.0 100.0))) "Undefined" "OverrideRootScale" null null))

(event `self.BossTarget.OnComponentBeginOverlap`
  (params (OverlappedComponent :type "PrimitiveComponent Object Reference") (OtherActor :type "Actor Object Reference") (OtherComp :type "PrimitiveComponent Object Reference") (OtherBodyIndex :type Integer) (bFromSweep :type Boolean) (SweepResult :type "HitResult Structure (by ref)"))
  (if (`ActorComponent.ComponentHasTag` OtherComp "PunchBox")
    (if (`/Game/ThirdPersonBP/Blueprints/ThirdPersonCharacter.Punch` (`self.Player`))
      (`self.Deal_Damage_CaC`))))

(event `Observer_Event`
  ;[1 1 1] Observer Event
  (`|SpawnActorFromClass` "/Game/Léo/Blueprint/Observer/Observer_BP.Observer_BP_C" (`KismetMathLibrary.MakeTransform` (`SceneComponent.K2_GetComponentLocation` (`self.Spawner`)) (`KismetMathLibrary.FindLookAtRotation` (`self.K2_GetActorLocation`) (`self.K2_GetActorLocation` (`self.Player`)))) "Undefined" "OverrideRootScale" null null)
  (`KismetSystemLibrary.Delay` 2.0)
  (if (== (`self.Observer_Count`) (`self.Observer_Count_Max`))
    (set `self.Observer_Count` 0)
    (else
      (`/Engine/EditorBlueprintResources/StandardMacros.IncrementInt` (`self.Observer_Count`)
        (:`  `
          (`self.Observer_Event`))))))

(event `Ulti_Event`
  ;[1 1 1] Ulti Event
  (`|SpawnActorFromClass` "/Game/Léo/Blueprint/Ultim_1/Ultim_1.Ultim_1_C" (`KismetMathLibrary.MakeTransform` (`SceneComponent.K2_GetComponentLocation` (`self.Ulti_Spawner`))) "Undefined" "OverrideRootScale" null null))

(fn `UserConstructionScript`)