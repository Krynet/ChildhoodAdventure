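; Explosion actor for the Phase 1 boss's homing projectiles that briefly damages and pushes on impact.
; On BeginPlay it caches the player's ThirdPersonCharacter, fires a RadialForce impulse, then destroys itself after a short delay.
; During that window, a sphere overlap with a component tagged PlayerCapsule calls ProjectileDamage on the cached character.
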(event `self.ReceiveBeginPlay`
  (bind _asthird_person_character (cast `/Game/ThirdPersonBP/Blueprints/ThirdPersonCharacter` (`GameplayStatics.GetPlayerCharacter` 0)))
  (set `self.Character` _asthird_person_character)
  (`RadialForceComponent.FireImpulse` (`self.RadialForce`))
  (`KismetSystemLibrary.Delay` 0.1)
  (`self.K2_DestroyActor`))

(event `self.Sphere.OnComponentBeginOverlap`
  (params (OverlappedComponent :type "PrimitiveComponent Object Reference") (OtherActor :type "Actor Object Reference") (OtherComp :type "PrimitiveComponent Object Reference") (OtherBodyIndex :type Integer) (bFromSweep :type Boolean) (SweepResult :type "HitResult Structure (by ref)"))
  (if (`ActorComponent.ComponentHasTag` OtherComp "PlayerCapsule")
    (`/Game/ThirdPersonBP/Blueprints/ThirdPersonCharacter.ProjectileDamage` (`self.Character`))))

(fn `UserConstructionScript`)