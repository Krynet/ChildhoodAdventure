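; Phase 2 boss character exposing attacks as events: timeline-driven jump and dash, rotating eye laser, homing projectiles, eye bombers, laser circles and Umbra spawners.
; Damage events lower boss life and count hits toward two-step defense thresholds, which cut punch damage, set NeedDefense or enlarge projectile volleys.
; CapacityDefend chains a shockwave, repeated dashes and jumps.
; Homing damage increments the punch counter, though its thresholds read the projectile counter.
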(event `Deal Damage Homing Projectiles`
  (`/Engine/EditorBlueprintResources/StandardMacros.IncrementInt` (`self.Defend Punch Count`)
    (:`  `
      (if (`self.Defend Projectiles Phase 1`)
        (if (`self.Defend Projectiles Phase 2`)
          (bind _output_get (set `self.Boss_2_Life` (- (`self.Boss_2_Life`) (`self.Homing Projectiles Damage`))))
          (`KismetSystemLibrary.PrintString` (`KismetStringLibrary.Conv_DoubleToString` _output_get))
          (else
            (if (>= (`self.Defend Projectiles Count`) (`self.Defend Projectiles Count Phase 2`))
              (`/Engine/EditorBlueprintResources/StandardMacros.DoOnce` false
                (:`Completed`
                  (set `self.Defend Projectiles Phase 2` true)
                  (set `self.Homing Projectiles Count Max` 20))))
            (bind _output_get_2 (set `self.Boss_2_Life` (- (`self.Boss_2_Life`) (`self.Homing Projectiles Damage`))))
            (`KismetSystemLibrary.PrintString` (`KismetStringLibrary.Conv_DoubleToString` _output_get_2))))
        (else
          (if (>= (`self.Defend Projectiles Count`) (`self.Defend Projectiles Count Phase 1`))
            (`/Engine/EditorBlueprintResources/StandardMacros.DoOnce` false
              (:`Completed`
                (set `self.Defend Projectiles Phase 1` true)
                (set `self.Homing Projectiles Count Max` 15))))
          (bind _output_get_3 (set `self.Boss_2_Life` (- (`self.Boss_2_Life`) (`self.Homing Projectiles Damage`))))
          (`KismetSystemLibrary.PrintString` (`KismetStringLibrary.Conv_DoubleToString` _output_get_3)))))))

(event `self.ReceiveBeginPlay`
  (bind _returnvalue (`GameplayStatics.GetActorOfClass` "/Game/ThirdPersonBP/Blueprints/ThirdPersonCharacter.ThirdPersonCharacter_C"))
  (set `self.Player` _returnvalue)
  (set `self.Homing Spawner Rotation` (`|MakeArray` (`SceneComponent.K2_GetComponentRotation` (`self.Arrow1`)) (`SceneComponent.K2_GetComponentRotation` (`self.Arrow2`)) (`SceneComponent.K2_GetComponentRotation` (`self.Arrow3`)) (`SceneComponent.K2_GetComponentRotation` (`self.Arrow4`)) (`SceneComponent.K2_GetComponentRotation` (`self.Arrow5`))))
  (set `self.Eyes Bomber Spawner Rotation 8` (`|MakeArray` (`SceneComponent.K2_GetComponentRotation` (`self.Eyes_Direction_1`)) (`SceneComponent.K2_GetComponentRotation` (`self.Eyes_Direction_2`)) (`SceneComponent.K2_GetComponentRotation` (`self.Eyes_Direction_3`)) (`SceneComponent.K2_GetComponentRotation` (`self.Eyes_Direction_4`)) (`SceneComponent.K2_GetComponentRotation` (`self.Eyes_Direction_5`)) (`SceneComponent.K2_GetComponentRotation` (`self.Eyes_Direction_6`)) (`SceneComponent.K2_GetComponentRotation` (`self.Eyes_Direction_7`)) (`SceneComponent.K2_GetComponentRotation` (`self.Eyes_Direction_8`))))
  (set `self.Eyes Bomber Spawner Rotation 6` (`|MakeArray` (`SceneComponent.K2_GetComponentRotation` (`self.Eyes_Direction_1`)) (`SceneComponent.K2_GetComponentRotation` (`self.Eyes_Direction_2`)) (`SceneComponent.K2_GetComponentRotation` (`self.Eyes_Direction_3`)) (`SceneComponent.K2_GetComponentRotation` (`self.Eyes_Direction_5`)) (`SceneComponent.K2_GetComponentRotation` (`self.Eyes_Direction_6`)) (`SceneComponent.K2_GetComponentRotation` (`self.Eyes_Direction_8`))))
  (set `self.Eyes Bomber Spawner Rotation 3` (`|MakeArray` (`SceneComponent.K2_GetComponentRotation` (`self.Eyes_Direction_1`)) (`SceneComponent.K2_GetComponentRotation` (`self.Eyes_Direction_3`)) (`SceneComponent.K2_GetComponentRotation` (`self.Eyes_Direction_8`)))))

(event `Deal Damage Eyes Bomber`
  (`/Engine/EditorBlueprintResources/StandardMacros.IncrementInt` (`self.Defend Eyes Count`)
    (:`  `
      (if (`self.Defend Eyes 1`)
        (if (`self.Defend Eyes 2`)
          (bind _output_get (set `self.Boss_2_Life` (- (`self.Boss_2_Life`) (`self.Eyes_Bomber_Damage`))))
          (`KismetSystemLibrary.PrintString` (`KismetStringLibrary.Conv_DoubleToString` _output_get))
          (else
            (if (>= (`self.Defend Eyes Count`) (`self.Defend Eyes Count Phase 2`))
              (`/Engine/EditorBlueprintResources/StandardMacros.DoOnce` false
                (:`Completed`
                  (set `self.Defend Eyes 2` true))))
            (bind _output_get_2 (set `self.Boss_2_Life` (- (`self.Boss_2_Life`) (`self.Eyes_Bomber_Damage`))))
            (`KismetSystemLibrary.PrintString` (`KismetStringLibrary.Conv_DoubleToString` _output_get_2))))
        (else
          (if (>= (`self.Defend Eyes Count`) (`self.Defend Eyes Count Phase 1`))
            (`/Engine/EditorBlueprintResources/StandardMacros.DoOnce` false
              (:`Completed`
                (set `self.Defend Eyes 1` true))))
          (bind _output_get_3 (set `self.Boss_2_Life` (- (`self.Boss_2_Life`) (`self.Eyes_Bomber_Damage`))))
          (`KismetSystemLibrary.PrintString` (`KismetStringLibrary.Conv_DoubleToString` _output_get_3)))))))

(event `self.Boss_2_Target.OnComponentBeginOverlap`
  (params (OverlappedComponent :type "PrimitiveComponent Object Reference") (OtherActor :type "Actor Object Reference") (OtherComp :type "PrimitiveComponent Object Reference") (OtherBodyIndex :type Integer) (bFromSweep :type Boolean) (SweepResult :type "HitResult Structure (by ref)"))
  (if (`ActorComponent.ComponentHasTag` OtherComp "PunchBox")
    (if (`/Game/ThirdPersonBP/Blueprints/ThirdPersonCharacter.Punch` (`self.Player`))
      (`self.Deal Damage CaC`))))

(event `Capacity_Jump`
  ;[1 1 1] Capacity Jump
  (set `self.Player_Location` (`self.K2_GetActorLocation` (`self.Player`)))
  (set `self.Boss_Location` (`self.K2_GetActorLocation`))
  (`TimelineComponent.SetPlayRate` (`self.Jump_Timeline`) (`KismetMathLibrary.FClamp` (* (`self.TimeLine`) (/ (`KismetMathLibrary.VSize` (- (`self.Player_Location`) (`self.Boss_Location`))) 800.0)) 1.5 2.0))
  (bind (_direction _moveup _moveto) (`Timeline|Jump_Timeline` :!via `PlayFromStart`)
    (:`Update`
      (`self.K2_SetActorLocation` (`KismetMathLibrary.MakeVector` (`KismetMathLibrary.Lerp` (.x (`self.Boss_Location`)) (.x (`NavigationSystemV1.K2_GetRandomReachablePointInRadius` (`self.Player_Location`) 100.0 null null)) _moveto) (`KismetMathLibrary.Lerp` (.y (`self.Boss_Location`)) (.y (`NavigationSystemV1.K2_GetRandomReachablePointInRadius` (`self.Player_Location`) 100.0 null null)) _moveto) (`KismetMathLibrary.Lerp` (.z (`self.Boss_Location`)) (`self.Jump_Height`) _moveup))))
    (:`Finished`
      (`self.Spawn_Shock_Wave`))))

(event `Deal Damage CaC`
  (`/Engine/EditorBlueprintResources/StandardMacros.IncrementInt` (`self.Defend Punch Count`)
    (:`  `
      (if (`self.Defend Punch Phase 1`)
        (if (`self.Defend Punch Phase 2`)
          (bind _output_get (set `self.Boss_2_Life` (- (`self.Boss_2_Life`) (/ (`self.Punch Damage`) 4.0))))
          (`KismetSystemLibrary.PrintString` (`KismetStringLibrary.Conv_DoubleToString` _output_get))
          (else
            (if (>= (`self.Defend Punch Count`) (`self.Defend Punch Count Phase 2`))
              (`/Engine/EditorBlueprintResources/StandardMacros.DoOnce` false
                (:`Completed`
                  (set `self.Defend Punch Phase 2` true)
                  (set `self.Need Defense` true))))
            (bind _output_get_2 (set `self.Boss_2_Life` (- (`self.Boss_2_Life`) (/ (`self.Punch Damage`) 2.0))))
            (`KismetSystemLibrary.PrintString` (`KismetStringLibrary.Conv_DoubleToString` _output_get_2))))
        (else
          (if (>= (`self.Defend Punch Count`) (`self.Defend Punch Count Phase 1`))
            (`/Engine/EditorBlueprintResources/StandardMacros.DoOnce` false
              (:`Completed`
                (set `self.Defend Punch Phase 1` true)
                (set `self.Need Defense` true))))
          (bind _output_get_3 (set `self.Boss_2_Life` (- (`self.Boss_2_Life`) (`self.Punch Damage`))))
          (`KismetSystemLibrary.PrintString` (`KismetStringLibrary.Conv_DoubleToString` _output_get_3)))))))

(event `Spawn_Shock_Wave`
  ;[1 1 1] Capacity Jump
  ;;[1 1 1] ShockWave
  (`|SpawnActorFromClass` "/Game/Léo/Blueprint/ShockWave/ShockWave_BP.ShockWave_BP_C" (`KismetMathLibrary.MakeTransform` (`SceneComponent.K2_GetComponentLocation` (`self.ShockWave_Spawner`))) "Undefined" "OverrideRootScale" null null))

(event `Capacity Dash`
  (bind _boss_location (`self.Boss_Location`))
  (bind _boss_location_2 (`self.Boss_Location`))
  (bind (_returnvalue_roll _returnvalue_pitch _returnvalue_yaw) (`KismetMathLibrary.BreakRotator` (`KismetMathLibrary.FindLookAtRotation` (`self.Boss_Location`) (`self.Player_Location`))))
  ;[1 1 1] Capacity Dash
  (set `self.Player_Location` (`self.K2_GetActorLocation` (`self.Player`)))
  (set `self.Boss_Location` (`self.K2_GetActorLocation`))
  (set `self.Boss_Rotation` (`self.K2_GetActorRotation`))
  (`MovementComponent.StopMovementImmediately` (`self.CharacterMovement`))
  (bind (_direction _newtrack_0) (`Timeline|Look Player Timeline` :!via `PlayFromStart`)
    (:`Update`
      (`self.K2_SetActorRotation` (`KismetMathLibrary.MakeRotator` 0.0 0.0 (`KismetMathLibrary.Lerp` (.yaw (`self.Boss_Rotation`)) _returnvalue_yaw _newtrack_0))))
    (:`Finished`
      (bind _outactors (`GameplayStatics.GetAllActorsWithTag` "Ignore For Dash"))
      (bind _outhit (`KismetSystemLibrary.LineTraceSingle` _boss_location (+ _boss_location (* (`self.GetActorForwardVector`) 1000000)) "TraceTypeQuery1" false _outactors))
      (bind (_bblockinghit _binitialoverlap _time _distance _location _impactpoint _normal _impactnormal _physmat _hitactor) (`GameplayStatics.BreakHitResult` _outhit))
      (if (`self.ActorHasTag` _hitactor "Limite")
        (bind _returnvalue (/ (`KismetMathLibrary.VSize` (- _location (`self.Boss_Location`))) 2000.0))
        (`KismetSystemLibrary.PrintString` (`KismetStringLibrary.Conv_DoubleToString` _returnvalue))
        (`TimelineComponent.SetPlayRate` (`self.Dash Timeline`) (`KismetMathLibrary.FClamp` _returnvalue 1.0 2.0))
        (bind (_direction_2 _dash) (`Timeline|Dash Timeline` :!via `PlayFromStart`)
          (:`Update`
            (`self.K2_SetActorLocation` (`KismetMathLibrary.VLerp` _boss_location_2 (`KismetMathLibrary.MakeVector` (.x (/ (* _location 70.0) 100.0)) (.y (/ (* _location 70.0) 100.0)) (.z _boss_location_2)) _dash))))))))

(event `Capacity Big Laser`
  (bind _big_eyes_laser_spawner (`self.Big Eyes Laser Spawner`))
  (bind (_returnvalue_roll _returnvalue_pitch _returnvalue_yaw) (`KismetMathLibrary.BreakRotator` (`KismetMathLibrary.FindLookAtRotation` (`self.Boss_Location`) (`self.Player_Location`))))
  (bind _roll (.roll (`self.Boss_Rotation`)))
  (bind _pitch (.pitch (`self.Boss_Rotation`)))
  (bind _roll_2 (.roll (`self.Boss_Rotation`)))
  (bind _pitch_2 (.pitch (`self.Boss_Rotation`)))
  (bind _yaw (.yaw (`self.Boss_Rotation`)))
  ;[1 1 1] Capacity Big Eyes
  (`MovementComponent.StopMovementImmediately` (`self.CharacterMovement`))
  (set `self.Player_Location` (`self.K2_GetActorLocation` (`self.Player`)))
  (set `self.Boss_Location` (`self.K2_GetActorLocation`))
  (set `self.Boss_Rotation` (`self.K2_GetActorRotation`))
  (bind (_direction _newtrack_0) (`Timeline|Look Player Timeline_2` :!via `PlayFromStart`)
    (:`Update`
      (`SceneComponent.K2_SetWorldRotation` (`self.CapsuleComponent`) (`KismetMathLibrary.RLerp` (`KismetMathLibrary.MakeRotator` _roll _pitch (`KismetMathLibrary.ClampAxis` (.yaw (`self.Boss_Rotation`)))) (`KismetMathLibrary.MakeRotator` _roll _pitch (`KismetMathLibrary.ClampAxis` _returnvalue_yaw)) _newtrack_0 true) false false))
    (:`Finished`
      (set `self.Boss_Rotation` (`self.K2_GetActorRotation`))
      (bind _returnvalue (`|SpawnActorFromClass` "/Game/Léo/Blueprint/LaserBeam/BigLaserEyes.BigLaserEyes_C" (`KismetMathLibrary.MakeTransform` (`SceneComponent.K2_GetComponentLocation` _big_eyes_laser_spawner) (`SceneComponent.K2_GetComponentRotation` (`self.Arrow Rotation`))) "Undefined" "OverrideRootScale" null null))
      (bind _output_get (set `self.Big_Eyes_Laser` _returnvalue))
      (`self.K2_AttachToComponent` _output_get _big_eyes_laser_spawner "None" "KeepWorld" "KeepWorld" "KeepWorld" true)
      (`KismetSystemLibrary.Delay` 5.0)
      (`/Engine/EditorBlueprintResources/StandardMacros.FlipFlop`
        (:`A`
          (set `self.Boss_End_Rotation` (`KismetMathLibrary.MakeRotator` _roll_2 _pitch_2 (- _yaw 359.0)))
          (bind (_direction_2 _360_lerp) (`Timeline|360° boss` :!via `PlayFromStart` :!label _label)
            (:`Update`
              (`self.K2_SetActorRotation` (`KismetMathLibrary.RLerp` (`self.Boss_Rotation`) (`self.Boss_End_Rotation`) _360_lerp)))
            (:`Finished`
              (`/Game/Léo/Blueprint/LaserBeam/BigLaserEyes.DispawnLaser` (`self.Big_Eyes_Laser`))
              (`KismetSystemLibrary.Delay` 1.0)
              (`self.K2_DestroyActor` (`self.Big_Eyes_Laser`)))))
        (:`B`
          (set `self.Boss_End_Rotation` (`KismetMathLibrary.MakeRotator` _roll_2 _pitch_2 (+ _yaw 359.0)))
          (goto _label :!via `PlayFromStart`))))))

(event `Capacity_Homing_Projectiles`
  ;[1 1 1] Capacity Homing Projectiles
  (`self.Launch_Homing_Projectile`
    (:`Repeat`
      (`KismetSystemLibrary.Delay` 0.2)
      (`self.Capacity_Homing_Projectiles`))
    (:`End`
      (set `self.Homing Projectiles Count` 0))))

(event `Capacity_Eyes_Bomber`
  ;[1 1 1] Capacity Eyes Bomber
  (if (`self.Defend Eyes 1`)
    (if (`self.Defend Eyes 2`)
      (`self.LaunchEyes_8`)
      (else
        (`self.LaunchEyes_6`)))
    (else
      (`self.LaunchEyes_3`))))

(event `Capacity Laser Circle`
  ;[1 1 1] Capacity Laser Circle
  (`|ExecutionSequence`
    (:`then_0`
      (`|SpawnActorFromClass` "/Game/Léo/Blueprint/LaserCircle/LaserCircle.LaserCircle_C" (`KismetMathLibrary.MakeTransform` (`SceneComponent.K2_GetComponentLocation` (`self.Laser Circle Spawn`))) "Undefined" "OverrideRootScale" null null))
    (:`then_1`
      (`|SpawnActorFromClass` "/Game/Léo/Blueprint/LaserCircle/LaserCircle_Vertical.LaserCircle_Vertical_C" (`KismetMathLibrary.MakeTransform` (`SceneComponent.K2_GetComponentLocation` (`self.Laser Circle Vertical Spawn`))) "Undefined" "OverrideRootScale" null null))))

(event `Capacity_Umbra`
  (set `self.Locations_1` (`|MakeArray` (`self.Target_1_Projectil_1`) (`self.Target_2_Projectil_1`) (`self.Target_3_Projectil_1`)))
  (set `self.Locations_2` (`|MakeArray` (`self.Target_1_Projectil_2`) (`self.Target_2_Projectil_2`) (`self.Target_3_Projectil_2`)))
  (set `self.Locations_3` (`|MakeArray` (`self.Target_1_Projectil_3`) (`self.Target_2_Projectil_3`) (`self.Target_3_Projectil_3`)))
  (set `self.Locations_4` (`|MakeArray` (`self.Target_1_Projectil_4`) (`self.Target_2_Projectil_4`) (`self.Target_3_Projectil_4`)))
  (set `self.Umbra_Projectiles_Rotation` (`|MakeArray` (`SceneComponent.K2_GetComponentRotation` (`self.Projectiles_Umbra_Direction_1`)) (`SceneComponent.K2_GetComponentRotation` (`self.Projectiles_Umbra_Direction_2`)) (`SceneComponent.K2_GetComponentRotation` (`self.Projectiles_Umbra_Direction_3`)) (`SceneComponent.K2_GetComponentRotation` (`self.Projectiles_Umbra_Direction_4`))))
  (set `self.Umbra_Projectiles_Location` (`|MakeArray` (`SceneComponent.K2_GetComponentLocation` (`self.Projectiles_Umbra_Direction_1`)) (`SceneComponent.K2_GetComponentLocation` (`self.Projectiles_Umbra_Direction_2`)) (`SceneComponent.K2_GetComponentLocation` (`self.Projectiles_Umbra_Direction_3`)) (`SceneComponent.K2_GetComponentLocation` (`self.Projectiles_Umbra_Direction_4`))))
  (bind _output_get (set `self.Projectile_Umbre_Spawner` (`|MakeArray` (`self.Projectiles_Umbra_Spawner_1`) (`self.Projectiles_Umbra_Spawner_2`) (`self.Projectiles_Umbra_Spawner_3`) (`self.Projectiles_Umbra_Spawner_4`))))
  (for (_ _array_index) _output_get
    (bind _returnvalue (`|SpawnActorFromClass` "/Game/Léo/Blueprint/Umbra_Boss_2/Umbra_Projectil_Spawner.Umbra_Projectil_Spawner_C" (`KismetMathLibrary.MakeTransform` (`|GetArrayItem` (`self.Umbra_Projectiles_Location`) _array_index) (`|GetArrayItem` (`self.Umbra_Projectiles_Rotation`) _array_index)) "Undefined" "OverrideRootScale" null null))
    (if (== _array_index 0)
      (set `/Game/Léo/Blueprint/Umbra_Boss_2/Umbra_Projectil_Spawner.Spawner_Component` (`self.Locations_1`) _returnvalue)
      (elif (== _array_index 1)
        (set `/Game/Léo/Blueprint/Umbra_Boss_2/Umbra_Projectil_Spawner.Spawner_Component` (`self.Locations_2`) _returnvalue)
        (elif (== _array_index 2)
          (set `/Game/Léo/Blueprint/Umbra_Boss_2/Umbra_Projectil_Spawner.Spawner_Component` (`self.Locations_3`) _returnvalue)
          (elif (== _array_index 3)
            (set `/Game/Léo/Blueprint/Umbra_Boss_2/Umbra_Projectil_Spawner.Spawner_Component` (`self.Locations_4`) _returnvalue)))))))

(event `Capacity Defend`
  (`|SpawnActorFromClass` "/Game/Léo/Blueprint/ShockWave/ShockWave_BP.ShockWave_BP_C" (`KismetMathLibrary.MakeTransform` (`SceneComponent.K2_GetComponentLocation` (`self.ShockWave_Spawner`))) "Undefined" "OverrideRootScale" null null)
  (`KismetSystemLibrary.Delay` 2.0)
  (`self.Capacity Dash` :!label _label_2)
  (`KismetSystemLibrary.Delay` 3.0)
  (bind _result (`/Engine/EditorBlueprintResources/StandardMacros.IncrementInt` (`self.Count Defend Capacity`))
    (:`  `
      (if (>= _result 3)
        (set `self.Count Defend Capacity` 0)
        (`self.Capacity_Jump` :!label _label_3)
        (`KismetSystemLibrary.Delay` 3.0)
        (bind _result_2 (`/Engine/EditorBlueprintResources/StandardMacros.IncrementInt` (`self.Count Defend Capacity`))
          (:`  `
            (if (>= _result_2 3)
              (set `self.Count Defend Capacity` 0)
              (else
                (goto _label_3)))))
        (else
          (goto _label_2))))))

(event `Capacity Ultim`)

(fn `UserConstructionScript`)