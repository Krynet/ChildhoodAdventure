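; Caro is a flying AI companion that follows the player, fires projectiles and can respawn at the player's right side.
; On BeginPlay it registers with the player and starts looping timers for random offsets and movement updates.
; Each update queries the player, interpolates rotation, and steers floating-pawn velocity toward the nearer left or right point plus offset, scaling with player speed.
; Fire spawns a ProjectileCaro and passes it the target.
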(event `Follower`
  (`CharacterMovementComponent.SetMovementMode` (`self.CharacterMovement`) "MOVE_Flying" 0 :!label _label)
  (bind _output_get (set `self.Player` (`GameplayStatics.GetPlayerCharacter` 0)))
  (`/Engine/EditorBlueprintResources/StandardMacros.IsValid` _output_get
    (:`Is Valid`
      (message `/Game/Léo/Blueprint/Caro/Interface/BPI_FollowerTalk.AddFollower` _output_get self)
      (bind _returnvalue (`KismetSystemLibrary.K2_SetTimerDelegate` (delegate `Generate Random Offset Tick`) (`self.Random Offset Tick`) true))
      (set `self.Random Offset Timer` _returnvalue)
      (bind _returnvalue_2 (`KismetSystemLibrary.K2_SetTimerDelegate` (delegate `VelocityUpdateTick`) (`self.VelocityUpdateTickrate`) true))
      (set `self.Velocity Update Timer` _returnvalue_2))))

(event `self.ReceiveBeginPlay`
  (goto _label))

(event `/Game/Léo/Blueprint/Caro/Interface/BPI_FollowerTalk.CommandFollower`
  (params (`New Mode` :type "/Game/Léo/Blueprint/Caro/Enums/E_FlyingMode Enum" :default "NewEnumerator0")))

(event `Generate Random Offset Tick`
  (set `self.RandomOffset` (`self.GenerateRandomOffset`)))

(event `VelocityUpdateTick`
  (bind _floatingpawnmovement (`self.FloatingPawnMovement`))
  (bind (_rot _left _right _speed) (message `/Game/Léo/Blueprint/Caro/Interface/BPI_FollowerTalk.FlyingPlayerQuery` (`self.Player`)))
  (if true
    (`|ExecutionSequence`
      (:`then_0`
        (`self.K2_SetActorRotation` (`KismetMathLibrary.RInterpTo` (`self.K2_GetActorRotation`) _rot (`self.VelocityUpdateTickrate`) (`self.RInterp Speed`))))
      (:`then_1`
        (bind _returnvalue (+ (* _speed 0.8) 150.0))
        (set `MovementComponent.Velocity` (`KismetMathLibrary.VInterpTo` (`MovementComponent.Velocity` _floatingpawnmovement) (* (`KismetMathLibrary.Normal` (- (+ (select `bool` (`self.GetLR` _left _right) :`false` _left :`true` _right) (`self.RandomOffset`)) (`self.K2_GetActorLocation`))) (`KismetMathLibrary.SelectFloat` 100.0 _returnvalue (< _returnvalue 200.0))) (`self.VelocityUpdateTickrate`) (`self.Interp Speed`)) _floatingpawnmovement)))))

(event `Fire`
  (params (Location :type "SphereComponent Object Reference"))
  (bind _returnvalue (`|SpawnActorFromClass` "/Game/Léo/Blueprint/Caro/Test/ProjectileCaro.ProjectileCaro_C" (`KismetMathLibrary.MakeTransform` (`SceneComponent.K2_GetComponentLocation` (`self.Sphere2`)) (`SceneComponent.K2_GetComponentRotation` (`self.Arrow1`))) "Undefined" "OverrideRootScale" null null))
  (set `/Game/Léo/Blueprint/Caro/Test/ProjectileCaro.ActorTarget` Location _returnvalue))

(event `Respawn Character`
  (bind _returnvalue (`GameplayStatics.GetActorOfClass` "/Game/ThirdPersonBP/Blueprints/ThirdPersonCharacter.ThirdPersonCharacter_C"))
  (`self.K2_SetActorLocationAndRotation` (`SceneComponent.K2_GetComponentLocation` (`/Game/ThirdPersonBP/Blueprints/ThirdPersonCharacter.RightLocation` _returnvalue)) (`SceneComponent.K2_GetComponentRotation` (`/Game/ThirdPersonBP/Blueprints/ThirdPersonCharacter.Arrow3` _returnvalue))))

(fn `FlyingPlayerQuery`
  (returns (Rot :type "Rotator Structure") (Left :type "Vector Structure") (Right :type "Vector Structure") (Speed :type "Float (double-precision)"))
  (return (struct) (0.0 0.0 0.0) (0.0 0.0 0.0) 0.0))

(fn `GenerateRandomOffset`
  (returns (`New Offset` :type "Vector Structure"))
  (bind (_randomoffsetminmax_x _randomoffsetminmax_y _randomoffsetminmax_z) (`KismetMathLibrary.BreakVector` (`self.RandomOffsetMinMax`)))
  (return (`KismetMathLibrary.MakeVector` (`KismetMathLibrary.RandomFloatInRange` (* -1 _randomoffsetminmax_x) _randomoffsetminmax_x) (`KismetMathLibrary.RandomFloatInRange` (* 1 _randomoffsetminmax_y) _randomoffsetminmax_y) (`KismetMathLibrary.RandomFloatInRange` (* -1 _randomoffsetminmax_z) _randomoffsetminmax_z))))

(fn `GetLR`
  (params (Left :type "Vector Structure") (Right :type "Vector Structure"))
  (returns (`GoRight?` :type Boolean))
  (bind _returnvalue (`self.K2_GetActorLocation`))
  (return (> (`KismetMathLibrary.VSize` (- _returnvalue Left)) (`KismetMathLibrary.VSize` (- _returnvalue Right)))))

(fn `UserConstructionScript`)