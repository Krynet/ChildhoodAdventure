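; Caro is a flying follower pawn that snaps to the player character's CaroTarget on BeginPlay and registers itself as a follower.
; Looping timers, rather than Tick, periodically refresh a random offset and query the player's flight rotation, speed and left/right points.
; While the query is valid, it interpolates rotation to match and steers FloatingPawnMovement velocity toward the nearer side point plus offset, at a speed derived from the player's.
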(event `self.ReceiveBeginPlay`
  (`/Engine/EditorBlueprintResources/StandardMacros.IsValid` null
    (:`Is Valid`
      (`|ExecutionSequence`
        (:`then_0`
          (bind _returnvalue (`GameplayStatics.GetActorOfClass` "/Game/ThirdPersonBP/Blueprints/ThirdPersonCharacter.ThirdPersonCharacter_C"))
          (`/Engine/EditorBlueprintResources/StandardMacros.DoOnce` false
            (:`Completed`
              (`SceneComponent.K2_SetWorldLocation` (`self.DefaultSceneRoot`) (`SceneComponent.K2_GetComponentLocation` (`/Game/ThirdPersonBP/Blueprints/ThirdPersonCharacter.Caro_Target` _returnvalue)) false false))))
        (:`then_1`
          (bind _output_get (set `self.Character` (`GameplayStatics.GetPlayerCharacter` 0)))
          (`/Engine/EditorBlueprintResources/StandardMacros.IsValid` _output_get
            (:`Is Valid`
              (message `/Game/Alexandre/Oracle/Follower.AddFollower` _output_get self)
              (bind _returnvalue_2 (`KismetSystemLibrary.K2_SetTimerDelegate` (delegate `GenerateRandomOffsetTick`) (`self.RandomOffsetTick`) true))
              (set `self.RandomOffsetTimer` _returnvalue_2)
              (bind _returnvalue_3 (`KismetSystemLibrary.K2_SetTimerDelegate` (delegate `VelocityUpdateTick`) (`self.VelocityUpdateTickrate`) true))
              (set `self.VelocityTimer` _returnvalue_3))))))))

(event `GenerateRandomOffsetTick`
  (set `self.RandomOffset` (`self.GenerateRandomOffset`)))

(event `VelocityUpdateTick`
  (bind _floatingpawnmovement (`self.FloatingPawnMovement`))
  (bind (_rot _left _right _speed _query_valid_) (message `/Game/Alexandre/Oracle/Follower.FlyingPlayerQuery` (`self.Character`)))
  (if _query_valid_
    (`|ExecutionSequence`
      (:`then_0`
        (`self.K2_SetActorRotation` (`KismetMathLibrary.RInterpTo` (`self.K2_GetActorRotation`) _rot (`self.VelocityUpdateTickrate`) (`self.RInterp Speed`))))
      (:`then_1`
        (bind _returnvalue (+ (* _speed 0.9) 150.0))
        (set `MovementComponent.Velocity` (`KismetMathLibrary.VInterpTo` (`MovementComponent.Velocity` _floatingpawnmovement) (* (`KismetMathLibrary.Normal` (- (+ (select `bool` (`self.GetLeftRight` _left _right) :`false` _left :`true` _right) (`self.RandomOffset`)) (`self.K2_GetActorLocation`)) 10.0) (`KismetMathLibrary.SelectFloat` 100.0 _returnvalue (< _returnvalue 200.0))) (`self.VelocityUpdateTickrate`) (`self.VInterp Speed`)) _floatingpawnmovement)))))

(fn `GenerateRandomOffset`
  (returns (NewOffset :type "Vector Structure"))
  (bind (_randomoffsetminmax_x _randomoffsetminmax_y _randomoffsetminmax_z) (`KismetMathLibrary.BreakVector` (`self.RandomOffsetMinMax`)))
  (return (`KismetMathLibrary.MakeVector` (`KismetMathLibrary.RandomFloatInRange` (* -1 _randomoffsetminmax_x) _randomoffsetminmax_x) (`KismetMathLibrary.RandomFloatInRange` (* 1 _randomoffsetminmax_y) _randomoffsetminmax_y) (`KismetMathLibrary.RandomFloatInRange` (* -1 _randomoffsetminmax_z) _randomoffsetminmax_z))))

(fn `GetLeftRight`
  (params (Left :type "Vector Structure") (Right :type "Vector Structure"))
  (returns (GoRight :type Boolean))
  (bind _returnvalue (`self.K2_GetActorLocation`))
  (return (> (`KismetMathLibrary.VSize` (- _returnvalue Left)) (`KismetMathLibrary.VSize` (- _returnvalue Right)))))

(fn `UserConstructionScript`)