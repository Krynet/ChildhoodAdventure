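; Eye actor for the phase 2 boss that makes its gaze wander at random while it is not set to look at the player.
; It caches the starting arrow rotation and parent boss, then a timeline eases the arrow to random pitch and yaw within a cone around that rotation.
; After each random pause it picks a new direction, waiting again while the boss is moving; the loop ends once LookAtPlayer is true.
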(event `self.ReceiveBeginPlay`
  (set `self.Init_Rotation` (`SceneComponent.RelativeRotation` (`self.Arrow`)))
  (bind _asboss_phase_2_bp (cast `/Game/Léo/Blueprint/Boss_Phase_2/BP/Boss_Phase_2_BP` (`self.GetParentActor`)))
  (set `self.As Boss Phase 2 BP` _asboss_phase_2_bp)
  (`self.Random Vision`))

(event `Random Vision`
  (bind _pitch (.pitch (`self.Init_Rotation`)))
  (bind _yaw (.yaw (`self.Init_Rotation`)))
  (bind _returnvalue (- _yaw 45.0))
  (bind _returnvalue_2 (- _pitch 45.0))
  (bind _returnvalue_3 (+ _pitch 45.0))
  (bind _returnvalue_4 (+ _yaw 45.0))
  (if (not (`self.LookAtPlayer`))
    (set `self.Actually_Rotation` (`SceneComponent.RelativeRotation` (`self.Arrow`)))
    (set `self.Idle_Rotation` (`KismetMathLibrary.MakeRotator` (.roll (`self.Init_Rotation`)) (`KismetMathLibrary.ClampAngle` (`KismetMathLibrary.RandomFloatInRange` _returnvalue_2 _returnvalue_3) _returnvalue_2 _returnvalue_3) (`KismetMathLibrary.ClampAngle` (`KismetMathLibrary.RandomFloatInRange` _returnvalue _returnvalue_4) _returnvalue _returnvalue_4)))
    (bind (_direction _newtrack_0) (`Timeline|Timeline_1` :!via `PlayFromStart`)
      (:`Update`
        (`SceneComponent.K2_SetRelativeRotation` (`self.Arrow`) (`KismetMathLibrary.RLerp` (`self.Actually_Rotation`) (`self.Idle_Rotation`) _newtrack_0 true) false false))
      (:`Finished`
        (`KismetSystemLibrary.Delay` (`KismetMathLibrary.RandomFloatInRange` 2.0 3.0) :!label _label)
        (if (`/Game/Léo/Blueprint/Boss_Phase_2/BP/Boss_Phase_2_BP.IsMoving` (`self.As Boss Phase 2 BP`))
          (goto _label)
          (else
            (`self.Random Vision`)))))))

(fn `UserConstructionScript`)