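; Boss eye actor that glances around at random and watches the player when their capsule enters its vision cone.
; Idle timeline turns the Arrow toward random angles near its initial rotation, with random pauses between glances.
; Cone overlap eases the Arrow onto the player, then Tick tracks them within clamped pitch and yaw limits.
; Losing the player triggers, once via DoOnce, a delayed return to the initial rotation before idling resumes.
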(event `self.ReceiveBeginPlay`
  (set `self.Init_Rotation` (`SceneComponent.K2_GetComponentRotation` (`self.Arrow`)))
  (`self.Random Vision`))

(event `self.Cone.OnComponentBeginOverlap`
  (params (OverlappedComponent :type "PrimitiveComponent Object Reference") (OtherActor :type "Actor Object Reference") (OtherComp :type "PrimitiveComponent Object Reference") (OtherBodyIndex :type Integer) (bFromSweep :type Boolean) (SweepResult :type "HitResult Structure (by ref)"))
  (bind _arrow (`self.Arrow`))
  (if (`ActorComponent.ComponentHasTag` OtherComp "PlayerCapsule")
    (bind (_direction _newtrack_0) (`Timeline|Timeline_2` :!via `PlayFromStart`)
      (:`Update`
        (`SceneComponent.K2_SetWorldRotation` (`self.Arrow`) (`KismetMathLibrary.RLerp` (`SceneComponent.K2_GetComponentRotation` _arrow) (`KismetMathLibrary.FindLookAtRotation` (`SceneComponent.K2_GetComponentLocation` _arrow) (`self.K2_GetActorLocation` (`GameplayStatics.GetPlayerCharacter` 0))) _newtrack_0) false false))
      (:`Finished`
        (set `self.LookAtPlayer` true)))))

(event `self.Cone.OnComponentEndOverlap`
  (params (OverlappedComponent :type "PrimitiveComponent Object Reference") (OtherActor :type "Actor Object Reference") (OtherComp :type "PrimitiveComponent Object Reference") (OtherBodyIndex :type Integer))
  (if (`ActorComponent.ComponentHasTag` OtherComp "PlayerCapsule")
    (set `self.LookAtPlayer` false)))

(event `self.ReceiveTick`
  (params (DeltaSeconds :type "Float (single-precision)"))
  (bind _pitch (.pitch (`self.Init_Rotation`)))
  (bind _yaw (.yaw (`self.Init_Rotation`)))
  (bind (_returnvalue_roll _returnvalue_pitch _returnvalue_yaw) (`KismetMathLibrary.BreakRotator` (`KismetMathLibrary.FindLookAtRotation` (`SceneComponent.K2_GetComponentLocation` (`self.Arrow`)) (`self.K2_GetActorLocation` (`GameplayStatics.GetPlayerCharacter` 0)))))
  (if (`self.LookAtPlayer`)
    (`|ExecutionSequence`
      (:`then_0`
        (`SceneComponent.K2_SetWorldRotation` (`self.Arrow`) (`KismetMathLibrary.MakeRotator` (.roll (`self.Init_Rotation`)) (`KismetMathLibrary.ClampAngle` _returnvalue_pitch (- _pitch 80.0) (+ _pitch 80.0)) (`KismetMathLibrary.ClampAngle` _returnvalue_yaw (- _yaw 80.0) (+ _yaw 80.0))) false false))
      (:`then_1`
        (goto _label_3 :!via `Reset`))
      (:`then_2`
        (bind (_direction _newtrack_0) (`Timeline|Timeline_0` :!via `Stop` :!label _label)
          (:`Update`
            (`SceneComponent.K2_SetWorldRotation` (`self.Arrow`) (`KismetMathLibrary.RLerp` (`SceneComponent.K2_GetComponentRotation` (`self.Arrow`)) (`self.Init_Rotation`) _newtrack_0 true) false false))
          (:`Finished`
            (`KismetSystemLibrary.Delay` 2.0)
            (`self.Random Vision`))))
      (:`then_3`
        (bind (_direction_2 _newtrack_0_2) (`Timeline|Timeline_1` :!via `Stop` :!label _label_2)
          (:`Update`
            (`SceneComponent.K2_SetWorldRotation` (`self.Arrow`) (`KismetMathLibrary.RLerp` (`self.Actually_Rotation`) (`self.Idle_Rotation`) _newtrack_0_2 true) false false))
          (:`Finished`
            (`KismetSystemLibrary.Delay` (`KismetMathLibrary.RandomFloatInRange` 0.2 1.0))
            (`self.Random Vision`)))))
    (else
      (`/Engine/EditorBlueprintResources/StandardMacros.DoOnce` false :!label _label_3
        (:`Completed`
          (`self.Restore`))))))

(event `Restore`
  (`KismetSystemLibrary.Delay` 3.0)
  (if (not (`self.LookAtPlayer`))
    (goto _label :!via `PlayFromStart`)))

(event `Random Vision`
  (bind _pitch (.pitch (`self.Init_Rotation`)))
  (bind _yaw (.yaw (`self.Init_Rotation`)))
  (bind _returnvalue (- _yaw 45.0))
  (bind _returnvalue_2 (- _pitch 45.0))
  (bind _returnvalue_3 (+ _pitch 45.0))
  (bind _returnvalue_4 (+ _yaw 45.0))
  (if (not (`self.LookAtPlayer`))
    (set `self.Actually_Rotation` (`SceneComponent.K2_GetComponentRotation` (`self.Arrow`)))
    (set `self.Idle_Rotation` (`KismetMathLibrary.MakeRotator` (.roll (`self.Init_Rotation`)) (`KismetMathLibrary.ClampAngle` (`KismetMathLibrary.RandomFloatInRange` _returnvalue_2 _returnvalue_3) _returnvalue_2 _returnvalue_3) (`KismetMathLibrary.ClampAngle` (`KismetMathLibrary.RandomFloatInRange` _returnvalue _returnvalue_4) _returnvalue _returnvalue_4)))
    (goto _label_2 :!via `PlayFromStart`)))

(fn `UserConstructionScript`)