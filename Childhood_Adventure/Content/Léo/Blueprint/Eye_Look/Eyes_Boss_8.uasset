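; Eye Blueprint, named for a boss, that idly glances around by rotating an Arrow component.
; BeginPlay stores the initial rotation, then RandomVision picks a random pitch and yaw within a 45-degree range either side of it.
; A Timeline lerps to that target by the shortest path, waits a random few seconds, then repeats.
; The loop stops when RandomVision finds LookAtPlayer set; this graph contains no player-tracking logic.
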(event `self.ReceiveBeginPlay`
  (set `self.Init_Rotation` (`SceneComponent.RelativeRotation` (`self.Arrow`)))
  (`self.Random Vision`))

(event `Random Vision`
  (bind _pitch (.pitch (`self.Init_Rotation`)))
  (bind _yaw (.yaw (`self.Init_Rotation`)))
  (bind _returnvalue (- _yaw 45.0))
  (bind _returnvalue_2 (- _pitch 45.0))
  (bind _returnvalue_3 (+ _pitch 45.0))
  (bind _returnvalue_4 (+ _yaw 45.0))
  (if (not (`self.LookAtPlayer`))
    (set `self.Actually_Rotation` (`SceneComponent.RelativeRotation` (`self.Arrow`)))
    (set `self.Idle_Rotation` (`KismetMathLibrary.MakeRotator` (.roll (`self.Init_Rotation`)) (`KismetMathLibrary.ClampAngle` (`KismetMathLibrary.RandomFloatInRange` _returnvalue_2 _returnvalue_3) _returnvalue_2 _returnvalue_3) (`KismetMathLibrary.ClampAngle` (`KismetMathLibrary.RandomFloatInRange` _returnvalue _returnvalue_4) _returnvalue _returnvalue_4)))
    (bind (_direction _newtrack_0) (`Timeline|Timeline_0` :!via `PlayFromStart`)
      (:`Update`
        (`SceneComponent.K2_SetRelativeRotation` (`self.Arrow`) (`KismetMathLibrary.RLerp` (`self.Actually_Rotation`) (`self.Idle_Rotation`) _newtrack_0 true) false false))
      (:`Finished`
        (`KismetSystemLibrary.Delay` (`KismetMathLibrary.RandomFloatInRange` 2.0 3.0))
        (`self.Random Vision`)))))

(fn `UserConstructionScript`)