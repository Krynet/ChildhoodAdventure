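; Bomber projectile Blueprint that turns into an Eyes_Bomber_Mob_BP enemy when it touches the floor.
; It plays a sound at its sphere's location on spawn.
; When the sphere overlaps an actor or component tagged "Floor", it hides itself, spawns the mob at its own location and destroys itself after a short delay.
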(event `self.ReceiveBeginPlay`
  (`GameplayStatics.PlaySoundAtLocation` null (`SceneComponent.K2_GetComponentLocation` (`self.Sphere1`)) (struct) 1.0 1.0 0.0 null null null))

(event `self.Sphere1.OnComponentBeginOverlap`
  (params (OverlappedComponent :type "PrimitiveComponent Object Reference") (OtherActor :type "Actor Object Reference") (OtherComp :type "PrimitiveComponent Object Reference") (OtherBodyIndex :type Integer) (bFromSweep :type Boolean) (SweepResult :type "HitResult Structure (by ref)"))
  (if (`self.ActorHasTag` OtherActor "Floor")
    (`SceneComponent.SetHiddenInGame` (`self.DefaultSceneRoot`) true true :!label _label)
    (`|SpawnActorFromClass` "/Game/Léo/Blueprint/EyesBombers/Eyes_Bomber_Mob_BP.Eyes_Bomber_Mob_BP_C" (`KismetMathLibrary.MakeTransform` (`self.K2_GetActorLocation`)) "Undefined" "OverrideRootScale" null null)
    (`KismetSystemLibrary.Delay` 0.2)
    (`self.K2_DestroyActor`)
    (elif (`ActorComponent.ComponentHasTag` OtherComp "Floor")
      (goto _label))))

(fn `UserConstructionScript`)