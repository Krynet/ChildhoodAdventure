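; Counter projectile for the Eyes Bombers that explodes on tagged boss or wall targets and can home on a given component.
; Sphere overlap checks component tags, hides and destroys the projectile, and damages the phase 1 or 2 boss or the hit Wall_Eyes_Bomber.
; The WallTargetMax branch spawns with no class set, and its damage call is disconnected.
; Set_Homing turns on ProjectileMovement homing toward the supplied component.
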(event `self.Sphere1.OnComponentBeginOverlap`
  (params (OverlappedComponent :type "PrimitiveComponent Object Reference") (OtherActor :type "Actor Object Reference") (OtherComp :type "PrimitiveComponent Object Reference") (OtherBodyIndex :type Integer) (bFromSweep :type Boolean) (SweepResult :type "HitResult Structure (by ref)"))
  (`|ExecutionSequence`
    (:`then_0`
      (if (`ActorComponent.ComponentHasTag` OtherComp "BossTarget")
        (`|ExecutionSequence`
          (:`then_0`
            (`SceneComponent.SetHiddenInGame` (`self.DefaultSceneRoot`) true true)
            (`|SpawnActorFromClass` "/Game/Léo/Blueprint/EyesBombers/Explosion_Eyes_Bomber.Explosion_Eyes_Bomber_C" (`KismetMathLibrary.MakeTransform` (`self.K2_GetActorLocation`)) "Undefined" "OverrideRootScale" null null)
            (`KismetSystemLibrary.Delay` 0.02)
            (`self.K2_DestroyActor`))
          (:`then_1`
            (bind _returnvalue (`GameplayStatics.GetActorOfClass` "/Game/Léo/Blueprint/Boss/Boss_Phase_1/BOSS_BP/Boss_Phase_1_BP.Boss_Phase_1_BP_C"))
            (`/Game/Léo/Blueprint/Boss/Boss_Phase_1/BOSS_BP/Boss_Phase_1_BP.Deal_Damage_Eyes_Bomber` _returnvalue)))))
    (:`then_1`
      (if (`ActorComponent.ComponentHasTag` OtherComp "WallTarget")
        (`|ExecutionSequence`
          (:`then_0`
            (`SceneComponent.SetHiddenInGame` (`self.DefaultSceneRoot`) true true)
            (`|SpawnActorFromClass` "/Game/Léo/Blueprint/EyesBombers/Explosion_Eyes_Bomber.Explosion_Eyes_Bomber_C" (`KismetMathLibrary.MakeTransform` (`self.K2_GetActorLocation`)) "Undefined" "OverrideRootScale" null null)
            (`KismetSystemLibrary.Delay` 0.02)
            (`self.K2_DestroyActor`))
          (:`then_1`
            (bind _aswall_eyes_bomber (cast `/Game/Léo/Blueprint/Wall/Wall_Eyes_Bomber` OtherActor))
            (`/Game/Léo/Blueprint/Wall/Wall_Eyes_Bomber.Deal_Damage` _aswall_eyes_bomber)))))
    (:`then_2`
      (if (`ActorComponent.ComponentHasTag` OtherComp "Boss_2_Target")
        (`|ExecutionSequence`
          (:`then_0`
            (`SceneComponent.SetHiddenInGame` (`self.DefaultSceneRoot`) true true)
            (`|SpawnActorFromClass` "/Game/Léo/Blueprint/EyesBombers/Explosion_Eyes_Bomber.Explosion_Eyes_Bomber_C" (`KismetMathLibrary.MakeTransform` (`self.K2_GetActorLocation`)) "Undefined" "OverrideRootScale" null null)
            (`KismetSystemLibrary.Delay` 0.02)
            (`self.K2_DestroyActor`))
          (:`then_1`
            (bind _returnvalue_2 (`GameplayStatics.GetActorOfClass` "/Game/Léo/Blueprint/Boss_Phase_2/BP/Boss_Phase_2_BP.Boss_Phase_2_BP_C"))
            (`/Game/Léo/Blueprint/Boss_Phase_2/BP/Boss_Phase_2_BP.Deal Damage Eyes Bomber` _returnvalue_2)))))
    (:`then_3`
      (if (`ActorComponent.ComponentHasTag` OtherComp "WallTargetMax")
        (`|ExecutionSequence`
          (:`then_0`
            (`SceneComponent.SetHiddenInGame` (`self.DefaultSceneRoot`) true true)
            (`|SpawnActorFromClass` "/Game/Léo/Blueprint/EyesBombers/Explosion_Eyes_Bomber.Explosion_Eyes_Bomber_C" (`KismetMathLibrary.MakeTransform` (`self.K2_GetActorLocation`)) "Undefined" "OverrideRootScale" null null)
            (`KismetSystemLibrary.Delay` 0.02)
            (`self.K2_DestroyActor`)))))))

(event `Set_Homing`
  (params (NewParam :type "SphereComponent Object Reference"))
  (bind _projectilemovement (`self.ProjectileMovement`))
  (set `ProjectileMovementComponent.bIsHomingProjectile` true _projectilemovement)
  (set `ProjectileMovementComponent.HomingTargetComponent` NewParam _projectilemovement)
  (set `ProjectileMovementComponent.HomingAccelerationMagnitude` 1500.0 _projectilemovement))

(fn `UserConstructionScript`)