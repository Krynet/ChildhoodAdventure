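; Explosion actor for the Eyes Bomber enemy that pushes physics objects and damages bomber-targeted walls.
; On BeginPlay it fires a radial force impulse, then destroys itself after a short delay.
; Its sphere overlap calls DealDamage on Wall_Eyes_Bomber actors whose component is tagged WallTarget.
; The PlayerCapsule branch only casts to ThirdPersonCharacter and has no effect on the player yet.
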(event `self.ReceiveBeginPlay`
  (`RadialForceComponent.FireImpulse` (`self.RadialForce`))
  (`KismetSystemLibrary.Delay` 0.5)
  (`self.K2_DestroyActor`))

(event `self.Sphere.OnComponentBeginOverlap`
  (params (OverlappedComponent :type "PrimitiveComponent Object Reference") (OtherActor :type "Actor Object Reference") (OtherComp :type "PrimitiveComponent Object Reference") (OtherBodyIndex :type Integer) (bFromSweep :type Boolean) (SweepResult :type "HitResult Structure (by ref)"))
  (`|ExecutionSequence`
    (:`then_0`
      (if (`ActorComponent.ComponentHasTag` OtherComp "WallTarget")
        (bind _aswall_eyes_bomber (cast `/Game/Léo/Blueprint/Wall/Wall_Eyes_Bomber` OtherActor))
        (`/Game/Léo/Blueprint/Wall/Wall_Eyes_Bomber.Deal_Damage` _aswall_eyes_bomber)))
    (:`then_1`
      (if (`ActorComponent.ComponentHasTag` OtherComp "PlayerCapsule")
        (cast `/Game/ThirdPersonBP/Blueprints/ThirdPersonCharacter` OtherActor)))))

(fn `UserConstructionScript`)