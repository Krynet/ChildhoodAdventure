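; Bomber enemy mob that bobs its sphere on a looping timeline and drives player chasing through blackboard flags set by overlap spheres.
; Entering the explosion sphere flags the player in range, stops the bob and starts a self-calling, intensifying random shake, then destroys the actor five seconds later.
; A player punch on the hit sphere replaces the mob with a counter projectile aimed away from the player.
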(event `Shake`
  (bind _radius (`self.Radius`))
  (bind _timer (`self.Timer`))
  (bind _sphere (`self.Sphere`))
  (bind _z (.z (`self.InitUpDown`)))
  (`|ExecutionSequence`
    (:`then_0`
      (bind _randomlocation (`NavigationSystemV1.K2_GetRandomLocationInNavigableRadius` (`KismetMathLibrary.MakeVector` (.x (`self.InitUpDown`)) (.y (`self.InitUpDown`)) _z) (`self.Radius`) null null))
      (`KismetSystemLibrary.MoveComponentTo` _sphere (`KismetMathLibrary.MakeVector` (.x _randomlocation) (.y _randomlocation) _z) (`SceneComponent.RelativeRotation` _sphere))
      (`KismetSystemLibrary.Delay` (`self.Timer`))
      (`|ExecutionSequence`
        (:`then_0`
          (if (not (>= _radius 15.0))
            (set `self.Radius` (+ _radius 1.0))))
        (:`then_1`
          (if (not (<= _timer 0.0001))
            (set `self.Timer` (- _timer 0.0001)))))
      (`self.Shake`))
    (:`then_1`
      (bind (_direction _newtrack_0) (`Timeline|UpDown` :!via `Stop` :!label _label)
        (:`Update`
          (`SceneComponent.K2_SetRelativeLocation` (`self.Sphere`) (`KismetMathLibrary.VLerp` (`self.InitUpDown`) (`self.EndUpDown`) _newtrack_0) false false))
        (:`Finished`
          (`self.Relaunch`))))))

(event `self.ReceiveBeginPlay`
  (bind _relativelocation (`SceneComponent.RelativeLocation` (`self.Sphere`)))
  (set `self.InitUpDown` _relativelocation)
  (set `self.EndUpDown` (+ _relativelocation (0.0 0.0 20.0)))
  (goto _label))

(event `Relaunch`
  (goto _label :!via `PlayFromStart`))

(event `self.ChaseSphere.OnComponentBeginOverlap`
  (params (OverlappedComponent :type "PrimitiveComponent Object Reference") (OtherActor :type "Actor Object Reference") (OtherComp :type "PrimitiveComponent Object Reference") (OtherBodyIndex :type Integer) (bFromSweep :type Boolean) (SweepResult :type "HitResult Structure (by ref)"))
  (if (`ActorComponent.ComponentHasTag` OtherComp "PlayerCapsule")
    (`BlackboardComponent.SetValueAsBool` (`AIBlueprintHelperLibrary.GetBlackboard` null) "ChasePlayer" true)))

(event `self.ExplosionSphere.OnComponentBeginOverlap`
  (params (OverlappedComponent :type "PrimitiveComponent Object Reference") (OtherActor :type "Actor Object Reference") (OtherComp :type "PrimitiveComponent Object Reference") (OtherBodyIndex :type Integer) (bFromSweep :type Boolean) (SweepResult :type "HitResult Structure (by ref)"))
  (if (`ActorComponent.ComponentHasTag` OtherComp "PlayerCapsule")
    (`/Engine/EditorBlueprintResources/StandardMacros.DoOnce` false
      (:`Completed`
        (`BlackboardComponent.SetValueAsBool` (`AIBlueprintHelperLibrary.GetBlackboard` null) "InRange" true)
        (`|ExecutionSequence`
          (:`then_0`
            (`self.Shake`))
          (:`then_1`
            (`KismetSystemLibrary.Delay` 5.0)
            (`self.K2_DestroyActor`)))))))

(event `self.HitSphere.OnComponentBeginOverlap`
  (params (OverlappedComponent :type "PrimitiveComponent Object Reference") (OtherActor :type "Actor Object Reference") (OtherComp :type "PrimitiveComponent Object Reference") (OtherBodyIndex :type Integer) (bFromSweep :type Boolean) (SweepResult :type "HitResult Structure (by ref)"))
  (if (`ActorComponent.ComponentHasTag` OtherComp "PunchBox")
    (bind _returnvalue (`GameplayStatics.GetActorOfClass` "/Game/ThirdPersonBP/Blueprints/ThirdPersonCharacter.ThirdPersonCharacter_C"))
    (if (`/Game/ThirdPersonBP/Blueprints/ThirdPersonCharacter.Punch` _returnvalue)
      (bind (_returnvalue_roll _returnvalue_pitch _returnvalue_yaw) (`KismetMathLibrary.BreakRotator` (`KismetMathLibrary.FindLookAtRotation` (`self.K2_GetActorLocation` _returnvalue) (`self.K2_GetActorLocation`))))
      (`SceneComponent.K2_SetWorldRotation` (`self.Arrow1`) (`KismetMathLibrary.MakeRotator` 0.0 0.0 _returnvalue_yaw) false false)
      (`|SpawnActorFromClass` "/Game/Léo/Blueprint/EyesBombers/Bomber_Projectiles_Counter_BP.Bomber_Projectiles_Counter_BP_C" (`KismetMathLibrary.MakeTransform` (`self.K2_GetActorLocation`) (`SceneComponent.K2_GetComponentRotation` (`self.Arrow1`))) "Undefined" "OverrideRootScale" null null)
      (`KismetSystemLibrary.Delay` 0.01)
      (`self.K2_DestroyActor`))))

(fn `UserConstructionScript`)