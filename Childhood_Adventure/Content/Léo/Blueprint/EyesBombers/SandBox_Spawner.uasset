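; Sandbox spawner that repeatedly fires Bomber_Projectiles_BP actors while the player is within its trigger area.
; Overlap events on Sphere1 set a Player flag for components tagged PlayerCapsule.
; From BeginPlay, a self-restarting Delay loop waits for Time, then spawns only if that flag is set.
; Projectiles spawn at the Sphere component's location, oriented along the Arrow component.
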(event `Respawn`
  (`KismetSystemLibrary.Delay` (`self.Time`) :!label _label)
  (if (`self.Player`)
    (`|SpawnActorFromClass` "/Game/Léo/Blueprint/EyesBombers/Bomber_Projectiles_BP.Bomber_Projectiles_BP_C" (`KismetMathLibrary.MakeTransform` (`SceneComponent.K2_GetComponentLocation` (`self.Sphere`)) (`SceneComponent.K2_GetComponentRotation` (`self.Arrow`))) "Undefined" "OverrideRootScale" null null)
    (`self.Respawn`)
    (else
      (goto _label))))

(event `self.ReceiveBeginPlay`
  (goto _label))

(event `self.Sphere1.OnComponentBeginOverlap`
  (params (OverlappedComponent :type "PrimitiveComponent Object Reference") (OtherActor :type "Actor Object Reference") (OtherComp :type "PrimitiveComponent Object Reference") (OtherBodyIndex :type Integer) (bFromSweep :type Boolean) (SweepResult :type "HitResult Structure (by ref)"))
  (if (`ActorComponent.ComponentHasTag` OtherComp "PlayerCapsule")
    (set `self.Player` true)))

(event `self.Sphere1.OnComponentEndOverlap`
  (params (OverlappedComponent :type "PrimitiveComponent Object Reference") (OtherActor :type "Actor Object Reference") (OtherComp :type "PrimitiveComponent Object Reference") (OtherBodyIndex :type Integer))
  (if (`ActorComponent.ComponentHasTag` OtherComp "PlayerCapsule")
    (set `self.Player` false)))

(fn `UserConstructionScript`)