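; Eyes minigun actor that sprays laser projectiles from Sphere2, then destroys itself once its shot limit is passed.
; ChargeEvent spawns a charge projectile attached to Sphere2.
; FireEvent re-calls itself on a short delay, picking each shot's rotation at random from FireDirection, which it resets once to all-zero entries.
; BeginPlay only caches the player and waits; the look-at and charge-then-fire chains are disconnected, so nothing here starts the attack.
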(event `self.ReceiveBeginPlay`
  (bind _returnvalue (`GameplayStatics.GetActorOfClass` "/Game/ThirdPersonBP/Blueprints/ThirdPersonCharacter.ThirdPersonCharacter_C"))
  (set `self.Player` _returnvalue)
  (`KismetSystemLibrary.Delay` 3.0))

(event `self.ReceiveTick`
  (params (DeltaSeconds :type "Float (single-precision)")))

(event `Charge Event`
  (bind _sphere2 (`self.Sphere2`))
  (bind _returnvalue (`|SpawnActorFromClass` "/Game/Léo/Blueprint/Observer/Charge_Projectile_Observer.Charge_Projectile_Observer_C" (`KismetMathLibrary.MakeTransform` (`SceneComponent.K2_GetComponentLocation` _sphere2)) "Undefined" "OverrideRootScale" null null))
  (`self.K2_AttachToComponent` _returnvalue _sphere2 "None" "SnapToTarget" "SnapToTarget" "KeepWorld" true))

(event `Fire Event`
  (`|ExecutionSequence`
    (:`then_0`
      (if (<= (`self.Fire_Count`) (`self.Fire_Count_Max`))
        (`|SpawnActorFromClass` "/Game/Léo/Blueprint/LaserProjectiles/LaserProjectiles_BP.LaserProjectiles_BP_C" (`KismetMathLibrary.MakeTransform` (`SceneComponent.K2_GetComponentLocation` (`self.Sphere2`)) (`|GetArrayItem` (`self.Fire_Direction`) (`KismetMathLibrary.RandomIntegerInRange` 0 19))) "Undefined" "OverrideRootScale" null null)
        (`/Engine/EditorBlueprintResources/StandardMacros.IncrementInt` (`self.Fire_Count`)
          (:`  `
            (`KismetSystemLibrary.Delay` 0.2)
            (`self.Fire Event`)))
        (else
          (`self.K2_DestroyActor`))))
    (:`then_1`
      (`/Engine/EditorBlueprintResources/StandardMacros.DoOnce` false
        (:`Completed`
          (set `self.Fire_Direction` (`|MakeArray` (struct) (struct) (struct) (struct) (struct) (struct) (struct) (struct) (struct) (struct) (struct) (struct) (struct) (struct) (struct) (struct) (struct) (struct) (struct) (struct) :!type "Rotator Structure")))))))

(fn `UserConstructionScript`)