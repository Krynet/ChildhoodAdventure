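; FX_Crash_Boss_2 is an effect actor, named for a boss crash, that repeatedly spawns FX_Boom effects while turning toward the player.
; BeginPlay gathers four PowLocation components and starts LaunchHit, which rotates the actor to face the ThirdPersonCharacter and spawns a randomly scaled boom at one of those points.
; LaunchHit re-calls itself after a two-second delay, looping while the player cast succeeds.
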(event `self.ReceiveBeginPlay`
  (set `self.PowLocationList` (`|MakeArray` (`self.Pow_Location_1`) (`self.Pow_Location_2`) (`self.Pow_Location_3`) (`self.Pow_Location_4`)))
  (set `self.FXHitLocation` (`|MakeArray` null null null null :!type "SphereComponent Object Reference"))
  (`self.LaunchHit`))

(event `LaunchHit`
  (bind _powlocationlist (`self.PowLocationList`))
  (bind _asthird_person_character (cast `/Game/ThirdPersonBP/Blueprints/ThirdPersonCharacter` (`GameplayStatics.GetPlayerCharacter` 0)))
  (`self.K2_SetActorRotation` (`KismetMathLibrary.FindLookAtRotation` (`self.K2_GetActorLocation`) (`self.K2_GetActorLocation` _asthird_person_character)))
  (`|ExecutionSequence`
    (:`then_1`
      (`|SpawnActorFromClass` "/Game/Léo/Blueprint/FX/FX_Boom.FX_Boom_C" (`KismetMathLibrary.MakeTransform` (`SceneComponent.K2_GetComponentLocation` (`|GetArrayItem` _powlocationlist (`KismetMathLibrary.RandomInteger` (`KismetArrayLibrary.Array_Length` _powlocationlist)))) (struct) (`KismetMathLibrary.MakeVector` (`KismetMathLibrary.RandomFloatInRange` 0.7 1.4) (`KismetMathLibrary.RandomFloatInRange` 0.7 1.4) (`KismetMathLibrary.RandomFloatInRange` 0.7 1.4))) "AlwaysSpawn" "OverrideRootScale" null null))
    (:`then_2`
      (`KismetSystemLibrary.Delay` 2.0)
      (`self.LaunchHit`))))

(fn `UserConstructionScript`)