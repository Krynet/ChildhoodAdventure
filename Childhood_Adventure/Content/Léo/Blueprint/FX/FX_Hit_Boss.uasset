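; Boss hit effect actor that repeatedly plays comic-style punch impact visuals, starting on BeginPlay.
; LaunchHit turns the actor toward the player character, then spawns FX_Punch_Explode and FX_Pow, each at a random point from its own four-location list.
; Each spawn gets a random per-axis scale, with Pow larger than the explosion.
; LaunchHit re-calls itself after a two-second delay, looping with no stop condition beyond a failed player cast.
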(event `self.ReceiveBeginPlay`
  (set `self.PowLocationList` (`|MakeArray` (`self.Pow_Location_1`) (`self.Pow_Location_2`) (`self.Pow_Location_3`) (`self.Pow_Location_4`)))
  (set `self.FXHitLocation` (`|MakeArray` (`self.FX_Hit_Location_1`) (`self.FX_Hit_Location_2`) (`self.FX_Hit_Location_3`) (`self.FX_Hit_Location_4`)))
  (`self.LaunchHit`))

(event `LaunchHit`
  (bind _powlocationlist (`self.PowLocationList`))
  (bind _fxhitlocation (`self.FXHitLocation`))
  (bind _asthird_person_character (cast `/Game/ThirdPersonBP/Blueprints/ThirdPersonCharacter` (`GameplayStatics.GetPlayerCharacter` 0)))
  (`self.K2_SetActorRotation` (`KismetMathLibrary.FindLookAtRotation` (`self.K2_GetActorLocation`) (`self.K2_GetActorLocation` _asthird_person_character)))
  (`|ExecutionSequence`
    (:`then_0`
      (`|SpawnActorFromClass` "/Game/Léo/Blueprint/Maé_BoxCollider/FX_Punch_Explode.FX_Punch_Explode_C" (`KismetMathLibrary.MakeTransform` (`SceneComponent.K2_GetComponentLocation` (`|GetArrayItem` _fxhitlocation (`KismetMathLibrary.RandomInteger` (`KismetArrayLibrary.Array_Length` _fxhitlocation)))) (struct) (`KismetMathLibrary.MakeVector` (`KismetMathLibrary.RandomFloatInRange` 0.2 0.6) (`KismetMathLibrary.RandomFloatInRange` 0.2 0.6) (`KismetMathLibrary.RandomFloatInRange` 0.2 0.6))) "AlwaysSpawn" "OverrideRootScale" null null))
    (:`then_1`
      (`|SpawnActorFromClass` "/Game/Léo/Blueprint/FX/FX_Pow.FX_Pow_C" (`KismetMathLibrary.MakeTransform` (`SceneComponent.K2_GetComponentLocation` (`|GetArrayItem` _powlocationlist (`KismetMathLibrary.RandomInteger` (`KismetArrayLibrary.Array_Length` _powlocationlist)))) (struct) (`KismetMathLibrary.MakeVector` (`KismetMathLibrary.RandomFloatInRange` 0.7 1.4) (`KismetMathLibrary.RandomFloatInRange` 0.7 1.4) (`KismetMathLibrary.RandomFloatInRange` 0.7 1.4))) "AlwaysSpawn" "OverrideRootScale" null null))
    (:`then_2`
      (`KismetSystemLibrary.Delay` 2.0)
      (`self.LaunchHit`))))

(fn `UserConstructionScript`)