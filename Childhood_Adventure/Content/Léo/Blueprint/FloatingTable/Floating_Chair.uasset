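; Floating chair actor that drifts and tilts around its placed transform in a continuous animation.
; At BeginPlay it stores its location and rotation, then picks a small random offset target for each once.
; Two timelines lerp each axis separately between start and target, one for location and one for rotation.
; When the location timeline finishes, RelaunchAtEnd restarts both, reusing the same targets.
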(event `Relaunch At End`
  (`|ExecutionSequence` :!label _label
    (:`then_0`
      (bind (_direction _x _y _z) (`Timeline|Timeline_0` :!via `PlayFromStart`)
        (:`Update`
          (`self.K2_SetActorLocation` (`KismetMathLibrary.MakeVector` (`KismetMathLibrary.Lerp` (.x (`self.Floating_Actor_Location`)) (.x (`self.Floating_Actor_Location_2`)) _x) (`KismetMathLibrary.Lerp` (.y (`self.Floating_Actor_Location`)) (.y (`self.Floating_Actor_Location_2`)) _y) (`KismetMathLibrary.Lerp` (.z (`self.Floating_Actor_Location`)) (.z (`self.Floating_Actor_Location_2`)) _z))))
        (:`Finished`
          (`self.Relaunch At End`))))
    (:`then_1`
      (bind (_direction_2 _x_2 _y_2 _z_2) (`Timeline|Timeline_1` :!via `PlayFromStart`)
        (:`Update`
          (`self.K2_SetActorRotation` (`KismetMathLibrary.MakeRotator` (`KismetMathLibrary.Lerp` (.roll (`self.Floating_Actor_Rotation`)) (.roll (`self.Floating_Actor_Rotation_2`)) _x_2) (`KismetMathLibrary.Lerp` (.pitch (`self.Floating_Actor_Rotation`)) (.pitch (`self.Floating_Actor_Rotation_2`)) _y_2) (`KismetMathLibrary.Lerp` (.yaw (`self.Floating_Actor_Rotation`)) (.yaw (`self.Floating_Actor_Rotation_2`)) _z_2))))))))

(event `self.ReceiveBeginPlay`
  (bind _output_get (set `self.Floating_Actor_Rotation` (`self.K2_GetActorRotation`)))
  (set `self.Floating_Actor_Rotation_2` (`KismetMathLibrary.MakeRotator` (+ (.roll _output_get) (`KismetMathLibrary.RandomFloatInRange` -10.0 10.0)) (+ (.pitch _output_get) (`KismetMathLibrary.RandomFloatInRange` -10.0 10.0)) (+ (.yaw _output_get) (`KismetMathLibrary.RandomFloatInRange` -10.0 10.0))))
  (bind _output_get_2 (set `self.Floating_Actor_Location` (`self.K2_GetActorLocation`)))
  (set `self.Floating_Actor_Location_2` (+ _output_get_2 (`KismetMathLibrary.MakeVector` (`KismetMathLibrary.RandomFloatInRange` -10.0 10.0) (`KismetMathLibrary.RandomFloatInRange` -10.0 10.0) (`KismetMathLibrary.RandomFloatInRange` -20.0 20.0))))
  (goto _label))

(fn `UserConstructionScript`)