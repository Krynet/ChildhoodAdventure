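; Floating platform actor that bobs in place and sinks when the player stands on it.
; A looping timeline drifts it toward a small random offset picked whenever floating starts.
; One second after a PlayerCapsule-tagged component enters the Box, floating stops and it lerps between world positions cached once from Up and Down.
; Three seconds after exit, if still empty, it rises back, resumes floating and re-arms the descent.
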(event `Relaunch At Up`
  (bind _output_get (set `self.Floating_Actor_Location` (`self.K2_GetActorLocation`) :!label _label))
  (set `self.Floating_Actor_Location_2` (+ _output_get (`KismetMathLibrary.MakeVector` (`KismetMathLibrary.RandomFloatInRange` -10.0 10.0) (`KismetMathLibrary.RandomFloatInRange` -10.0 10.0) (`KismetMathLibrary.RandomFloatInRange` -10.0 10.0))))
  (bind (_direction _x _y _z) (`Timeline|Timeline_0` :!via `PlayFromStart` :!label _label_2)
    (:`Update`
      (`self.K2_SetActorLocation` (`KismetMathLibrary.MakeVector` (`KismetMathLibrary.Lerp` (.x (`self.Floating_Actor_Location`)) (.x (`self.Floating_Actor_Location_2`)) _x) (`KismetMathLibrary.Lerp` (.y (`self.Floating_Actor_Location`)) (.y (`self.Floating_Actor_Location_2`)) _y) (`KismetMathLibrary.Lerp` (.z (`self.Floating_Actor_Location`)) (.z (`self.Floating_Actor_Location_2`)) _z))))
    (:`Finished`
      (`self.Relaunch At End`))))

(event `Relaunch At End`
  (goto _label_2 :!via `PlayFromStart`))

(event `self.ReceiveBeginPlay`
  (goto _label))

(event `Stop Floating`
  (goto _label_2 :!via `Stop`))

(event `self.Box.OnComponentBeginOverlap`
  (params (OverlappedComponent :type "PrimitiveComponent Object Reference") (OtherActor :type "Actor Object Reference") (OtherComp :type "PrimitiveComponent Object Reference") (OtherBodyIndex :type Integer) (bFromSweep :type Boolean) (SweepResult :type "HitResult Structure (by ref)"))
  (if (`ActorComponent.ComponentHasTag` OtherComp "PlayerCapsule")
    (set `self.ActorOnBoard` true)
    (`KismetSystemLibrary.Delay` 1.0)
    (`|ExecutionSequence`
      (:`then_0`
        (`/Engine/EditorBlueprintResources/StandardMacros.DoOnce` false
          (:`Completed`
            (set `self.ActorInitLocation` (`SceneComponent.K2_GetComponentLocation` (`self.Up`)))
            (set `self.ActorEndLocation` (`SceneComponent.K2_GetComponentLocation` (`self.Down`))))))
      (:`then_1`
        (`/Engine/EditorBlueprintResources/StandardMacros.DoOnce` false :!label _label_3
          (:`Completed`
            (`|ExecutionSequence`
              (:`then_0`
                (`self.Stop Floating`))
              (:`then_1`
                (bind (_direction _godown) (`Timeline|Go Down` :!via `PlayFromStart`)
                  (:`Update`
                    (`self.K2_SetActorLocation` (`KismetMathLibrary.VLerp` (`self.ActorInitLocation`) (`self.ActorEndLocation`) _godown))))))))))))

(event `self.Box.OnComponentEndOverlap`
  (params (OverlappedComponent :type "PrimitiveComponent Object Reference") (OtherActor :type "Actor Object Reference") (OtherComp :type "PrimitiveComponent Object Reference") (OtherBodyIndex :type Integer))
  (if (`ActorComponent.ComponentHasTag` OtherComp "PlayerCapsule")
    (set `self.ActorOnBoard` false)
    (`|ExecutionSequence`
      (:`then_0`
        (`KismetSystemLibrary.Delay` 3.0)
        (if (not (`self.ActorOnBoard`))
          (bind (_direction _newtrack_0) (`Timeline|Timeline_1` :!via `PlayFromStart`)
            (:`Update`
              (`self.K2_SetActorLocation` (`KismetMathLibrary.VLerp` (`self.ActorEndLocation`) (`self.ActorInitLocation`) _newtrack_0)))
            (:`Finished`
              (`self.Relaunch At Up`)
              (goto _label_3 :!via `Reset`))))))))

(fn `UserConstructionScript`)