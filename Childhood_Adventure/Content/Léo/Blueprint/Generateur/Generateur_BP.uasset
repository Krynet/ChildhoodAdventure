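; Punchable generator that, once hit enough times, powers a street lamp (Lampadaire) and removes a light door (Porte_Lumière_BP).
; Overlaps from the player's PunchBox during a punch play a vibration timeline on the cube and increment a hit counter until CountMax.
; A further punch calls Launch, which replays a motion timeline by calling itself, while a DoOnce activates the lamp and destroys the door a second later.
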(event `self.ReceiveBeginPlay`
  (set `self.Init Location` (`SceneComponent.K2_GetComponentLocation` (`self.Cube`)))
  (bind _returnvalue (`GameplayStatics.GetActorOfClass` "/Game/ThirdPersonBP/Blueprints/ThirdPersonCharacter.ThirdPersonCharacter_C"))
  (set `self.Player` _returnvalue))

(event `self.Box.OnComponentBeginOverlap`
  (params (OverlappedComponent :type "PrimitiveComponent Object Reference") (OtherActor :type "Actor Object Reference") (OtherComp :type "PrimitiveComponent Object Reference") (OtherBodyIndex :type Integer) (bFromSweep :type Boolean) (SweepResult :type "HitResult Structure (by ref)"))
  (if (`ActorComponent.ComponentHasTag` OtherComp "PunchBox")
    (if (`/Game/ThirdPersonBP/Blueprints/ThirdPersonCharacter.Punch` (`self.Player`))
      (if (< (`self.Count`) (`self.Count_Max`))
        (bind (_direction _vibration) (`Timeline|Vibration` :!via `PlayFromStart`)
          (:`Update`
            (`SceneComponent.K2_SetWorldLocation` (`self.Cube`) (+ _vibration (`self.Init Location`)) false false))
          (:`Finished`
            (`SceneComponent.K2_SetWorldLocation` (`self.Cube`) (`self.Init Location`) false false)
            (`/Engine/EditorBlueprintResources/StandardMacros.IncrementInt` (`self.Count`))))
        (else
          (`self.Launch`))))))

(event `Launch`
  (`|ExecutionSequence`
    (:`then_0`
      (bind (_direction _newtrack_0) (`Timeline|Timeline_0` :!via `PlayFromStart`)
        (:`Update`
          (`SceneComponent.K2_SetWorldLocation` (`self.Cube`) (+ _newtrack_0 (`self.Init Location`)) false false))
        (:`Finished`
          (`SceneComponent.K2_SetWorldLocation` (`self.Cube`) (0.0 0.0 0.0) false false)
          (`self.Launch`))))
    (:`then_1`
      (`/Engine/EditorBlueprintResources/StandardMacros.DoOnce` false
        (:`Completed`
          (`|ExecutionSequence`
            (:`then_0`
              (bind _returnvalue (`GameplayStatics.GetActorOfClass` "/Game/Léo/Blueprint/Generateur/Lampadaire.Lampadaire_C"))
              (`/Game/Léo/Blueprint/Generateur/Lampadaire.Activate` _returnvalue))
            (:`then_1`
              (`KismetSystemLibrary.Delay` 1.0)
              (bind _returnvalue_2 (`GameplayStatics.GetActorOfClass` "/Game/Léo/Blueprint/Generateur/Porte_Lumière_BP.Porte_Lumière_BP_C"))
              (`self.K2_DestroyActor` _returnvalue_2))))))))

(fn `UserConstructionScript`)