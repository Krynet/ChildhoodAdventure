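; Fracture is a geyser fissure Blueprint that cycles five charge and five emitter effect systems in an endless timed loop.
; On BeginPlay it gathers the systems into two lists, then after a short delay activates the charge effects as a build-up.
; It then swaps them for the longer eruption emitters, deactivates those and immediately restarts the cycle.
; The Blueprint handles only visual effects timing, with no collision or gameplay logic in its graphs.
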(event `self.ReceiveBeginPlay`
  (set `self.Charge_FX_List` (`|MakeArray` (`self.Geyser_Charge_System`) (`self.Geyser_Charge_System1`) (`self.Geyser_Charge_System2`) (`self.Geyser_Charge_System3`) (`self.Geyser_Charge_System4`)))
  (set `self.FX_List` (`|MakeArray` (`self.Geyser_Emiter_System`) (`self.Geyser_Emiter_System1`) (`self.Geyser_Emiter_System2`) (`self.Geyser_Emiter_System3`) (`self.Geyser_Emiter_System4`)))
  (`KismetSystemLibrary.Delay` 2.0)
  (for _array_element (`self.Charge_FX_List`) :!label _label
    (`ActorComponent.Activate` _array_element false))
  (`KismetSystemLibrary.Delay` 2.0)
  (for _array_element_2 (`self.Charge_FX_List`)
    (`ActorComponent.Deactivate` _array_element_2))
  (for _array_element_3 (`self.FX_List`)
    (`ActorComponent.Activate` _array_element_3 false))
  (`KismetSystemLibrary.Delay` 9.0)
  (for _array_element_4 (`self.FX_List`)
    (`ActorComponent.Deactivate` _array_element_4))
  (goto _label))

(fn `UserConstructionScript`)