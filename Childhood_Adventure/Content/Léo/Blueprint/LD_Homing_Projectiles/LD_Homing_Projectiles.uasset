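; Homing projectile that chases the player's PlayerTarget component and self-destructs after a fixed lifetime.
; Capsule overlaps with the player capsule or DestroyProjectil-tagged actors spawn an explosion and destroy it, while components tagged "Enable Homing" switch homing off despite the name.
; A PunchBox overlap during a punch shakes the camera and swaps it for a rotated LD_Return_Homing_Projectiles, which receives the originating spawner reference.
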(event `self.ReceiveBeginPlay`
  (bind _projectilemovement (`self.ProjectileMovement`))
  (`GameplayStatics.PlaySoundAtLocation` "/Game/Sounds/Ombras/oeil_attaque_Cue.oeil_attaque_Cue" (`SceneComponent.K2_GetComponentLocation` (`self.Capsule`)) (struct) 1.0 1.0 0.0 null null null)
  (bind _returnvalue (`GameplayStatics.GetActorOfClass` "/Game/ThirdPersonBP/Blueprints/ThirdPersonCharacter.ThirdPersonCharacter_C"))
  (set `ProjectileMovementComponent.bIsHomingProjectile` true _projectilemovement)
  (set `ProjectileMovementComponent.HomingTargetComponent` (`/Game/ThirdPersonBP/Blueprints/ThirdPersonCharacter.PlayerTarget` _returnvalue) _projectilemovement)
  (set `ProjectileMovementComponent.HomingAccelerationMagnitude` 3000.0 _projectilemovement)
  (`KismetSystemLibrary.Delay` 10.0)
  (`self.K2_DestroyActor`))

(event `self.Capsule.OnComponentBeginOverlap`
  (params (OverlappedComponent :type "PrimitiveComponent Object Reference") (OtherActor :type "Actor Object Reference") (OtherComp :type "PrimitiveComponent Object Reference") (OtherBodyIndex :type Integer) (bFromSweep :type Boolean) (SweepResult :type "HitResult Structure (by ref)"))
  (`|ExecutionSequence`
    (:`then_0`
      (if (or (`ActorComponent.ComponentHasTag` OtherComp "PlayerCapsule") (`self.ActorHasTag` OtherActor "DestroyProjectil"))
        (`/Engine/EditorBlueprintResources/StandardMacros.DoOnce` false
          (:`Completed`
            (`|SpawnActorFromClass` "/Game/Léo/Blueprint/Boss/Boss_Phase_1/BOSS_BP/Homing_Projectiles/Projectile_Explosion_BP.Projectile_Explosion_BP_C" (`KismetMathLibrary.MakeTransform` (`KismetMathLibrary.MakeVector` (.x (`SceneComponent.K2_GetComponentLocation` (`self.DefaultSceneRoot`))) (.y (`SceneComponent.K2_GetComponentLocation` (`self.DefaultSceneRoot`))) (- (.z (`SceneComponent.K2_GetComponentLocation` (`self.DefaultSceneRoot`))) 100.0))) "Undefined" "OverrideRootScale" null null)
            (`KismetSystemLibrary.Delay` 0.02)
            (`self.K2_DestroyActor`)))))
    (:`then_1`
      (if (`ActorComponent.ComponentHasTag` OtherComp "Enable Homing")
        (set `ProjectileMovementComponent.bIsHomingProjectile` false (`self.ProjectileMovement`))))
    (:`then_2`
      (if (`ActorComponent.ComponentHasTag` OtherComp "PunchBox")
        (bind _returnvalue (`GameplayStatics.GetActorOfClass` "/Game/ThirdPersonBP/Blueprints/ThirdPersonCharacter.ThirdPersonCharacter_C"))
        (if (`/Game/ThirdPersonBP/Blueprints/ThirdPersonCharacter.Punch` _returnvalue)
          (`PlayerController.ClientStartCameraShake` :`self` (`GameplayStatics.GetPlayerController` 0) :`Shake` "/Game/Léo/Blueprint/ShakeCamera/BP_Camera_Shake.BP_Camera_Shake_C")
          (bind _returnvalue_2 (`|SpawnActorFromClass` "/Game/Léo/Blueprint/LD_Homing_Projectiles/LD_Return_Homing_Projectiles.LD_Return_Homing_Projectiles_C" (`KismetMathLibrary.MakeTransform` (`self.K2_GetActorLocation`) (`KismetMathLibrary.MakeRotator` (+ (.roll (`self.K2_GetActorRotation`)) 180.0) (+ (.pitch (`self.K2_GetActorRotation`)) 180.0) (.yaw (`self.K2_GetActorRotation`)))) "AlwaysSpawn" "OverrideRootScale" null null))
          (bind _asspawner_projectile_bp (cast `/Game/Léo/Blueprint/Spawner/Spawner_HomingProjectile/Spawner_Projectile_BP` (`self.Spawner_Homing_Projectile`)))
          (set `/Game/Léo/Blueprint/LD_Homing_Projectiles/LD_Return_Homing_Projectiles.Spawner_Homing_Projectile` _asspawner_projectile_bp _returnvalue_2)
          (`KismetSystemLibrary.Delay` 0.01)
          (`self.K2_DestroyActor`))))))

(fn `UserConstructionScript`)