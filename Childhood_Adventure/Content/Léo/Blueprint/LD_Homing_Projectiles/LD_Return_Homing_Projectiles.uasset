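; LD_Return_Homing_Projectiles is a returning projectile actor that homes in on the target of its SpawnerHomingProjectile and damages that spawner on a hit.
; Shortly after BeginPlay it turns on ProjectileMovement homing toward that target, then self-destroys after a fixed lifetime.
; Capsule overlap with a TentacleTarget-tagged component spawns an explosion, destroys the projectile and calls the spawner's TakeDamage.
; Overlap with anything tagged DestroyProjectil only explodes and destroys it.
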(event `self.ReceiveBeginPlay`
  (bind _projectilemovement (`self.ProjectileMovement`))
  (`KismetSystemLibrary.Delay` 0.05)
  (set `ProjectileMovementComponent.bIsHomingProjectile` true _projectilemovement)
  (set `ProjectileMovementComponent.HomingTargetComponent` (`/Game/Léo/Blueprint/Spawner/Spawner_HomingProjectile/Spawner_Projectile_BP.Target` (`self.Spawner_Homing_Projectile`)) _projectilemovement)
  (set `ProjectileMovementComponent.HomingAccelerationMagnitude` 3000.0 _projectilemovement)
  (`KismetSystemLibrary.Delay` 10.0)
  (`self.K2_DestroyActor`))

(event `self.Capsule.OnComponentBeginOverlap`
  (params (OverlappedComponent :type "PrimitiveComponent Object Reference") (OtherActor :type "Actor Object Reference") (OtherComp :type "PrimitiveComponent Object Reference") (OtherBodyIndex :type Integer) (bFromSweep :type Boolean) (SweepResult :type "HitResult Structure (by ref)"))
  (`|ExecutionSequence`
    (:`then_0`
      (if (`ActorComponent.ComponentHasTag` OtherComp "TentacleTarget")
        (`|ExecutionSequence`
          (:`then_0`
            (`|SpawnActorFromClass` "/Game/Léo/Blueprint/Boss/Boss_Phase_1/BOSS_BP/Homing_Projectiles/Projectile_Explosion_BP.Projectile_Explosion_BP_C" (`KismetMathLibrary.MakeTransform` (`KismetMathLibrary.MakeVector` (.x (`SceneComponent.K2_GetComponentLocation` (`self.DefaultSceneRoot`))) (.y (`SceneComponent.K2_GetComponentLocation` (`self.DefaultSceneRoot`))) (- (.z (`SceneComponent.K2_GetComponentLocation` (`self.DefaultSceneRoot`))) 100.0))) "Undefined" "OverrideRootScale" null null)
            (`KismetSystemLibrary.Delay` 0.02)
            (`self.K2_DestroyActor`))
          (:`then_1`
            (`/Game/Léo/Blueprint/Spawner/Spawner_HomingProjectile/Spawner_Projectile_BP.Take_Damage` (`self.Spawner_Homing_Projectile`))))))
    (:`then_1`
      (if (or (`ActorComponent.ComponentHasTag` OtherComp "DestroyProjectil") (`self.ActorHasTag` OtherActor "DestroyProjectil"))
        (`|SpawnActorFromClass` "/Game/Léo/Blueprint/Boss/Boss_Phase_1/BOSS_BP/Homing_Projectiles/Projectile_Explosion_BP.Projectile_Explosion_BP_C" (`KismetMathLibrary.MakeTransform` (`KismetMathLibrary.MakeVector` (.x (`SceneComponent.K2_GetComponentLocation` (`self.DefaultSceneRoot`))) (.y (`SceneComponent.K2_GetComponentLocation` (`self.DefaultSceneRoot`))) (- (.z (`SceneComponent.K2_GetComponentLocation` (`self.DefaultSceneRoot`))) 100.0))) "Undefined" "OverrideRootScale" null null)
        (`KismetSystemLibrary.Delay` 0.02)
        (`self.K2_DestroyActor`)))))

(fn `UserConstructionScript`)