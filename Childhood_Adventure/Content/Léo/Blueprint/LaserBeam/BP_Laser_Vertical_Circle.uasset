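; Laser beam hazard that fires along the LaserEyes actor's facing and damages the player.
; Each tick it line traces up to weapon range, drives the Niagara beam end and toggles hit particles through paired DoOnce gates.
; Hits on components tagged PlayerMesh call LaserDamage on the cached ThirdPersonCharacter.
; StopLaser shuts off the effects, animates beam scale through a timeline, then destroys the actor.
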(event `self.ReceiveBeginPlay`
  (bind _returnvalue (`GameplayStatics.GetActorOfClass` "/Game/ThirdPersonBP/Blueprints/ThirdPersonCharacter.ThirdPersonCharacter_C"))
  (set `self.Character` _returnvalue))

(event `self.ReceiveTick`
  (params (DeltaSeconds :type "Float (single-precision)"))
  (bind _p_laser_hit (`self.P_Laser_Hit`))
  (bind _lasereyes (`self.LaserEyes`))
  (bind _starttrace (`self.StartTrace`))
  (bind _output_get (set `self.StartTrace` (`self.K2_GetActorLocation` _lasereyes)))
  (bind _output_get_2 (set `self.ShootDir` (`KismetMathLibrary.Conv_RotatorToVector` (`self.K2_GetActorRotation` _lasereyes))))
  (bind _outhit (`KismetSystemLibrary.LineTraceSingle` (+ (* _output_get_2 (`KismetMathLibrary.Dot_VectorVector` (- (`self.K2_GetActorLocation`) _output_get) _output_get_2)) _starttrace) (+ _starttrace (* _output_get_2 (`self.WeaponRange`))) "TraceTypeQuery1"))
  (bind (_bblockinghit _binitialoverlap _time _distance _location _impactpoint _normal _impactnormal _physmat _hitactor _hitcomponent _hitbonename _hititem _faceindex _tracestart _traceend) (`GameplayStatics.BreakHitResult` _outhit))
  (bind _returnvalue (`KismetSystemLibrary.IsValid` _hitcomponent))
  (`FXSystemComponent.SetVectorParameter` (`self.Laser`) "User.BeamEnd" (`KismetMathLibrary.SelectVector` _impactpoint _traceend _returnvalue))
  (if _returnvalue
    (`|ExecutionSequence`
      (:`then_0`
        (`FXSystemComponent.SetVectorParameter` _p_laser_hit "User.HitLocation" _impactpoint)
        (`/Engine/EditorBlueprintResources/StandardMacros.DoOnce` false :!label _label
          (:`Completed`
            (if (not (`self.End`))
              (`ActorComponent.Activate` (`self.P_Laser_Hit`) false)))))
      (:`then_1`
        (goto _label_2 :!via `Reset`))
      (:`then_2`
        (if (`ActorComponent.ComponentHasTag` _hitcomponent "PlayerMesh")
          (`/Game/ThirdPersonBP/Blueprints/ThirdPersonCharacter.LaserDamage` (`self.Character`)))))
    (else
      (`/Engine/EditorBlueprintResources/StandardMacros.DoOnce` false :!label _label_2
        (:`Completed`
          (`ActorComponent.Deactivate` _p_laser_hit)
          (goto _label :!via `Reset`))))))

(event `StopLaser`
  (`/Engine/EditorBlueprintResources/StandardMacros.DoOnce` false
    (:`Completed`
      (`ActorComponent.Deactivate` (`self.Laser`))
      (`ActorComponent.Deactivate` (`self.P_Weapon_Fire`))
      (set `self.End` true)
      (`ActorComponent.Deactivate` (`self.P_Laser_Hit`))
      (bind (_direction _scale) (`Timeline|StopEffect` :!via `PlayFromStart`)
        (:`Update`
          (`FXSystemComponent.SetFloatParameter` (`self.Laser`) "User.Scale" _scale))
        (:`Finished`
          (`self.K2_DestroyActor`))))))

(fn `UserConstructionScript`)