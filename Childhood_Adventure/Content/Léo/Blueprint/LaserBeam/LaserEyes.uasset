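; LaserEyes is an actor that charges and fires a laser from its Arrow component and can turn to track the player.
; On BeginPlay it attaches a ChargeProjectile, then after a delay spawns an attached BP_Laser unless the charge was cancelled.
; DispawnLaser cancels the charge and stops any active laser, while SpawnLaser is empty.
; Once Lookplayer is called, Tick rotates the actor toward the player character every frame.
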(event `self.ReceiveBeginPlay`
  (bind _laser (`self.Laser`))
  (bind _arrow (`self.Arrow`))
  (bind _arrow_2 (`self.Arrow`))
  (set `self.SetCharge` true)
  (bind _returnvalue (`|SpawnActorFromClass` "/Game/Léo/Blueprint/ChargeProjectiles/ChargeProjectile.ChargeProjectile_C" (`KismetMathLibrary.MakeTransform` (`SceneComponent.K2_GetComponentLocation` _arrow) (`SceneComponent.K2_GetComponentRotation` _arrow)) "Undefined" "OverrideRootScale" null null))
  (`self.K2_AttachToComponent` _returnvalue _arrow "None" "SnapToTarget" "SnapToTarget" "KeepRelative" true)
  (`KismetSystemLibrary.Delay` 5.0)
  (if (`self.SetCharge`)
    (`/Engine/EditorBlueprintResources/StandardMacros.DoOnce` false :!label _label
      (:`Completed`
        (`/Engine/EditorBlueprintResources/StandardMacros.IsValid` _laser
          (:`Is Valid`
            (`/Game/Léo/Blueprint/LaserBeam/BP_Laser.StopLaser` _laser))
          (:`Is Not Valid`
            _))
        (bind _returnvalue_2 (`|SpawnActorFromClass` "/Game/Léo/Blueprint/LaserBeam/BP_Laser.BP_Laser_C" (`KismetMathLibrary.MakeTransform` (`SceneComponent.K2_GetComponentLocation` _arrow_2) (`SceneComponent.K2_GetComponentRotation` _arrow_2)) "Undefined" "OverrideRootScale" null self null))
        (bind _output_get (set `self.Laser` _returnvalue_2))
        (`self.K2_AttachToComponent` _output_get (`self.Arrow`) "None" "SnapToTarget" "SnapToTarget" "KeepRelative" true)))))

(event `SpawnLaser`)

(event `DispawnLaser`
  (bind _laser (`self.Laser`))
  (set `self.SetCharge` false)
  (`/Engine/EditorBlueprintResources/StandardMacros.IsValid` _laser
    (:`Is Valid`
      (`/Game/Léo/Blueprint/LaserBeam/BP_Laser.StopLaser` _laser)
      (goto _label :!via `Reset`))))

(event `Look player`
  (set `self.LookPlayer` true))

(event `self.ReceiveTick`
  (params (DeltaSeconds :type "Float (single-precision)"))
  (if (`self.LookPlayer`)
    (`self.K2_SetActorRotation` (`KismetMathLibrary.FindLookAtRotation` (`self.K2_GetActorLocation`) (`self.K2_GetActorLocation` (`GameplayStatics.GetPlayerCharacter` 0))))))

(fn `UserConstructionScript`)