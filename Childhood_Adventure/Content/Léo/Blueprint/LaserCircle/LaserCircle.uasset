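; LaserCircle is a temporary actor carrying eight LaserEyes, which it spawns and attaches to its sphere components on BeginPlay.
; A timeline raises the actor, then two timelines run together: one spins it toward 360 yaw, the other moves two groups of four spheres vertically in opposite directions.
; When the spin finishes, it stops every laser, dissolves the eyes and destroys itself after short delays.
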(event `self.ReceiveBeginPlay`
  (bind _returnvalue (`self.K2_GetActorLocation`))
  (bind _relativelocation (`SceneComponent.RelativeLocation` (`self.Sphere1`)))
  (set `self.Up` (+ _relativelocation (0.0 0.0 40.0)))
  (set `self.Down` (- _relativelocation (0.0 0.0 40.0)))
  (set `self.Init` _relativelocation)
  (set `self.LaserEyesPosition` (`|MakeArray` (`self.Sphere1`) (`self.Sphere2`) (`self.Sphere3`) (`self.Sphere4`) (`self.Sphere5`) (`self.Sphere6`) (`self.Sphere7`) (`self.Sphere8`)))
  (set `self.Eyes_Location` (`|MakeArray` (`SceneComponent.K2_GetComponentLocation` (`self.Sphere1`)) (`SceneComponent.K2_GetComponentLocation` (`self.Sphere2`)) (`SceneComponent.K2_GetComponentLocation` (`self.Sphere3`)) (`SceneComponent.K2_GetComponentLocation` (`self.Sphere4`)) (`SceneComponent.K2_GetComponentLocation` (`self.Sphere5`)) (`SceneComponent.K2_GetComponentLocation` (`self.Sphere6`)) (`SceneComponent.K2_GetComponentLocation` (`self.Sphere7`)) (`SceneComponent.K2_GetComponentLocation` (`self.Sphere8`))))
  (set `self.Eyes_Rotation` (`|MakeArray` (`SceneComponent.K2_GetComponentRotation` (`self.Arrow1`)) (`SceneComponent.K2_GetComponentRotation` (`self.Arrow2`)) (`SceneComponent.K2_GetComponentRotation` (`self.Arrow3`)) (`SceneComponent.K2_GetComponentRotation` (`self.Arrow4`)) (`SceneComponent.K2_GetComponentRotation` (`self.Arrow5`)) (`SceneComponent.K2_GetComponentRotation` (`self.Arrow6`)) (`SceneComponent.K2_GetComponentRotation` (`self.Arrow7`)) (`SceneComponent.K2_GetComponentRotation` (`self.Arrow8`))))
  (bind _output_get (set `self.ActorRotation A` (`self.K2_GetActorRotation`)))
  (set `self.ActorRotation B` (`KismetMathLibrary.MakeRotator` (.roll _output_get) (.pitch _output_get) 360.0))
  (`|ExecutionSequence`
    (:`then_1`
      (for (_array_element _array_index) (`self.LaserEyesPosition`)
        (bind _returnvalue_2 (`|SpawnActorFromClass` "/Game/Léo/Blueprint/LaserBeam/LaserEyes.LaserEyes_C" (`KismetMathLibrary.MakeTransform` (`|GetArrayItem` (`self.Eyes_Location`) _array_index) (`|GetArrayItem` (`self.Eyes_Rotation`) _array_index) (0.2 0.2 0.2)) "AlwaysSpawn" "OverrideRootScale" null null))
        (`KismetArrayLibrary.Array_Add` (`self.LaserEyesObject`) _returnvalue_2)
        (`self.K2_AttachToComponent` _returnvalue_2 _array_element "None" "SnapToTarget" "SnapToTarget" "KeepWorld" true)))
    (:`then_3`
      (set `self.Actor position` _returnvalue)
      (set `self.Actor End Position` (+ _returnvalue (0.0 0.0 100.0)))
      (bind (_direction _newtrack_0) (`Timeline|Timeline_1`)
        (:`Update`
          (`self.K2_SetActorLocation` (`KismetMathLibrary.VLerp` (`self.Actor position`) (`self.Actor End Position`) _newtrack_0)))
        (:`Finished`
          (`|ExecutionSequence`
            (:`then_0`
              (bind (_direction_2 _newtrack_0_2) (`Timeline|UpDown` :!via `PlayFromStart`)
                (:`Update`
                  (`|ExecutionSequence`
                    (:`then_0`
                      (`|ExecutionSequence`
                        (:`then_0`
                          (bind (_returnvalue_x _returnvalue_y _returnvalue_z) (`KismetMathLibrary.BreakVector` (`KismetMathLibrary.VLerp` (`self.Init`) (`self.Up`) _newtrack_0_2)))
                          (`self.MoveUpDown` (`self.Sphere1`) _returnvalue_z))
                        (:`then_1`
                          (`self.MoveUpDown` (`self.Sphere3`) _returnvalue_z))
                        (:`then_2`
                          (`self.MoveUpDown` (`self.Sphere4`) _returnvalue_z))
                        (:`then_3`
                          (`self.MoveUpDown` (`self.Sphere7`) _returnvalue_z))))
                    (:`then_1`
                      (`|ExecutionSequence`
                        (:`then_0`
                          (bind (_returnvalue_x_2 _returnvalue_y_2 _returnvalue_z_2) (`KismetMathLibrary.BreakVector` (`KismetMathLibrary.VLerp` (`self.Init`) (`self.Down`) _newtrack_0_2)))
                          (`self.MoveUpDown` (`self.Sphere2`) _returnvalue_z_2))
                        (:`then_1`
                          (`self.MoveUpDown` (`self.Sphere5`) _returnvalue_z_2))
                        (:`then_2`
                          (`self.MoveUpDown` (`self.Sphere6`) _returnvalue_z_2))
                        (:`then_3`
                          (`self.MoveUpDown` (`self.Sphere8`) _returnvalue_z_2))))))))
            (:`then_1`
              (bind (_direction_3 _newtrack_0_3) (`Timeline|Timeline_0` :!via `PlayFromStart`)
                (:`Update`
                  (`self.K2_SetActorRotation` (`KismetMathLibrary.RLerp` (`self.ActorRotation A`) (`self.ActorRotation B`) _newtrack_0_3)))
                (:`Finished`
                  (for _array_element_2 (`self.LaserEyesObject`)
                    (`/Game/Léo/Blueprint/LaserBeam/BP_Laser.StopLaser` (`/Game/Léo/Blueprint/LaserBeam/LaserEyes.Laser` _array_element_2)))
                  (`KismetSystemLibrary.Delay` 0.5)
                  (for _array_element_3 (`self.LaserEyesObject`)
                    (`/Game/Léo/Blueprint/LaserBeam/LaserEyes.Disolve` _array_element_3))
                  (`KismetSystemLibrary.Delay` 1.0)
                  (`self.K2_DestroyActor`))))))))))

(event `Relaunch`)

(fn `UserConstructionScript`)