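; ExplosionLaser is a short-lived explosion actor for laser projectiles that applies physics impulses and damage.
; Shortly after spawning it fires two radial force impulses, then destroys itself half a second later.
; Its overlap sphere checks component tags to deal damage to the two Wall_Eyes_Bomber variants and to apply explosion damage to the ThirdPersonCharacter.
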(event `self.ReceiveBeginPlay`
  (`KismetSystemLibrary.Delay` 0.1)
  (`|ExecutionSequence`
    (:`then_0`
      (`RadialForceComponent.FireImpulse` (`self.RadialForce`))
      (`KismetSystemLibrary.Delay` 0.5)
      (`self.K2_DestroyActor`))
    (:`then_1`
      (`RadialForceComponent.FireImpulse` (`self.RadialForce1`)))))

(event `self.Sphere.OnComponentBeginOverlap`
  (params (OverlappedComponent :type "PrimitiveComponent Object Reference") (OtherActor :type "Actor Object Reference") (OtherComp :type "PrimitiveComponent Object Reference") (OtherBodyIndex :type Integer) (bFromSweep :type Boolean) (SweepResult :type "HitResult Structure (by ref)"))
  (`|ExecutionSequence`
    (:`then_0`
      (if (`ActorComponent.ComponentHasTag` OtherComp "WallTarget")
        (bind _aswall_eyes_bomber (cast `/Game/Léo/Blueprint/Wall/Wall_Eyes_Bomber` OtherActor))
        (`/Game/Léo/Blueprint/Wall/Wall_Eyes_Bomber.Deal_Damage` _aswall_eyes_bomber)))
    (:`then_1`
      (if (`ActorComponent.ComponentHasTag` OtherComp "PlayerCapsule")
        (bind _asthird_person_character (cast `/Game/ThirdPersonBP/Blueprints/ThirdPersonCharacter` OtherActor))
        (`/Game/ThirdPersonBP/Blueprints/ThirdPersonCharacter.ExplosionDamage` _asthird_person_character)))
    (:`then_2`
      (if (`ActorComponent.ComponentHasTag` OtherComp "WallTargetDroit")
        (bind _aswall_eyes_bomber_2 (cast `/Game/Léo/Blueprint/Wall/Wall_Eyes_Bomber_2` OtherActor))
        (`/Game/Léo/Blueprint/Wall/Wall_Eyes_Bomber_2.Deal_Damage` _aswall_eyes_bomber_2)))))

(fn `UserConstructionScript`)