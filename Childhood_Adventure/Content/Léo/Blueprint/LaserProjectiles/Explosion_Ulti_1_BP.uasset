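; Explosion_Ulti_1_BP is a short-lived explosion actor among the laser projectile Blueprints that damages the player.
; On BeginPlay it plays an impact sound at its Sphere's location, then destroys itself after a brief delay.
; During that window, a Sphere overlap with a component tagged PlayerCapsule calls ProjectileDamage on the ThirdPersonCharacter, gated by DoOnce so each explosion hits only once.
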(event `self.ReceiveBeginPlay`
  (`GameplayStatics.PlaySoundAtLocation` "/Game/Sounds/News/projectile_impact_Cue.projectile_impact_Cue" (`SceneComponent.K2_GetComponentLocation` (`self.Sphere`)) (struct) 0.5 1.0 0.0 null null null)
  (`KismetSystemLibrary.Delay` 0.2)
  (`self.K2_DestroyActor`))

(event `self.Sphere.OnComponentBeginOverlap`
  (params (OverlappedComponent :type "PrimitiveComponent Object Reference") (OtherActor :type "Actor Object Reference") (OtherComp :type "PrimitiveComponent Object Reference") (OtherBodyIndex :type Integer) (bFromSweep :type Boolean) (SweepResult :type "HitResult Structure (by ref)"))
  (if (`ActorComponent.ComponentHasTag` OtherComp "PlayerCapsule")
    (bind _asthird_person_character (cast `/Game/ThirdPersonBP/Blueprints/ThirdPersonCharacter` OtherActor))
    (`/Engine/EditorBlueprintResources/StandardMacros.DoOnce` false
      (:`Completed`
        (`/Game/ThirdPersonBP/Blueprints/ThirdPersonCharacter.ProjectileDamage` _asthird_person_character)))))

(fn `UserConstructionScript`)