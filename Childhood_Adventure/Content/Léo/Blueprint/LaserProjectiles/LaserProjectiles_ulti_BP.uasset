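; Laser projectile actor for an ultimate attack that damages the player or explodes on level geometry.
; On BeginPlay it starts its Niagara trail and caches the player's ThirdPersonCharacter.
; A capsule overlap with the player calls ProjectileDamage, while one with a tagged wall or floor spawns an Explosion_Ulti_1_BP.
; Either hit stops the trail, plays hit effects at the impact point and destroys the actor after a one-second delay.
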(event `self.ReceiveBeginPlay`
  (`ActorComponent.Activate` (`self.Niagara`) false)
  (bind _asthird_person_character (cast `/Game/ThirdPersonBP/Blueprints/ThirdPersonCharacter` (`GameplayStatics.GetPlayerCharacter` 0)))
  (set `self.Character` _asthird_person_character))

(event `self.Capsule.OnComponentBeginOverlap`
  (params (OverlappedComponent :type "PrimitiveComponent Object Reference") (OtherActor :type "Actor Object Reference") (OtherComp :type "PrimitiveComponent Object Reference") (OtherBodyIndex :type Integer) (bFromSweep :type Boolean) (SweepResult :type "HitResult Structure (by ref)"))
  (bind _returnvalue (`self.K2_GetActorLocation`))
  (bind _hiteffects (`self.Hiteffects`))
  (bind _hiteffects_2 (`self.Hiteffects`))
  (if (`ActorComponent.ComponentHasTag` OtherComp "PlayerCapsule")
    (`ActorComponent.Deactivate` (`self.Niagara`))
    (`/Game/ThirdPersonBP/Blueprints/ThirdPersonCharacter.ProjectileDamage` (`self.Character`))
    (`ActorComponent.SetActive` _hiteffects_2 true false)
    (`SceneComponent.K2_SetWorldLocation` _hiteffects_2 (`self.K2_GetActorLocation`) false false)
    (`KismetSystemLibrary.Delay` 1.0)
    (`self.K2_DestroyActor`)
    (elif (or (`ActorComponent.ComponentHasTag` OtherComp "Wall") (`ActorComponent.ComponentHasTag` OtherComp "Floor"))
      (`ActorComponent.Deactivate` (`self.Niagara`))
      (`ActorComponent.SetActive` _hiteffects true false)
      (`SceneComponent.K2_SetWorldLocation` _hiteffects _returnvalue false false)
      (`|SpawnActorFromClass` "/Game/Léo/Blueprint/LaserProjectiles/Explosion_Ulti_1_BP.Explosion_Ulti_1_BP_C" (`KismetMathLibrary.MakeTransform` _returnvalue) "Undefined" "OverrideRootScale" null null)
      (`KismetSystemLibrary.Delay` 1.0)
      (`self.K2_DestroyActor`))))

(fn `UserConstructionScript`)