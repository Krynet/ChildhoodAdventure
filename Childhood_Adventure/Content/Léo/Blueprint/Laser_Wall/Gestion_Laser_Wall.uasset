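; Manager that triggers fire spawns on randomly chosen laser walls in the level.
; On BeginPlay it caches all Laser_Wall_BP actors, waits briefly, then calls SpawnFire on a random entry.
; After each delay, Launch_Capacity increments a counter and loops back until the limit is passed.
; The random index's upper bound is the list length, so it can land one past the last wall.
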(event `self.ReceiveBeginPlay`
  (bind _list (`self.List`))
  (bind _outactors (`GameplayStatics.GetAllActorsOfClass` "/Game/Léo/Blueprint/Laser_Wall/Laser_Wall_BP.Laser_Wall_BP_C"))
  (set `self.List` _outactors)
  (`KismetSystemLibrary.Delay` 5.0)
  (`/Game/Léo/Blueprint/Laser_Wall/Laser_Wall_BP.Spawn&Fire` (`|GetArrayItem` _list (`KismetMathLibrary.RandomIntegerInRange` 0 (`KismetArrayLibrary.Array_Length` _list))) :!label _label)
  (`KismetSystemLibrary.Delay` 3.0)
  (`self.Launch_Capacity`))

(event `Launch_Capacity`
  (bind _count (`self.Count`))
  (`/Engine/EditorBlueprintResources/StandardMacros.IncrementInt` _count
    (:`  `
      (if (<= _count 5)
        (goto _label)))))

(fn `UserConstructionScript`)