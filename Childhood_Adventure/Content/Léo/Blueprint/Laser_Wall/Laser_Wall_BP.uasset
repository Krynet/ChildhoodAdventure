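; Laser_Wall_BP is a wall actor that fires lasers from a fixed set of emission points.
; On BeginPlay it gathers its many sphere components into a location list.
; The Spawn&Fire event loops over that list and spawns a Wall_Eyes_Laser actor at each sphere's world location.
; Nothing in this Blueprint calls Spawn&Fire itself.
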(event `self.ReceiveBeginPlay`
  (set `self.Location_List` (`|MakeArray` (`self.Sphere16`) (`self.Sphere`) (`self.Sphere1`) (`self.Sphere2`) (`self.Sphere3`) (`self.Sphere4`) (`self.Sphere5`) (`self.Sphere6`) (`self.Sphere7`) (`self.Sphere8`) (`self.Sphere9`) (`self.Sphere10`) (`self.Sphere11`) (`self.Sphere12`) (`self.Sphere13`) (`self.Sphere14`) (`self.Sphere15`) (`self.Sphere34`) (`self.Sphere17`) (`self.Sphere18`) (`self.Sphere19`) (`self.Sphere20`) (`self.Sphere21`) (`self.Sphere22`) (`self.Sphere23`) (`self.Sphere24`) (`self.Sphere25`) (`self.Sphere26`) (`self.Sphere27`) (`self.Sphere28`) (`self.Sphere29`) (`self.Sphere30`) (`self.Sphere31`) (`self.Sphere32`) (`self.Sphere33`))))

(event `Spawn&Fire`
  (for _array_element (`self.Location_List`)
    (`|SpawnActorFromClass` "/Game/Léo/Blueprint/Laser_Wall/Wall_Eyes_Laser.Wall_Eyes_Laser_C" (`KismetMathLibrary.MakeTransform` (`SceneComponent.K2_GetComponentLocation` _array_element)) "Undefined" "OverrideRootScale" null null)))

(fn `UserConstructionScript`)