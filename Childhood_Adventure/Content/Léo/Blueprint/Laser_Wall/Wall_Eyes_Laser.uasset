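; Short-lived laser emitter actor, apparently a wall eye, that charges, fires once and then removes itself.
; On BeginPlay it spawns a Charge_Projectile_Observer at Sphere1 with the Arrow's rotation and snaps it to that sphere.
; After a delay it spawns a LaserProjectiles_BP from the sphere's location along the Arrow's rotation, then destroys itself shortly afterward.
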(event `self.ReceiveBeginPlay`
  (`self.Charge_Event`)
  (`KismetSystemLibrary.Delay` 2.0)
  (`self.Fire_Event`)
  (`KismetSystemLibrary.Delay` 1.0)
  (`self.K2_DestroyActor`))

(event `Charge_Event`
  (bind _returnvalue (`|SpawnActorFromClass` "/Game/Léo/Blueprint/Observer/Charge_Projectile_Observer.Charge_Projectile_Observer_C" (`KismetMathLibrary.MakeTransform` (`SceneComponent.K2_GetComponentLocation` (`self.Sphere1`)) (`SceneComponent.K2_GetComponentRotation` (`self.Arrow`))) "Undefined" "OverrideRootScale" null null))
  (`self.K2_AttachToComponent` _returnvalue (`self.Sphere1`) "None" "SnapToTarget" "SnapToTarget" "KeepWorld" true))

(event `Fire_Event`
  (`|SpawnActorFromClass` "/Game/Léo/Blueprint/LaserProjectiles/LaserProjectiles_BP.LaserProjectiles_BP_C" (`KismetMathLibrary.MakeTransform` (`SceneComponent.K2_GetComponentLocation` (`self.Sphere1`)) (`SceneComponent.K2_GetComponentRotation` (`self.Arrow`))) "Undefined" "OverrideRootScale" null null))

(fn `UserConstructionScript`)