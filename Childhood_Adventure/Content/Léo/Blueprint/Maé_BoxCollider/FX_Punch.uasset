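; FX_Punch is a short-lived punch effect actor with a particle system and a capsule for hit detection.
; On spawn it briefly plays, deactivates its particles, then destroys itself after a second short delay.
; If the capsule first overlaps a component tagged HitFX, it spawns FX_Punch_Explode at its own location and rotation, once only, then destroys itself shortly after.
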(event `self.ReceiveBeginPlay`
  (`KismetSystemLibrary.Delay` 0.2)
  (`ActorComponent.Deactivate` (`self.ParticleSystem`))
  (`KismetSystemLibrary.Delay` 0.2)
  (`self.K2_DestroyActor`))

(event `self.Capsule.OnComponentBeginOverlap`
  (params (OverlappedComponent :type "PrimitiveComponent Object Reference") (OtherActor :type "Actor Object Reference") (OtherComp :type "PrimitiveComponent Object Reference") (OtherBodyIndex :type Integer) (bFromSweep :type Boolean) (SweepResult :type "HitResult Structure (by ref)"))
  (if (`ActorComponent.ComponentHasTag` OtherComp "HitFX")
    (`/Engine/EditorBlueprintResources/StandardMacros.DoOnce` false
      (:`Completed`
        (`|SpawnActorFromClass` "/Game/Léo/Blueprint/Maé_BoxCollider/FX_Punch_Explode.FX_Punch_Explode_C" (`KismetMathLibrary.MakeTransform` (`self.K2_GetActorLocation`) (`self.K2_GetActorRotation`)) "Undefined" "OverrideRootScale" null null)
        (`KismetSystemLibrary.Delay` 0.1)
        (`self.K2_DestroyActor`)))))

(fn `UserConstructionScript`)