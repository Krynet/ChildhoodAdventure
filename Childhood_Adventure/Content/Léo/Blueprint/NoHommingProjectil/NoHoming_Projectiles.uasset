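; NoHoming_Projectiles is a projectile actor driven by ProjectileMovement that destroys itself after ten seconds.
; BeginPlay sets a homing acceleration and looks up the ThirdPersonCharacter, but never assigns a homing target in the graph.
; When its Capsule overlaps a component tagged DestroyProjectil, it spawns Projectile_Explosion_BP slightly below its root and destroys itself after a brief delay.
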(event `self.ReceiveBeginPlay`
  (`GameplayStatics.GetActorOfClass` "/Game/ThirdPersonBP/Blueprints/ThirdPersonCharacter.ThirdPersonCharacter_C")
  (set `ProjectileMovementComponent.HomingAccelerationMagnitude` 1200.0 (`self.ProjectileMovement`))
  (`KismetSystemLibrary.Delay` 10.0)
  (`self.K2_DestroyActor`))

(event `self.Capsule.OnComponentBeginOverlap`
  (params (OverlappedComponent :type "PrimitiveComponent Object Reference") (OtherActor :type "Actor Object Reference") (OtherComp :type "PrimitiveComponent Object Reference") (OtherBodyIndex :type Integer) (bFromSweep :type Boolean) (SweepResult :type "HitResult Structure (by ref)"))
  (`|ExecutionSequence`
    (:`then_0`
      (if (`ActorComponent.ComponentHasTag` OtherComp "DestroyProjectil")
        (`|SpawnActorFromClass` "/Game/Léo/Blueprint/Boss/Boss_Phase_1/BOSS_BP/Homing_Projectiles/Projectile_Explosion_BP.Projectile_Explosion_BP_C" (`KismetMathLibrary.MakeTransform` (`KismetMathLibrary.MakeVector` (.x (`SceneComponent.K2_GetComponentLocation` (`self.DefaultSceneRoot`))) (.y (`SceneComponent.K2_GetComponentLocation` (`self.DefaultSceneRoot`))) (- (.z (`SceneComponent.K2_GetComponentLocation` (`self.DefaultSceneRoot`))) 100.0))) "Undefined" "OverrideRootScale" null null)
        (`KismetSystemLibrary.Delay` 0.02)
        (`self.K2_DestroyActor`)))))

(fn `UserConstructionScript`)