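; Observer is an enemy linked to Boss_Phase_1_BP that hops between nine boss location points, firing lasers while facing the player.
; A timeline lerps it to a random point, then it spawns an attached charge effect, fires after a delay and repeats until FireCount reaches its limit, then destroys itself.
; The differs-from-current check and the destination use separate random picks; the sphere bobbing timeline is unwired, leaving MoveUpDown empty.
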(event `self.ReceiveBeginPlay`
  (bind _relativelocation (`SceneComponent.RelativeLocation` (`self.Sphere`)))
  (bind _returnvalue (`GameplayStatics.GetActorOfClass` "/Game/Léo/Blueprint/Boss/Boss_Phase_1/BOSS_BP/Boss_Phase_1_BP.Boss_Phase_1_BP_C"))
  (bind _output_get (set `self.Boss` _returnvalue))
  (set `self.Location` (`|MakeArray` (`SceneComponent.K2_GetComponentLocation` (`/Game/Léo/Blueprint/Boss/Boss_Phase_1/BOSS_BP/Boss_Phase_1_BP.Location_0` _output_get)) (`SceneComponent.K2_GetComponentLocation` (`/Game/Léo/Blueprint/Boss/Boss_Phase_1/BOSS_BP/Boss_Phase_1_BP.Location_1` _output_get)) (`SceneComponent.K2_GetComponentLocation` (`/Game/Léo/Blueprint/Boss/Boss_Phase_1/BOSS_BP/Boss_Phase_1_BP.Location_2` _output_get)) (`SceneComponent.K2_GetComponentLocation` (`/Game/Léo/Blueprint/Boss/Boss_Phase_1/BOSS_BP/Boss_Phase_1_BP.Location_3` _output_get)) (`SceneComponent.K2_GetComponentLocation` (`/Game/Léo/Blueprint/Boss/Boss_Phase_1/BOSS_BP/Boss_Phase_1_BP.Location_4` _output_get)) (`SceneComponent.K2_GetComponentLocation` (`/Game/Léo/Blueprint/Boss/Boss_Phase_1/BOSS_BP/Boss_Phase_1_BP.Location_5` _output_get)) (`SceneComponent.K2_GetComponentLocation` (`/Game/Léo/Blueprint/Boss/Boss_Phase_1/BOSS_BP/Boss_Phase_1_BP.Location_6` _output_get)) (`SceneComponent.K2_GetComponentLocation` (`/Game/Léo/Blueprint/Boss/Boss_Phase_1/BOSS_BP/Boss_Phase_1_BP.Location_7` _output_get)) (`SceneComponent.K2_GetComponentLocation` (`/Game/Léo/Blueprint/Boss/Boss_Phase_1/BOSS_BP/Boss_Phase_1_BP.Location_8` _output_get))))
  (set `self.ActualyLocation` (`self.K2_GetActorLocation`))
  (set `self.SphereInitRelativeLocation` _relativelocation)
  (set `self.SphereEndRelativeLocation` (+ _relativelocation (0.0 0.0 20.0)))
  (`KismetSystemLibrary.Delay` 1.0)
  (bind _returnvalue_2 (`GameplayStatics.GetActorOfClass` "/Game/ThirdPersonBP/Blueprints/ThirdPersonCharacter.ThirdPersonCharacter_C"))
  (set `self.Player` _returnvalue_2)
  (set `self.SetLookPlayer` true)
  (`self.FindLocation`))

(event `FindLocation`
  (bind _actualylocation (`self.ActualyLocation`))
  (bind _location (`self.Location`))
  (bind _output (`|GetArrayItem` _location (`KismetMathLibrary.RandomInteger` (`KismetArrayLibrary.Array_Length` _location))))
  (if (!= _actualylocation _output)
    (set `self.EndLocation` _output)
    (bind (_direction _timeline) (`Timeline|MoveToLocation` :!via `PlayFromStart`)
      (:`Update`
        (`self.K2_SetActorLocation` (`KismetMathLibrary.VLerp` _actualylocation (`self.EndLocation`) _timeline)))
      (:`Finished`
        (`self.MoveUpDown`)
        (set `self.ActualyLocation` (`self.K2_GetActorLocation`))
        (`self.ChargeEvent`)
        (`KismetSystemLibrary.Delay` 2.0)
        (`self.FireEvent`)
        (`KismetSystemLibrary.Delay` 1.0)
        (if (< (`self.FireCount`) (`self.FireCountMax`))
          (`/Engine/EditorBlueprintResources/StandardMacros.IncrementInt` (`self.FireCount`)
            (:`  `
              (`self.FindLocation`)))
          (else
            (`self.K2_DestroyActor`)))))
    (else
      (`self.FindLocation`))))

(event `ChargeEvent`
  (bind _returnvalue (`|SpawnActorFromClass` "/Game/Léo/Blueprint/Observer/Charge_Projectile_Observer.Charge_Projectile_Observer_C" (`KismetMathLibrary.MakeTransform` (`SceneComponent.K2_GetComponentLocation` (`self.Sphere2`)) (`SceneComponent.K2_GetComponentRotation` (`self.Arrow`))) "Undefined" "OverrideRootScale" null null))
  (`self.K2_AttachToComponent` _returnvalue (`self.Sphere2`) "None" "SnapToTarget" "SnapToTarget" "KeepWorld" true))

(event `MoveUpDown`)

(event `FireEvent`
  (`|SpawnActorFromClass` "/Game/Léo/Blueprint/LaserProjectiles/LaserProjectiles_BP.LaserProjectiles_BP_C" (`KismetMathLibrary.MakeTransform` (`SceneComponent.K2_GetComponentLocation` (`self.Sphere2`)) (`SceneComponent.K2_GetComponentRotation` (`self.Arrow`))) "Undefined" "OverrideRootScale" null null))

(event `self.ReceiveTick`
  (params (DeltaSeconds :type "Float (single-precision)"))
  (if (`self.SetLookPlayer`)
    (`self.K2_SetActorRotation` (`KismetMathLibrary.FindLookAtRotation` (`self.K2_GetActorLocation`) (`SceneComponent.K2_GetComponentLocation` (`Character.CapsuleComponent` (`self.Player`)))))))

(fn `UserConstructionScript`)