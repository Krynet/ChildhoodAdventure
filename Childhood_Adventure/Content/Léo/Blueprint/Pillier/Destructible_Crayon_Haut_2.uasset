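; Destructible crayon pillar actor that breaks apart on spawn and then dissolves away.
; On BeginPlay it turns off gravity on its broken crayon mesh and fires a radial force impulse to scatter it.
; After a short delay it swaps in a dissolve material, drives a scalar parameter from a timeline, and destroys itself when the timeline finishes.
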(event `self.ReceiveBeginPlay`
  (`PrimitiveComponent.SetEnableGravity` (`self.crayon_cassé_bas_DM`) false)
  (`RadialForceComponent.FireImpulse` (`self.RadialForce`))
  (`KismetSystemLibrary.Delay` 3.0)
  (`|ExecutionSequence`
    (:`then_0`
      (`PrimitiveComponent.SetMaterial` (`self.crayon_cassé_bas_DM`) 0 (`self.Disolve_Crayon`))
      (bind (_direction _newtrack_0) (`Timeline|Timeline_0` :!via `PlayFromStart`)
        (:`Update`
          (`MeshComponent.SetScalarParameterValueOnMaterials` (`self.crayon_cassé_bas_DM`) (`self.Parameter Name`) _newtrack_0))
        (:`Finished`
          (`self.K2_DestroyActor`))))))

(fn `UserConstructionScript`)