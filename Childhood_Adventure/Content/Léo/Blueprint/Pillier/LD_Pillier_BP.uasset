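; LD_Pillier_BP is a punchable pillar that falls over once its life runs out.
; Its Box removes one life when a component tagged PunchBox overlaps it while the cached ThirdPersonCharacter's Punch flag is set.
; At zero life, a timeline's Fall track drives a rotation lerp of the Pillier component from the initial rotation to a FinalAngle pitch computed on BeginPlay.
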(event `self.ReceiveBeginPlay`
  (bind _returnvalue (`GameplayStatics.GetActorOfClass` "/Game/ThirdPersonBP/Blueprints/ThirdPersonCharacter.ThirdPersonCharacter_C"))
  (set `self.Player` _returnvalue)
  (set `self.Life` (`self.Life_Max`))
  (bind _output_get (set `self.InitRotation` (`self.K2_GetActorRotation`)))
  (set `self.EndRotation` (`KismetMathLibrary.MakeRotator` (.roll _output_get) (`self.FinalAngle`) (.yaw _output_get))))

(event `self.Box.OnComponentBeginOverlap`
  (params (OverlappedComponent :type "PrimitiveComponent Object Reference") (OtherActor :type "Actor Object Reference") (OtherComp :type "PrimitiveComponent Object Reference") (OtherBodyIndex :type Integer) (bFromSweep :type Boolean) (SweepResult :type "HitResult Structure (by ref)"))
  (if (`ActorComponent.ComponentHasTag` OtherComp "PunchBox")
    (if (`/Game/ThirdPersonBP/Blueprints/ThirdPersonCharacter.Punch` (`self.Player`))
      (`self.Deal_Damage`))))

(event `Deal_Damage`
  (bind _result (`/Engine/EditorBlueprintResources/StandardMacros.DecrementFloat` (`self.Life`))
    (:`  `
      (if (<= _result 0.0)
        (`self.Destroy_Pillar`)))))

(event `Destroy_Pillar`
  (bind (_direction _fall) (`Timeline|Timeline_0`)
    (:`Update`
      (`SceneComponent.K2_SetWorldRotation` (`self.Pillier`) (`KismetMathLibrary.RLerp` (`self.InitRotation`) (`self.EndRotation`) _fall) false false))))

(fn `UserConstructionScript`)