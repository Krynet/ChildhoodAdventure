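; Destructible pillar for the phase 1 boss fight that loses life when the player's punch box overlaps it.
; Each hit is reported to the Pillier_Gestion manager, and at zero life a timeline tips the pillar over.
; Once fallen, it notifies the manager, destroys its defenders, damages the boss and removes itself.
; A defend event spawns a Defenser_BP linked to the pillar and gives it a move target.
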(event `self.ReceiveBeginPlay`
  (bind _returnvalue (`GameplayStatics.GetActorOfClass` "/Game/ThirdPersonBP/Blueprints/ThirdPersonCharacter.ThirdPersonCharacter_C"))
  (set `self.Player` _returnvalue)
  (bind _returnvalue_2 (`GameplayStatics.GetActorOfClass` "/Game/Léo/Blueprint/Pillier/Pillier_Gestion.Pillier_Gestion_C"))
  (set `self.Gestion_Pillier` _returnvalue_2)
  (set `self.Life` (`self.Life_Max`))
  (bind _output_get (set `self.InitRotation` (`self.K2_GetActorRotation`)))
  (set `self.EndRotation` (`KismetMathLibrary.MakeRotator` (.roll _output_get) -90.0 (.yaw _output_get))))

(event `self.Box.OnComponentBeginOverlap`
  (params (OverlappedComponent :type "PrimitiveComponent Object Reference") (OtherActor :type "Actor Object Reference") (OtherComp :type "PrimitiveComponent Object Reference") (OtherBodyIndex :type Integer) (bFromSweep :type Boolean) (SweepResult :type "HitResult Structure (by ref)"))
  (if (`ActorComponent.ComponentHasTag` OtherComp "PunchBox")
    (if (`/Game/ThirdPersonBP/Blueprints/ThirdPersonCharacter.Punch` (`self.Player`))
      (`self.Deal_Damage`)
      (`/Game/Léo/Blueprint/Pillier/Pillier_Gestion.Add_Damage` (`self.Gestion_Pillier`) self))))

(event `Deal_Damage`
  (bind _result (`/Engine/EditorBlueprintResources/StandardMacros.DecrementFloat` (`self.Life`))
    (:`  `
      (if (<= _result 0.0)
        (`self.Destroy_Pillar`)))))

(event `Destroy_Pillar`
  (bind (_direction _fall) (`Timeline|Timeline_0`)
    (:`Update`
      (`SceneComponent.K2_SetWorldRotation` (`self.Pillier`) (`KismetMathLibrary.RLerp` (`self.InitRotation`) (`self.EndRotation`) _fall) false false))
    (:`Finished`
      (`/Game/Léo/Blueprint/Pillier/Pillier_Gestion.Pillier_Destroy` (`self.Gestion_Pillier`) self)
      (for _array_element (`self.List_Defense`)
        (`self.K2_DestroyActor` _array_element))
      (bind _returnvalue (`GameplayStatics.GetActorOfClass` "/Game/Léo/Blueprint/Boss/Boss_Phase_1/BOSS_BP/Boss_Phase_1_BP.Boss_Phase_1_BP_C"))
      (set `self.Boss` _returnvalue)
      (`/Game/Léo/Blueprint/Boss/Boss_Phase_1/BOSS_BP/Boss_Phase_1_BP.LD_Deal_Damage` (`self.Boss`))
      (`KismetSystemLibrary.Delay` 0.2)
      (`self.K2_DestroyActor`))))

(event `Defend_Pillar`
  (bind _returnvalue (`|SpawnActorFromClass` "/Game/Léo/Blueprint/Pillier/Defenser_BP.Defenser_BP_C" (`KismetMathLibrary.MakeTransform` (`SceneComponent.K2_GetComponentLocation` (`self.Spawn_Point`)) (`self.K2_GetActorRotation`)) "AlwaysSpawn" "OverrideRootScale" null null))
  (set `/Game/Léo/Blueprint/Pillier/Defenser_BP.Pillier` self _returnvalue)
  (`KismetArrayLibrary.Array_Add` (`self.List_Defense`) _returnvalue)
  (set `/Game/Léo/Blueprint/Pillier/Defenser_BP.MoveLocation` (`SceneComponent.K2_GetComponentLocation` (`self.End_Spawn`)) _returnvalue))

(fn `UserConstructionScript`)