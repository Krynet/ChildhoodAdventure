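; Test actor that periodically jumps to the Position marker actor farthest from player 0.
; On BeginPlay it caches all Position actors, waits, then starts the repeating Change event.
; Change scans the cached list for the greatest distance to the player's capsule, moves the actor to that marker's location, then resets the maximum and re-invokes itself after delays.
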(event `self.ReceiveBeginPlay`
  (bind _outactors (`GameplayStatics.GetAllActorsOfClass` "/Game/Léo/Blueprint/Position_Before_Ultim_2/Position.Position_C"))
  (set `self.Positions_List` _outactors)
  (`KismetSystemLibrary.Delay` 5.0)
  (`self.Change`))

(event `Change`
  (for _array_element (`self.Positions_List`)
    (if (== (`self.MaxDistance`) 0.0)
      (bind _returnvalue (`KismetMathLibrary.Vector_Distance` (`SceneComponent.K2_GetComponentLocation` (`/Game/Léo/Blueprint/Position_Before_Ultim_2/Position.DefaultSceneRoot` _array_element)) (`SceneComponent.K2_GetComponentLocation` (`Character.CapsuleComponent` (`GameplayStatics.GetPlayerCharacter` 0)))))
      (set `self.MaxDistance` _returnvalue :!label _label)
      (set `self.Target` _array_element)
      (elif (< (`self.MaxDistance`) _returnvalue)
        (goto _label))))
  (`self.K2_SetActorLocation` self (`SceneComponent.K2_GetComponentLocation` (`/Game/Léo/Blueprint/Position_Before_Ultim_2/Position.DefaultSceneRoot` (`self.Target`))) false false)
  (`KismetSystemLibrary.Delay` 1.0)
  (set `self.MaxDistance` 0.0)
  (`KismetSystemLibrary.Delay` 4.0)
  (`self.Change`))

(fn `UserConstructionScript`)