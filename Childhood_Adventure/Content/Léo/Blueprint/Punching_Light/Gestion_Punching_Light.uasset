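; Manager Blueprint that coordinates all Punching_Light_BP actors in the level, which it gathers at BeginPlay.
; LightAll calls FatLight and resets Count on every cached light, then after a short delay calls DestroyLittleLight on the calling actor.
; Add_Damage increments a hit counter shared across lights and, at a fixed threshold, resets it and calls Defense on the light passed in.
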(event `self.ReceiveBeginPlay`
  (bind _outactors (`GameplayStatics.GetAllActorsOfClass` "/Game/Léo/Blueprint/Punching_Light/Punching_Light_BP.Punching_Light_BP_C"))
  (set `self.All_Punching_Light` _outactors))

(event `Light All`
  (params (`Actor Call` :type "/Game/Léo/Blueprint/Punching_Light/Punching_Light_BP Object Reference"))
  (for _array_element (`self.All_Punching_Light`)
    (`/Game/Léo/Blueprint/Punching_Light/Punching_Light_BP.Fat Light` _array_element)
    (set `/Game/Léo/Blueprint/Punching_Light/Punching_Light_BP.Count` 0 _array_element))
  (`KismetSystemLibrary.Delay` 2.0)
  (`/Game/Léo/Blueprint/Punching_Light/Punching_Light_BP.Destroy Little Light` `Actor Call`))

(event `Add_Damage`
  (params (PunchingLight :type "/Game/Léo/Blueprint/Punching_Light/Punching_Light_BP Object Reference"))
  (bind _result (`/Engine/EditorBlueprintResources/StandardMacros.IncrementInt` (`self.hit`))
    (:`  `
      (if (>= _result 7)
        (set `self.hit` 0)
        (`/Game/Léo/Blueprint/Punching_Light/Punching_Light_BP.Defense` PunchingLight)))))

(fn `UserConstructionScript`)