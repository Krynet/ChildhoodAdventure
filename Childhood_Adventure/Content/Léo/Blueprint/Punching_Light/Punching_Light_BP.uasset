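; Punchable light actor that lights up in stages as the player punches it.
; Box overlaps tagged PunchBox during a player punch increment a counter, switching on sphere pairs via the material "Switch" parameter.
; The fourth hit calls LightAll on the Gestion_Punching_Light manager.
; FatLight animates the main sphere with two chained timelines, then switches off the six small spheres; DestroyFatLight hides those six.
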(event `self.ReceiveBeginPlay`
  (set `self.Light` (`|MakeArray` (`self.Sphere2`) (`self.Sphere3`) (`self.Sphere4`) (`self.Sphere5`) (`self.Sphere6`) (`self.Sphere1`))))

(event `self.Box.OnComponentBeginOverlap`
  (params (OverlappedComponent :type "PrimitiveComponent Object Reference") (OtherActor :type "Actor Object Reference") (OtherComp :type "PrimitiveComponent Object Reference") (OtherBodyIndex :type Integer) (bFromSweep :type Boolean) (SweepResult :type "HitResult Structure (by ref)"))
  (if (`ActorComponent.ComponentHasTag` OtherComp "PunchBox")
    (bind _asthird_person_character (cast `/Game/ThirdPersonBP/Blueprints/ThirdPersonCharacter` (`GameplayStatics.GetPlayerCharacter` 0)))
    (if (`/Game/ThirdPersonBP/Blueprints/ThirdPersonCharacter.Punch` _asthird_person_character)
      (`/Engine/EditorBlueprintResources/StandardMacros.IncrementInt` (`self.Count`)
        (:`  `
          (`self.PowerUp`))))))

(event `PowerUp`
  (if (== (`self.Count`) 1)
    (`|ExecutionSequence`
      (:`then_0`
        (`MeshComponent.SetScalarParameterValueOnMaterials` (`self.Sphere5`) "Switch" 1.0))
      (:`then_1`
        (`MeshComponent.SetScalarParameterValueOnMaterials` (`self.Sphere6`) "Switch" 1.0)))
    (elif (== (`self.Count`) 2)
      (`|ExecutionSequence`
        (:`then_0`
          (`MeshComponent.SetScalarParameterValueOnMaterials` (`self.Sphere3`) "Switch" 1.0))
        (:`then_1`
          (`MeshComponent.SetScalarParameterValueOnMaterials` (`self.Sphere4`) "Switch" 1.0)))
      (elif (== (`self.Count`) 3)
        (`|ExecutionSequence`
          (:`then_0`
            (`MeshComponent.SetScalarParameterValueOnMaterials` (`self.Sphere1`) "Switch" 1.0))
          (:`then_1`
            (`MeshComponent.SetScalarParameterValueOnMaterials` (`self.Sphere2`) "Switch" 1.0)))
        (elif (== (`self.Count`) 4)
          (bind _returnvalue (`GameplayStatics.GetActorOfClass` "/Game/Léo/Blueprint/Punching_Light/Gestion_Punching_Light.Gestion_Punching_Light_C"))
          (`/Game/Léo/Blueprint/Punching_Light/Gestion_Punching_Light.Light All` _returnvalue self))))))

(event `Fat Light`
  (bind (_direction _newtrack_0) (`Timeline|Timeline_0` :!via `PlayFromStart`)
    (:`Update`
      (`MeshComponent.SetScalarParameterValueOnMaterials` (`self.Sphere`) "Switch" _newtrack_0))
    (:`Finished`
      (bind (_direction_2 _newtrack_0_2) (`Timeline|Timeline_1` :!via `PlayFromStart`)
        (:`Update`
          (`MeshComponent.SetScalarParameterValueOnMaterials` (`self.Sphere`) "Switch" _newtrack_0_2))
        (:`Finished`
          (for _array_element (`self.Light`)
            (`MeshComponent.SetScalarParameterValueOnMaterials` _array_element "Switch" 0.0)))))))

(event `Destroy Fat Light`
  (for _array_element (`self.Light`)
    (`SceneComponent.SetHiddenInGame` _array_element true false)))

(fn `UserConstructionScript`)