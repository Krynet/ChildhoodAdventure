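; Punching-machine puzzle Blueprint that counts the player's punches and opens the way by destroying the Porte_Lumière_BP light door.
; A punch overlapping the box drives two cylinders through chained timelines, which later reverse to reset.
; Each hit switches one of twelve mini lights to a lit material until the count exceeds them.
; The machine then stops accepting hits, animates its big light's material and intensity, and removes the door.
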(event `self.ReceiveBeginPlay`
  (bind _output_get (set `self.Move_1_Init` (`SceneComponent.RelativeLocation` (`self.punch_machine2_pCylinder7`))))
  (set `self.Move_1_End` (+ _output_get (0.0 60.0 0.0)))
  (bind _output_get_2 (set `self.Move_2_Init` (`SceneComponent.RelativeLocation` (`self.punch_machine2_pCylinder4`))))
  (set `self.Move_2_End` (+ _output_get_2 (0.0 120.0 0.0)))
  (bind _returnvalue (`GameplayStatics.GetActorOfClass` "/Game/Léo/Blueprint/Punching_Light/Gestion_Punching_Light.Gestion_Punching_Light_C"))
  (set `self.Gestion_PL` _returnvalue)
  (set `self.Light` (`|MakeArray` (`self.MiniLight_1`) (`self.MiniLight_2`) (`self.MiniLight_3`) (`self.MiniLight_4`) (`self.MiniLight_5`) (`self.MiniLight_6`) (`self.MiniLight_7`) (`self.MiniLight_8`) (`self.MiniLight_9`) (`self.MiniLight_10`) (`self.MiniLight_11`) (`self.MiniLight_12`))))

(event `PowerUp`
  (if (> (+ (`self.Count`) 1) (`KismetArrayLibrary.Array_Length` (`self.Light`)))
    (`self.Fat Light`)
    (set `self.Can_be_hit` false)
    (else
      (`PrimitiveComponent.SetMaterial` (`|GetArrayItem` (`self.Light`) (`self.Count`)) 0 "/Game/Danial/Props/punchmachinparts/Materials/lumiere_montante.lumiere_montante"))))

(event `self.Box.OnComponentBeginOverlap`
  (params (OverlappedComponent :type "PrimitiveComponent Object Reference") (OtherActor :type "Actor Object Reference") (OtherComp :type "PrimitiveComponent Object Reference") (OtherBodyIndex :type Integer) (bFromSweep :type Boolean) (SweepResult :type "HitResult Structure (by ref)"))
  (if (`ActorComponent.ComponentHasTag` OtherComp "PunchBox")
    (bind _asthird_person_character (cast `/Game/ThirdPersonBP/Blueprints/ThirdPersonCharacter` (`GameplayStatics.GetPlayerCharacter` 0)))
    (if (`/Game/ThirdPersonBP/Blueprints/ThirdPersonCharacter.Punch` _asthird_person_character)
      (if (`self.Can_be_hit`)
        (`self.Launch`)
        (`/Engine/EditorBlueprintResources/StandardMacros.IncrementInt` (`self.Count`)
          (:`  `
            (`self.PowerUp`)))))))

(event `Launch`
  (if (`self.Hited`)
    (`|ExecutionSequence`
      (:`then_0`
        (bind (_direction _newtrack_0) (`Timeline|Timeline_2` :!label _label)
          (:`Update`
            (`SceneComponent.K2_SetRelativeLocation` (`self.punch_machine2_pCylinder7`) (`KismetMathLibrary.VLerp` (`self.Move_1_Init`) (`self.Move_1_End`) _newtrack_0) false false))
          (:`Finished`
            (if (`self.Restaure_Launched`)
              (set `self.Restaure_Launched` false)
              (elif (`self.Hited`)
                (bind (_direction_2 _newtrack_0_2) (`Timeline|Timeline_3` :!via `PlayFromStart` :!label _label_2)
                  (:`Update`
                    (`SceneComponent.K2_SetRelativeLocation` (`self.punch_machine2_pCylinder4`) (`KismetMathLibrary.VLerp` (`self.Move_2_Init`) (`self.Move_2_End`) _newtrack_0_2) false false))
                  (:`Finished`
                    (if (`self.Restaure_Launched`)
                      (goto _label :!via `ReverseFromEnd`)
                      (else
                        (set `self.Hited` false)
                        (`self.Restaure`)))))
                (else
                  (goto _label_2)))))))
      (:`then_1`
        (goto _label_2 :!via `Stop`)))
    (else
      (set `self.Hited` true)
      (goto _label :!via `PlayFromStart`))))

(event `Restaure`
  (set `self.Restaure_Launched` true)
  (`|ExecutionSequence`
    (:`then_0`
      (goto _label :!via `Stop`))
    (:`then_1`
      (goto _label_2 :!via `ReverseFromEnd`))))

(event `Fat Light`
  (`|ExecutionSequence`
    (:`then_0`
      (bind (_direction _newtrack_0 _newtrack_1) (`Timeline|Timeline_0` :!via `PlayFromStart`)
        (:`Update`
          (`|ExecutionSequence`
            (:`then_0`
              (`MeshComponent.SetScalarParameterValueOnMaterials` (`self.punch_machine2_pHelix2`) "BigLight" _newtrack_0))
            (:`then_1`
              (`LightComponent.SetIntensity` (`self.PointLight`) _newtrack_1))))
        (:`Finished`
          (`|ExecutionSequence`
            (:`then_0`
              (bind (_direction_2 _newtrack_0_2 _lightintensity) (`Timeline|Timeline_1` :!via `PlayFromStart`)
                (:`Update`
                  (`|ExecutionSequence`
                    (:`then_0`
                      (`MeshComponent.SetScalarParameterValueOnMaterials` (`self.punch_machine2_pHelix2`) "BigLight" _newtrack_0_2))
                    (:`then_1`
                      (`LightComponent.SetIntensity` (`self.PointLight`) _lightintensity))))))
            (:`then_1`
              (bind _returnvalue (`GameplayStatics.GetActorOfClass` "/Game/Léo/Blueprint/Generateur/Porte_Lumière_BP.Porte_Lumière_BP_C"))
              (`self.K2_DestroyActor` _returnvalue))))))
    (:`then_1`
      (`PrimitiveComponent.SetMaterial` (`self.punch_machine2_polySurface61`) 0 "/Game/Danial/Props/punchmachinparts/Materials/lumiere_montante.lumiere_montante"))))

(event `Destroy Little Light`
  (for _array_element (`self.Light`)
    (`SceneComponent.SetHiddenInGame` _array_element true false)))

(fn `UserConstructionScript`)