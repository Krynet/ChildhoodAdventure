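; Acid rain area-of-effect actor that showers random projectiles and damages the player standing inside it, apparently a boss attack.
; On BeginPlay, a self-calling, delayed spawn event drops projectiles at random points in a box, then destroys the actor after the set count.
; Cylinder overlaps with the tagged player capsule toggle a damage flag.
; Tick calls the character's AOEDamage while flagged and replays the rain sound behind a delay gate.
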(event `self.ReceiveBeginPlay`
  (bind _returnvalue (`GameplayStatics.GetActorOfClass` "/Game/ThirdPersonBP/Blueprints/ThirdPersonCharacter.ThirdPersonCharacter_C"))
  (set `self.Character` _returnvalue)
  (`self.Spawn_Projectile` 0))

(event `Spawn_Projectile`
  (params (Loop :type Integer))
  (bind _projectile_type (`self.Projectile_Type`))
  (bind _box (`self.Box`))
  (if (< Loop (`self.Nb_Projectiles`))
    (`|SpawnActorFromClass` (`|GetArrayItem` _projectile_type (`KismetMathLibrary.RandomIntegerInRange` 0 (`KismetArrayLibrary.Array_LastIndex` _projectile_type))) (`KismetMathLibrary.MakeTransform` (`KismetMathLibrary.RandomPointInBoundingBox` (`SceneComponent.K2_GetComponentLocation` _box) (`BoxComponent.GetScaledBoxExtent` _box)) (`SceneComponent.K2_GetComponentRotation` (`self.Arrow1`)) (0.1 0.1 0.1)) "AlwaysSpawn" "OverrideRootScale" null null)
    (`KismetSystemLibrary.Delay` (`self.SpawnRate`))
    (`self.Spawn_Projectile` (+ Loop 1))
    (else
      (`self.K2_DestroyActor`))))

(event `self.ReceiveTick`
  (params (DeltaSeconds :type "Float (single-precision)"))
  (if (not (`self.Raining`))
    (`GameplayStatics.PlaySoundAtLocation` "/Game/Sounds/News/boss_pluie_acide_Cue.boss_pluie_acide_Cue" (`SceneComponent.K2_GetComponentLocation` (`self.Mesh`)) (struct) 1.0 1.0 0.0 null null null)
    (set `self.Raining` true)
    (`KismetSystemLibrary.Delay` 2.0)
    (set `self.Raining` false))
  (if (`self.Deal_Damage`)
    (`/Game/ThirdPersonBP/Blueprints/ThirdPersonCharacter.AOE Damage` (`self.Character`))))

(event `self.Cylinder.OnComponentBeginOverlap`
  (params (OverlappedComponent :type "PrimitiveComponent Object Reference") (OtherActor :type "Actor Object Reference") (OtherComp :type "PrimitiveComponent Object Reference") (OtherBodyIndex :type Integer) (bFromSweep :type Boolean) (SweepResult :type "HitResult Structure (by ref)"))
  (if (`ActorComponent.ComponentHasTag` OtherComp "PlayerCapsule")
    (set `self.Deal_Damage` true)))

(event `self.Cylinder.OnComponentEndOverlap`
  (params (OverlappedComponent :type "PrimitiveComponent Object Reference") (OtherActor :type "Actor Object Reference") (OtherComp :type "PrimitiveComponent Object Reference") (OtherBodyIndex :type Integer))
  (if (`ActorComponent.ComponentHasTag` OtherComp "PlayerCapsule")
    (set `self.Deal_Damage` false)))

(fn `UserConstructionScript`)