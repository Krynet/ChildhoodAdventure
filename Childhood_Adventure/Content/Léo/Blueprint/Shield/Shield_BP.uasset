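; Shield actor that spawns as a short-lived sphere and triggers a radial push when it touches a player.
; On BeginPlay a timeline drives the sphere's uniform world scale between the Begin and End values, then destroys the actor when finished.
; Any component tagged PlayerCapsule that begins overlapping the sphere makes the RadialForce component fire an impulse.
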(event `self.ReceiveBeginPlay`
  (`|ExecutionSequence`
    (:`then_1`
      (bind (_direction _newtrack_1 _newtrack_0) (`Timeline|Timeline_0` :!via `PlayFromStart`)
        (:`Update`
          (`|ExecutionSequence`
            (:`then_0`
              (bind _returnvalue (* (`KismetMathLibrary.Lerp` (`self.Begin`) (`self.End`) _newtrack_0) 13.0))
              (`SceneComponent.SetWorldScale3D` (`self.Sphere`) (`KismetMathLibrary.MakeVector` _returnvalue _returnvalue _returnvalue)))))
        (:`Finished`
          (`self.K2_DestroyActor`))))))

(event `self.Sphere.OnComponentBeginOverlap`
  (params (OverlappedComponent :type "PrimitiveComponent Object Reference") (OtherActor :type "Actor Object Reference") (OtherComp :type "PrimitiveComponent Object Reference") (OtherBodyIndex :type Integer) (bFromSweep :type Boolean) (SweepResult :type "HitResult Structure (by ref)"))
  (if (`ActorComponent.ComponentHasTag` OtherComp "PlayerCapsule")
    (`RadialForceComponent.FireImpulse` (`self.RadialForce`))))

(fn `UserConstructionScript`)