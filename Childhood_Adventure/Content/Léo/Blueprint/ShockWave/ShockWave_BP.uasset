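; ShockWave_BP is an expanding shockwave actor that knocks back and damages the player, then destroys itself.
; On BeginPlay a timeline lerps between Begin and End to drive the Niagara effect's scale and opacity and grow a collision sphere in step.
; When the sphere first overlaps a component tagged PlayerCapsule while CanPush is true, a RadialForce impulse fires and BumpDamage is called on the ThirdPersonCharacter.
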(event `self.ReceiveBeginPlay`
  (bind (_direction _newtrack_0 _newtrack_1) (`Timeline|Timeline_0`)
    (:`Update`
      (`|ExecutionSequence`
        (:`then_0`
          (bind _returnvalue (`KismetMathLibrary.Lerp` (`self.Begin`) (`self.End`) _newtrack_0))
          (`FXSystemComponent.SetFloatParameter` (`self.ShockWave_FX`) "User.SphereScale" _returnvalue))
        (:`then_1`
          (`FXSystemComponent.SetFloatParameter` (`self.ShockWave_FX`) "User.GlobalOpacity" _newtrack_1))
        (:`then_2`
          (bind _returnvalue_2 (* _returnvalue 30.0))
          (`SceneComponent.SetRelativeScale3D` (`self.Sphere`) (`KismetMathLibrary.MakeVector` _returnvalue_2 _returnvalue_2 _returnvalue_2)))))
    (:`Finished`
      (set `self.Can_Push` false)
      (`self.K2_DestroyActor`))))

(event `self.Sphere.OnComponentBeginOverlap`
  (params (OverlappedComponent :type "PrimitiveComponent Object Reference") (OtherActor :type "Actor Object Reference") (OtherComp :type "PrimitiveComponent Object Reference") (OtherBodyIndex :type Integer) (bFromSweep :type Boolean) (SweepResult :type "HitResult Structure (by ref)"))
  (if (`ActorComponent.ComponentHasTag` OtherComp "PlayerCapsule")
    (if (`self.Can_Push`)
      (`/Engine/EditorBlueprintResources/StandardMacros.DoOnce` false
        (:`Completed`
          (`RadialForceComponent.FireImpulse` (`self.RadialForce`))
          (bind _asthird_person_character (cast `/Game/ThirdPersonBP/Blueprints/ThirdPersonCharacter` OtherActor))
          (`/Game/ThirdPersonBP/Blueprints/ThirdPersonCharacter.BumpDamage` _asthird_person_character))))))

(fn `UserConstructionScript`)