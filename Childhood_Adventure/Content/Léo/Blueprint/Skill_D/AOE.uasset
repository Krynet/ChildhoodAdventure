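; AOE is a self-destroying area-of-effect indicator actor in the Skill_D folder, showing a circumference and an animated area.
; On BeginPlay, its Circum and Area components each get a dynamic material instance, with the CircumArea scalar switching between outline and area.
; The AreaValue timeline drives the area material's AreaValue parameter, then the actor destroys itself after a short delay.
; It contains only visual logic, with no damage or overlap handling.
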(event `self.ReceiveBeginPlay`
  (`|ExecutionSequence`
    (:`then_0`
      (bind _returnvalue (`DecalComponent.CreateDynamicMaterialInstance` (`self.Circum`)))
      (bind _output_get (set `self.CircumRef` _returnvalue))
      (`MaterialInstanceDynamic.SetScalarParameterValue` _output_get "CircumArea" 1.0))
    (:`then_1`
      (bind _returnvalue_2 (`DecalComponent.CreateDynamicMaterialInstance` (`self.Area`)))
      (bind _output_get_2 (set `self.AreaRef` _returnvalue_2))
      (`MaterialInstanceDynamic.SetScalarParameterValue` _output_get_2 "CircumArea" 0.0))
    (:`then_2`
      (bind (_direction _newtrack_0) (`Timeline|AreaValue` :!via `PlayFromStart`)
        (:`Update`
          (`MaterialInstanceDynamic.SetScalarParameterValue` (`self.AreaRef`) "AreaValue" _newtrack_0))
        (:`Finished`
          (`KismetSystemLibrary.Delay` 0.2)
          (`self.K2_DestroyActor`))))))

(fn `UserConstructionScript`)