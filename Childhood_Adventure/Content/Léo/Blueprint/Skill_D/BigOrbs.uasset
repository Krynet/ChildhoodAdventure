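; BigOrbs is a skill actor that releases a burst of EyesDown actors toward a preset pattern of points.
; On BeginPlay it gathers the world positions of its many Sphere components and spawns one EyesDown per point from its center, facing that point and receiving it as NextPosition.
; A Delay inside the spawn loop leads to the orb destroying itself five seconds later.
; Tick keeps its Arrow pointed at the player character.
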(event `self.ReceiveBeginPlay`
  (bind _returnvalue (`self.K2_GetActorLocation`))
  (bind _asthird_person_character (cast `/Game/ThirdPersonBP/Blueprints/ThirdPersonCharacter` (`GameplayStatics.GetPlayerCharacter` 0)))
  (set `self.Character` _asthird_person_character)
  (bind _output_get (set `self.Locations` (`|MakeArray` (`SceneComponent.K2_GetComponentLocation` (`self.Sphere1`)) (`SceneComponent.K2_GetComponentLocation` (`self.Sphere2`)) (`SceneComponent.K2_GetComponentLocation` (`self.Sphere3`)) (`SceneComponent.K2_GetComponentLocation` (`self.Sphere4`)) (`SceneComponent.K2_GetComponentLocation` (`self.Sphere32`)) (`SceneComponent.K2_GetComponentLocation` (`self.Sphere7`)) (`SceneComponent.K2_GetComponentLocation` (`self.Sphere8`)) (`SceneComponent.K2_GetComponentLocation` (`self.Sphere9`)) (`SceneComponent.K2_GetComponentLocation` (`self.Sphere10`)) (`SceneComponent.K2_GetComponentLocation` (`self.Sphere11`)) (`SceneComponent.K2_GetComponentLocation` (`self.Sphere12`)) (`SceneComponent.K2_GetComponentLocation` (`self.Sphere13`)) (`SceneComponent.K2_GetComponentLocation` (`self.Sphere14`)) (`SceneComponent.K2_GetComponentLocation` (`self.Sphere15`)) (`SceneComponent.K2_GetComponentLocation` (`self.Sphere16`)) (`SceneComponent.K2_GetComponentLocation` (`self.Sphere17`)) (`SceneComponent.K2_GetComponentLocation` (`self.Sphere18`)) (`SceneComponent.K2_GetComponentLocation` (`self.Sphere19`)) (`SceneComponent.K2_GetComponentLocation` (`self.Sphere20`)) (`SceneComponent.K2_GetComponentLocation` (`self.Sphere21`)) (`SceneComponent.K2_GetComponentLocation` (`self.Sphere22`)) (`SceneComponent.K2_GetComponentLocation` (`self.Sphere23`)) (`SceneComponent.K2_GetComponentLocation` (`self.Sphere24`)) (`SceneComponent.K2_GetComponentLocation` (`self.Sphere25`)) (`SceneComponent.K2_GetComponentLocation` (`self.Sphere26`)) (`SceneComponent.K2_GetComponentLocation` (`self.Sphere27`)) (`SceneComponent.K2_GetComponentLocation` (`self.Sphere28`)) (`SceneComponent.K2_GetComponentLocation` (`self.Sphere29`)) (`SceneComponent.K2_GetComponentLocation` (`self.Sphere30`)) (`SceneComponent.K2_GetComponentLocation` (`self.Sphere31`)) (`SceneComponent.K2_GetComponentLocation` (`self.Sphere6`)) (`SceneComponent.K2_GetComponentLocation` (`self.Sphere33`)) (`SceneComponent.K2_GetComponentLocation` (`self.Sphere35`)) (`SceneComponent.K2_GetComponentLocation` (`self.Sphere36`)) (`SceneComponent.K2_GetComponentLocation` (`self.Sphere37`)) (`SceneComponent.K2_GetComponentLocation` (`self.Sphere34`)) (`SceneComponent.K2_GetComponentLocation` (`self.Sphere38`)) (`SceneComponent.K2_GetComponentLocation` (`self.Sphere39`)) (`SceneComponent.K2_GetComponentLocation` (`self.Sphere40`)) (`SceneComponent.K2_GetComponentLocation` (`self.Sphere41`)) (`SceneComponent.K2_GetComponentLocation` (`self.Sphere42`)) (`SceneComponent.K2_GetComponentLocation` (`self.Sphere43`)) (`SceneComponent.K2_GetComponentLocation` (`self.Sphere44`)) (`SceneComponent.K2_GetComponentLocation` (`self.Sphere45`)) (`SceneComponent.K2_GetComponentLocation` (`self.Sphere46`)) (`SceneComponent.K2_GetComponentLocation` (`self.Sphere47`)) (`SceneComponent.K2_GetComponentLocation` (`self.Sphere48`)) (`SceneComponent.K2_GetComponentLocation` (`self.Sphere49`)) (`SceneComponent.K2_GetComponentLocation` (`self.Sphere50`)) (`SceneComponent.K2_GetComponentLocation` (`self.Sphere51`)) (`SceneComponent.K2_GetComponentLocation` (`self.Sphere52`)) (`SceneComponent.K2_GetComponentLocation` (`self.Sphere53`)) (`SceneComponent.K2_GetComponentLocation` (`self.Sphere54`)) (`SceneComponent.K2_GetComponentLocation` (`self.Sphere55`)) (`SceneComponent.K2_GetComponentLocation` (`self.Sphere56`)) (`SceneComponent.K2_GetComponentLocation` (`self.Sphere57`)))))
  (bind _result (`/Engine/EditorBlueprintResources/StandardMacros.DecrementInt` (`KismetArrayLibrary.Array_Length` _output_get))
    (:`  `
      (for _index (range (+ _result 1))
        (bind _output (`|GetArrayItem` (`self.Locations`) _index))
        (bind _returnvalue_2 (`|SpawnActorFromClass` "/Game/Léo/Blueprint/Skill_D/EyesDown.EyesDown_C" (`KismetMathLibrary.MakeTransform` _returnvalue (`KismetMathLibrary.FindLookAtRotation` _returnvalue _output)) "AlwaysSpawn" "OverrideRootScale" null null))
        (set `/Game/Léo/Blueprint/Skill_D/EyesDown.NextPosition` _output _returnvalue_2)
        (`KismetSystemLibrary.Delay` 5.0)
        (`self.K2_DestroyActor`)))))

(event `self.ReceiveTick`
  (params (DeltaSeconds :type "Float (single-precision)"))
  (`SceneComponent.K2_SetWorldRotation` (`self.Arrow`) (`KismetMathLibrary.FindLookAtRotation` (`SceneComponent.K2_GetComponentLocation` (`self.Arrow`)) (`self.K2_GetActorLocation` (`self.Character`))) false false))

(fn `UserConstructionScript`)