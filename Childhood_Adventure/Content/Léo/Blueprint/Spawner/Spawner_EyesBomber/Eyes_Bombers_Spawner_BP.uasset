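; Spawner actor that fires Bomber_Projectiles_BP actors while the player is within its trigger sphere.
; Sphere overlap begin and end with a component tagged PlayerCapsule toggle the Active flag.
; A self-calling delay loop starts on BeginPlay and runs constantly, spawning a projectile at the actor's location along the Arrow's rotation on each pass when Active.
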(event `Spawn Eyes`
  (`KismetSystemLibrary.Delay` 5.0 :!label _label)
  (if (`self.Active`)
    (`|SpawnActorFromClass` "/Game/Léo/Blueprint/EyesBombers/Bomber_Projectiles_BP.Bomber_Projectiles_BP_C" (`KismetMathLibrary.MakeTransform` (`self.K2_GetActorLocation`) (`SceneComponent.K2_GetComponentRotation` (`self.Arrow`))) "Undefined" "OverrideRootScale" null null)
    (`self.Spawn Eyes`)
    (else
      (`self.Spawn Eyes`))))

(event `self.ReceiveBeginPlay`
  (goto _label))

(event `self.Sphere.OnComponentBeginOverlap`
  (params (OverlappedComponent :type "PrimitiveComponent Object Reference") (OtherActor :type "Actor Object Reference") (OtherComp :type "PrimitiveComponent Object Reference") (OtherBodyIndex :type Integer) (bFromSweep :type Boolean) (SweepResult :type "HitResult Structure (by ref)"))
  (if (`ActorComponent.ComponentHasTag` OtherComp "PlayerCapsule")
    (set `self.Active` true)))

(event `self.Sphere.OnComponentEndOverlap`
  (params (OverlappedComponent :type "PrimitiveComponent Object Reference") (OtherActor :type "Actor Object Reference") (OtherComp :type "PrimitiveComponent Object Reference") (OtherBodyIndex :type Integer))
  (if (`ActorComponent.ComponentHasTag` OtherComp "PlayerCapsule")
    (set `self.Active` false)))

(fn `UserConstructionScript`)