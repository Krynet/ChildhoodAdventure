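; Destructible spawner actor that launches homing projectiles on a repeating five-second delay, starting at BeginPlay.
; Each projectile spawns at the actor's location along the Arrow component's rotation and receives a reference back to its spawner.
; The spawn event re-triggers itself to keep the cycle running.
; Take_Damage decrements a life counter initialized from MaxLife and destroys the spawner shortly after it hits zero.
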(event `Spawn_Projectile`
  (`KismetSystemLibrary.Delay` 5.0 :!label _label)
  (bind _returnvalue (`|SpawnActorFromClass` "/Game/Léo/Blueprint/LD_Homing_Projectiles/LD_Homing_Projectiles.LD_Homing_Projectiles_C" (`KismetMathLibrary.MakeTransform` (`self.K2_GetActorLocation`) (`SceneComponent.K2_GetComponentRotation` (`self.Arrow`))) "Undefined" "OverrideRootScale" null null))
  (set `/Game/Léo/Blueprint/LD_Homing_Projectiles/LD_Homing_Projectiles.Spawner_Homing_Projectile` self _returnvalue)
  (`self.Spawn_Projectile`))

(event `self.ReceiveBeginPlay`
  (`|ExecutionSequence`
    (:`then_0`
      (goto _label))
    (:`then_1`
      (set `self.Current_Life` (`self.Max_Life`)))))

(event `Take_Damage`
  (bind _result (`/Engine/EditorBlueprintResources/StandardMacros.DecrementFloat` (`self.Current_Life`))
    (:`  `
      (if (== _result 0.0)
        (`KismetSystemLibrary.Delay` 0.01)
        (`self.K2_DestroyActor`)))))

(fn `UserConstructionScript`)