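; FirstBoss is a transition actor that plays the pre-boss cinematic and then spawns the phase 1 boss at its own transform.
; On BeginPlay it disables player input and plays the level sequence, using a GameInstance flag to skip it once it has been launched.
; When the sequence finishes or is skipped, it unhides itself, restores input, spawns Boss_Phase_1_BP, starts a camera fade and destroys the LalzVReBossPhase1 actor after a short delay.
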(event `self.ReceiveBeginPlay`
  (bind _asmaxence_game_instance (cast `/Game/Maxence/MaxenceGameInstance` (`GameplayStatics.GetGameInstance`)))
  (if (`/Game/Maxence/MaxenceGameInstance.IsCinéPréBosslaunched?` _asmaxence_game_instance)
    (`self.OnFinished_Event_0`)
    (else
      (`self.DisableInput` (`GameplayStatics.GetPlayerCharacter` 0) null)
      (bind (_outactor _returnvalue) (`LevelSequencePlayer.CreateLevelSequencePlayer` "/Game/Lalo/Sequencers/Ciné_PréBoss.Ciné_PréBoss" (make `MovieSceneSequencePlaybackSettings` false (make `MovieSceneSequenceLoopCount` 0))))
      (`MovieSceneSequencePlayer.Play` _returnvalue)
      (set `/Game/Maxence/MaxenceGameInstance.IsCinéPréBosslaunched?` true _asmaxence_game_instance)
      (add `MovieSceneSequencePlayer.OnFinished` _returnvalue (delegate `OnFinished_Event_0`)))))

(event `LaunchBoss1`)

(event `OnFinished_Event_0`
  (`self.SetActorHiddenInGame` false)
  (`self.EnableInput` (`GameplayStatics.GetPlayerCharacter` 0) null)
  (`|SpawnActorFromClass` "/Game/Léo/Blueprint/Boss/Boss_Phase_1/BOSS_BP/Boss_Phase_1_BP.Boss_Phase_1_BP_C" (`KismetMathLibrary.MakeTransform` (`self.K2_GetActorLocation`) (`self.K2_GetActorRotation`)) "Undefined" "OverrideRootScale" null null)
  (`PlayerCameraManager.StartCameraFade` :`self` (`GameplayStatics.GetPlayerCameraManager` 0) :`FromAlpha` 1.0 :`Duration` 1.0)
  (`KismetSystemLibrary.Delay` 0.2)
  (bind _returnvalue (`GameplayStatics.GetActorOfClass` "/Game/Lalo/LalzVReBossPhase1.LalzVReBossPhase1_C"))
  (`self.K2_DestroyActor` _returnvalue))

(fn `UserConstructionScript`)