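; Boss transition Blueprint that plays a cinematic and then hands the player off to the second boss respawn.
; LaunchTransition hides the player character, fades the camera out and, after a matching delay, creates and plays the CinéTransiBoss Level Sequence.
; The sequence's OnFinished callback finds the Respawn_To_Boss_2 actor by class and calls its Respawn.
; The Blueprint itself neither unhides the character nor fades the camera back in.
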(event `LaunchTransition`
  (`|ExecutionSequence`
    (:`then_0`
      (`self.SetActorHiddenInGame` (`GameplayStatics.GetPlayerCharacter` 0) true))
    (:`then_1`
      (`PlayerCameraManager.StartCameraFade` :`self` (`GameplayStatics.GetPlayerCameraManager` 0) :`ToAlpha` 1.0 :`Duration` 1.0)
      (`KismetSystemLibrary.Delay` 1.0)
      (bind (_outactor _returnvalue) (`LevelSequencePlayer.CreateLevelSequencePlayer` "/Game/Lalo/Sequencers/CinéTransiBoss.CinéTransiBoss"))
      (`MovieSceneSequencePlayer.Play` _returnvalue)
      (add `MovieSceneSequencePlayer.OnFinished` _returnvalue (delegate `OnFinished`)))))

(event `OnFinished`
  (bind _returnvalue (`GameplayStatics.GetActorOfClass` "/Game/Léo/Blueprint/Spawner/SpawnerToBoss2/Respawn_To_Boss_2.Respawn_To_Boss_2_C"))
  (`/Game/Léo/Blueprint/Spawner/SpawnerToBoss2/Respawn_To_Boss_2.Respawn` _returnvalue))

(fn `UserConstructionScript`)