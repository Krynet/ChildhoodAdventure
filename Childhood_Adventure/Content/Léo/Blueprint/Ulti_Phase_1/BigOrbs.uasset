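; BigOrbs is a large eye orb, apparently for an ultimate's first phase, that fades in, releases EyesDown actors and removes itself.
; A timeline drives the appear material, then the orb gathers world locations of tagged sphere components and spawns an EyesDown aimed at each, passing it as NextPosition.
; After a delay, a reversed timeline plays the material out and destroys the orb.
; Once spawned, Tick keeps the Arrow facing the player.
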(event `self.ReceiveBeginPlay`
  (bind _returnvalue (`self.K2_GetActorLocation`))
  (bind _asthird_person_character (cast `/Game/ThirdPersonBP/Blueprints/ThirdPersonCharacter` (`GameplayStatics.GetPlayerCharacter` 0)))
  (set `self.Character` _asthird_person_character)
  (`PrimitiveComponent.SetMaterial` (`self.Sphere`) 0 (`self.Appear_Eyes`))
  (bind (_direction _newtrack_0) (`Timeline|Timeline_0` :!via `PlayFromStart`)
    (:`Update`
      (`MeshComponent.SetScalarParameterValueOnMaterials` (`self.Sphere`) (`self.Parameter Name`) _newtrack_0))
    (:`Finished`
      (set `self.Spawned` true)
      (for _array_element (`self.GetComponentsByTag` "/Script/Engine.SphereComponent" "Location_Big_Eye")
        (`KismetArrayLibrary.Array_Add` (`self.Locations`) (`SceneComponent.K2_GetComponentLocation` _array_element)))
      (bind _result (`/Engine/EditorBlueprintResources/StandardMacros.DecrementInt` (`KismetArrayLibrary.Array_Length` (`self.Locations`)))
        (:`  `
          (for _index (range (+ _result 1))
            (bind _output (`|GetArrayItem` (`self.Locations`) _index))
            (bind _returnvalue_2 (`|SpawnActorFromClass` "/Game/Léo/Blueprint/Ulti_Phase_1/EyesDown.EyesDown_C" (`KismetMathLibrary.MakeTransform` _returnvalue (`KismetMathLibrary.FindLookAtRotation` _returnvalue _output)) "AlwaysSpawn" "OverrideRootScale" null null))
            (set `/Game/Léo/Blueprint/Ulti_Phase_1/EyesDown.NextPosition` _output _returnvalue_2)
            (`KismetSystemLibrary.Delay` 5.0)
            (bind (_direction_2 _newtrack_0_2) (`Timeline|Timeline_1` :!via `ReverseFromEnd`)
              (:`Update`
                (`MeshComponent.SetScalarParameterValueOnMaterials` (`self.Sphere`) (`self.Parameter Name`) _newtrack_0_2))
              (:`Finished`
                (`self.K2_DestroyActor`)))))))))

(event `self.ReceiveTick`
  (params (DeltaSeconds :type "Float (single-precision)"))
  (if (`self.Spawned`)
    (`SceneComponent.K2_SetWorldRotation` (`self.Arrow`) (`KismetMathLibrary.FindLookAtRotation` (`SceneComponent.K2_GetComponentLocation` (`self.Arrow`)) (`self.K2_GetActorLocation` (`self.Character`))) false false)))

(fn `UserConstructionScript`)