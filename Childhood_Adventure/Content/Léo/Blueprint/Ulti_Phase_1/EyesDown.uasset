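; EyesDown is an ultimate phase-one attack actor that moves into position and fires lasers, marking the ground below with AOEs.
; Timelines lerp it to NextPosition, then to a fixed rotation, before starting FireEvent.
; Each volley waits randomly, spawns a charge effect and an AOE at the downward trace hit, then launches a laser projectile.
; FireEvent calls itself for three volleys, then destroys the actor.
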(event `self.ReceiveBeginPlay`
  (`|ExecutionSequence`
    (:`then_0`
      (set `self.WorldPosition` (`self.K2_GetActorLocation`))
      (set `self.WorldRotation` (`self.K2_GetActorRotation`))
      (bind (_direction _newtrack_0) (`Timeline|Actor Move To`)
        (:`Update`
          (`self.K2_SetActorLocation` (`KismetMathLibrary.VLerp` (`self.WorldPosition`) (`self.NextPosition`) _newtrack_0)))
        (:`Finished`
          (`KismetSystemLibrary.Delay` 0.5)
          (bind (_direction_2 _newtrack_0_2) (`Timeline|Actor Rotate To`)
            (:`Update`
              (`self.K2_SetActorRotation` (`KismetMathLibrary.RLerp` (`self.WorldRotation`) (struct :`Pitch` -90.0) _newtrack_0_2)))
            (:`Finished`
              (`self.FireEvent`))))))))

(event `FireEvent`
  (bind _sphere3 (`self.Sphere3`))
  (`/Engine/EditorBlueprintResources/StandardMacros.IncrementInt` (`self.FireCount`)
    (:`  `
      (if (== (`self.FireCount`) 4)
        (`KismetSystemLibrary.Delay` 2.0)
        (`self.K2_DestroyActor`)
        (else
          (`KismetSystemLibrary.Delay` (`KismetMathLibrary.RandomFloatInRange` 0.0 3.0))
          (bind _returnvalue (`|SpawnActorFromClass` "/Game/Léo/Blueprint/Ulti_Phase_1/Charge_Projectile_Ulti.Charge_Projectile_Ulti_C" (`KismetMathLibrary.MakeTransform` (`SceneComponent.K2_GetComponentLocation` (`self.Sphere3`)) (`SceneComponent.K2_GetComponentRotation` (`self.Arrow`))) "Undefined" "OverrideRootScale" null null))
          (`self.K2_AttachToComponent` _returnvalue null "None" "SnapToTarget" "SnapToTarget" "KeepWorld" true)
          (bind _outhit (`KismetSystemLibrary.LineTraceSingle` (`self.K2_GetActorLocation`) (`KismetMathLibrary.MakeVector` (.x (`self.K2_GetActorLocation`)) (.y (`self.K2_GetActorLocation`)) -1000.0) "TraceTypeQuery1"))
          (`|SpawnActorFromClass` "/Game/Léo/Blueprint/Ulti_Phase_1/AOE.AOE_C" (`KismetMathLibrary.MakeTransform` (`.Location` (`GameplayStatics.BreakHitResult` _outhit))) "Undefined" "OverrideRootScale" null null)
          (`KismetSystemLibrary.Delay` 3.0)
          (`|SpawnActorFromClass` "/Game/Léo/Blueprint/LaserProjectiles/LaserProjectiles_ulti_BP.LaserProjectiles_ulti_BP_C" (`KismetMathLibrary.MakeTransform` (`SceneComponent.K2_GetComponentLocation` _sphere3) (`SceneComponent.K2_GetComponentRotation` _sphere3) (1.4 1.4 1.4)) "Undefined" "OverrideRootScale" null null)
          (`self.FireEvent`))))))

(fn `UserConstructionScript`)