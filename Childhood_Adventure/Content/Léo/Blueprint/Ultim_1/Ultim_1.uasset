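; Ultim_1 is a self-destroying actor that creates a spinning laser attack from 18 LaserEyes actors.
; On BeginPlay it spawns one LaserEyes per sphere component and snaps it to that sphere.
; Two parallel timelines rotate the Horaire and AntiHoraire components in opposite yaw directions through lerps toward two-turn offsets.
; When the counter-clockwise timeline finishes, delayed steps hide and despawn the lasers, then destroy them and the actor.
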(event `self.ReceiveBeginPlay`
  (bind _horaire_rotation_init (`self.Horaire_Rotation_Init`))
  (bind _anti_horaire_rotation_init (`self.Anti_Horaire_Rotation_Init`))
  (set `self.Horaire_Rotation_Init` (`SceneComponent.RelativeRotation` (`self.Horaire`)))
  (set `self.Anti_Horaire_Rotation_Init` (`SceneComponent.RelativeRotation` (`self.Anti_Horaire`)))
  (set `self.Arrow_List` (`|MakeArray` (`self.Arrow1`) (`self.Arrow2`) (`self.Arrow3`) (`self.Arrow4`) (`self.Arrow5`) (`self.Arrow6`) (`self.Arrow7`) (`self.Arrow8`) (`self.Arrow9`) (`self.Arrow10`) (`self.Arrow11`) (`self.Arrow12`) (`self.Arrow13`) (`self.Arrow14`) (`self.Arrow15`) (`self.Arrow16`) (`self.Arrow17`) (`self.Arrow18`)))
  (bind _output_get (set `self.Get_Sphere_List` (`|MakeArray` (`self.Sphere1`) (`self.Sphere2`) (`self.Sphere3`) (`self.Sphere4`) (`self.Sphere5`) (`self.Sphere6`) (`self.Sphere7`) (`self.Sphere8`) (`self.Sphere9`) (`self.Sphere10`) (`self.Sphere11`) (`self.Sphere12`) (`self.Sphere13`) (`self.Sphere14`) (`self.Sphere15`) (`self.Sphere16`) (`self.Sphere17`) (`self.Sphere18`))))
  (for _array_element _output_get
    (`KismetArrayLibrary.Array_Add` (`self.Get_Sphere_List_Location`) (`SceneComponent.RelativeLocation` _array_element)))
  (for _array_element_2 (`self.Arrow_List`)
    (`KismetArrayLibrary.Array_Add` (`self.Get_Arrow_List_Rotation`) (`SceneComponent.RelativeRotation` _array_element_2)))
  (for (_array_element_3 _array_index) (`self.Get_Sphere_List`)
    (bind _returnvalue (`|SpawnActorFromClass` "/Game/Léo/Blueprint/LaserBeam/LaserEyes.LaserEyes_C" (`KismetMathLibrary.MakeTransform` (`|GetArrayItem` (`self.Get_Sphere_List_Location`) _array_index) (`SceneComponent.RelativeRotation` (`self.Arrow2`)) (0.2 0.2 0.2)) "Undefined" "OverrideRootScale" null null))
    (`KismetArrayLibrary.Array_Add` (`self.Get_Laser_Eyes_List`) _returnvalue)
    (`self.K2_AttachToComponent` _returnvalue _array_element_3 "None" "SnapToTarget" "SnapToTarget" "KeepWorld" true))
  (`|ExecutionSequence`
    (:`then_0`
      (bind (_direction _newtrack_0) (`Timeline|Horaire_Timeline` :!via `PlayFromStart`)
        (:`Update`
          (`SceneComponent.K2_SetRelativeRotation` (`self.Horaire`) (`KismetMathLibrary.RLerp` _horaire_rotation_init (`KismetMathLibrary.MakeRotator` (.roll _horaire_rotation_init) (.pitch _horaire_rotation_init) (+ (.yaw _horaire_rotation_init) 720.0)) _newtrack_0) false false))))
    (:`then_1`
      (bind (_direction_2 _newtrack_0_2) (`Timeline|Anti_Horaire_Timeline` :!via `PlayFromStart`)
        (:`Update`
          (`SceneComponent.K2_SetRelativeRotation` (`self.Anti_Horaire`) (`KismetMathLibrary.RLerp` _anti_horaire_rotation_init (`KismetMathLibrary.MakeRotator` (.roll _anti_horaire_rotation_init) (.pitch _anti_horaire_rotation_init) (+ (.yaw _anti_horaire_rotation_init) -720.0)) _newtrack_0_2) false false))
        (:`Finished`
          (`KismetSystemLibrary.Delay` 2.0)
          (for _array_element_4 (`self.Get_Laser_Eyes_List`)
            (`self.SetActorHiddenInGame` _array_element_4 true)
            (`/Game/Léo/Blueprint/LaserBeam/LaserEyes.DispawnLaser` _array_element_4))
          (`KismetSystemLibrary.Delay` 5.0)
          (for _array_element_5 (`self.Get_Laser_Eyes_List`)
            (`self.K2_DestroyActor` _array_element_5))
          (`self.K2_DestroyActor`))))))

(fn `UserConstructionScript`)