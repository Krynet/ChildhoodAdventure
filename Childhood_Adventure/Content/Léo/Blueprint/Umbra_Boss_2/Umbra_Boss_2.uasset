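; Boss actor Umbra_Boss_2 that turns to face the player after a short delay.
; On BeginPlay it finds and stores the ThirdPersonCharacter, waits briefly, then enables a look flag.
; While that flag is set, Tick snaps its full rotation toward the player's location using a look-at rotation, without interpolation.
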(event `self.ReceiveBeginPlay`
  (bind _returnvalue (`GameplayStatics.GetActorOfClass` "/Game/ThirdPersonBP/Blueprints/ThirdPersonCharacter.ThirdPersonCharacter_C"))
  (set `self.Player` _returnvalue)
  (`|ExecutionSequence`
    (:`then_0`
      (`KismetSystemLibrary.Delay` 2.0)
      (set `self.Look Player` true))))

(event `self.ReceiveTick`
  (params (DeltaSeconds :type "Float (single-precision)"))
  (if (`self.Look Player`)
    (`self.K2_SetActorRotation` (`KismetMathLibrary.FindLookAtRotation` (`self.K2_GetActorLocation`) (`self.K2_GetActorLocation` (`self.Player`))))))

(fn `UserConstructionScript`)