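; Homing projectile for the Umbra boss that flies a tagged waypoint path, then turns into an Ombra_Ten_S spawn.
; It homes through SpawnerComponent targets as its sphere overlaps tagged components, then switches to the player's PlayerTargetLow with weaker homing.
; About five seconds after launch, overlapping a SpawnUmbra tag traces down for ground, spawns the Ombra above it with yaw toward the player, and destroys the projectile.
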(event `self.ReceiveBeginPlay`
  (bind _projectilemovement (`self.ProjectileMovement`))
  (`KismetSystemLibrary.Delay` 0.1)
  (set `ProjectileMovementComponent.bIsHomingProjectile` true _projectilemovement)
  (set `ProjectileMovementComponent.HomingTargetComponent` (`|GetArrayItem` (`self.Spawner_Component`)) _projectilemovement)
  (set `ProjectileMovementComponent.HomingAccelerationMagnitude` 900.0 _projectilemovement)
  (`KismetSystemLibrary.Delay` 5.0)
  (set `self.Can_Spawn` true))

(event `self.Sphere1.OnComponentBeginOverlap`
  (params (OverlappedComponent :type "PrimitiveComponent Object Reference") (OtherActor :type "Actor Object Reference") (OtherComp :type "PrimitiveComponent Object Reference") (OtherBodyIndex :type Integer) (bFromSweep :type Boolean) (SweepResult :type "HitResult Structure (by ref)"))
  (bind _returnvalue (`self.K2_GetActorLocation`))
  (bind _projectilemovement (`self.ProjectileMovement`))
  (`|ExecutionSequence`
    (:`then_0`
      (if (`ActorComponent.ComponentHasTag` OtherComp "Target1")
        (set `ProjectileMovementComponent.HomingTargetComponent` (`|GetArrayItem` (`self.Spawner_Component`) 1) (`self.ProjectileMovement`))))
    (:`then_1`
      (if (`ActorComponent.ComponentHasTag` OtherComp "Target2")
        (set `ProjectileMovementComponent.HomingTargetComponent` (`|GetArrayItem` (`self.Spawner_Component`) 2) (`self.ProjectileMovement`))))
    (:`then_2`
      (if (`ActorComponent.ComponentHasTag` OtherComp "Target3")
        (bind _returnvalue_2 (`GameplayStatics.GetActorOfClass` "/Game/ThirdPersonBP/Blueprints/ThirdPersonCharacter.ThirdPersonCharacter_C"))
        (set `ProjectileMovementComponent.HomingTargetComponent` (`/Game/ThirdPersonBP/Blueprints/ThirdPersonCharacter.PlayerTargetLow` _returnvalue_2) _projectilemovement)
        (set `ProjectileMovementComponent.HomingAccelerationMagnitude` 150.0 _projectilemovement)))
    (:`then_3`
      (if (`ActorComponent.ComponentHasTag` OtherComp "SpawnUmbra")
        (if (`self.Can_Spawn`)
          (bind _outhit (`KismetSystemLibrary.LineTraceSingle` _returnvalue (- _returnvalue (0.0 0.0 200.0)) "TraceTypeQuery1" false (`|MakeArray` _returnvalue_2 :!type "Actor Object Reference") "ForDuration"))
          (bind (_bblockinghit _binitialoverlap _time _distance _location _impactpoint _normal _impactnormal _physmat _hitactor _hitcomponent _hitbonename _hititem _faceindex _tracestart _traceend) (`GameplayStatics.BreakHitResult` _outhit))
          (bind (_returnvalue_roll _returnvalue_pitch _returnvalue_yaw) (`KismetMathLibrary.BreakRotator` (`KismetMathLibrary.FindLookAtRotation` (`self.K2_GetActorLocation`) (`self.K2_GetActorLocation` _returnvalue_2))))
          (`|SpawnActorFromClass` "/Game/Maxence/Ombras/Ombra_Ten_S.Ombra_Ten_S_C" (`KismetMathLibrary.MakeTransform` (+ (`KismetMathLibrary.SelectVector` _impactpoint _traceend (`KismetSystemLibrary.IsValid` _hitcomponent)) (0.0 0.0 130.0)) (`KismetMathLibrary.MakeRotator` 0.0 0.0 _returnvalue_yaw)) "AdjustIfPossibleButAlwaysSpawn" "OverrideRootScale" null null)
          (`self.K2_DestroyActor`))))))

(fn `UserConstructionScript`)