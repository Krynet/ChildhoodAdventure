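; Destructible wall actor that redirects bomber counter projectiles toward a target.
; When a component tagged Eyes_Bomber enters its sphere, it casts the owning actor to Bomber_Projectiles_Counter_BP and sets homing on its Target.
; Life starts at LifeMax and drops with each Deal_Damage call; once depleted, the wall hides, then destroys itself after a short delay.
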(event `self.ReceiveBeginPlay`
  (set `self.Life` (`self.Life_Max`)))

(event `Deal_Damage`
  (bind _result (`/Engine/EditorBlueprintResources/StandardMacros.DecrementFloat` (`self.Life`))
    (:`  `
      (if (<= _result 0.0)
        (`self.SetActorHiddenInGame` true)
        (`KismetSystemLibrary.Delay` 0.2)
        (`self.K2_DestroyActor`)))))

(event `self.Sphere.OnComponentBeginOverlap`
  (params (OverlappedComponent :type "PrimitiveComponent Object Reference") (OtherActor :type "Actor Object Reference") (OtherComp :type "PrimitiveComponent Object Reference") (OtherBodyIndex :type Integer) (bFromSweep :type Boolean) (SweepResult :type "HitResult Structure (by ref)"))
  (if (`ActorComponent.ComponentHasTag` OtherComp "Eyes_Bomber")
    (`KismetSystemLibrary.PrintString` "Hello")
    (bind _asbomber_projectiles_counter_bp (cast `/Game/Léo/Blueprint/EyesBombers/Bomber_Projectiles_Counter_BP` OtherActor))
    (`/Game/Léo/Blueprint/EyesBombers/Bomber_Projectiles_Counter_BP.Set_Homing` _asbomber_projectiles_counter_bp (`self.Target`))))

(fn `UserConstructionScript`)