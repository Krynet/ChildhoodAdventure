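; Breakable wall actor that attracts countered Bomber projectiles and shatters once its life runs out.
; Its Sphere detects components tagged Eyes_Bomber and sets homing on their Bomber_Projectiles_Counter_BP owner toward the wall's Target.
; Each Deal_Damage call plays a breaking sound, shakes the camera and decrements Life.
; At zero, it disables Cube collision, hides, spawns a destructible replacement with smoke FX, then destroys itself after a brief delay.
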(event `self.ReceiveBeginPlay`
  (set `self.Life` (`self.Life_Max`)))

(event `Deal_Damage`
  (bind _returnvalue (`self.K2_GetActorLocation`))
  (bind _returnvalue_2 (`self.K2_GetActorRotation`))
  (`GameplayStatics.PlaySoundAtLocation` "/Game/Sounds/LD/mur_casse_Cue.mur_casse_Cue" (`SceneComponent.K2_GetComponentLocation` (`self.Cube`)) (struct) 1.0 1.0 0.0 null null null)
  (`PlayerController.ClientStartCameraShake` :`self` (`GameplayStatics.GetPlayerController` 0) :`Shake` "/Game/Léo/Blueprint/ShakeCamera/BP_Camera_Shake.BP_Camera_Shake_C" :`Scale` 5.0)
  (bind _result (`/Engine/EditorBlueprintResources/StandardMacros.DecrementFloat` (`self.Life`))
    (:`  `
      (if (<= _result 0.0)
        (`|ExecutionSequence`
          (:`then_0`
            (`self.SetActorHiddenInGame` true)
            (`|SpawnActorFromClass` "/Game/Léo/Destructible_mesh/Destructible_Wall_3.Destructible_Wall_3_C" (`KismetMathLibrary.MakeTransform` _returnvalue _returnvalue_2) "Undefined" "OverrideRootScale" null null)
            (`|SpawnActorFromClass` "/Game/Léo/Blueprint/FX/FX_Fumée.FX_Fumée_C" (`KismetMathLibrary.MakeTransform` _returnvalue _returnvalue_2 (6.0 6.0 6.0)) "Undefined" "OverrideRootScale" null null)
            (`KismetSystemLibrary.Delay` 0.02)
            (`self.K2_DestroyActor`))
          (:`then_1`
            (`PrimitiveComponent.SetCollisionEnabled` (`self.Cube`) "NoCollision")))))))

(event `self.Sphere.OnComponentBeginOverlap`
  (params (OverlappedComponent :type "PrimitiveComponent Object Reference") (OtherActor :type "Actor Object Reference") (OtherComp :type "PrimitiveComponent Object Reference") (OtherBodyIndex :type Integer) (bFromSweep :type Boolean) (SweepResult :type "HitResult Structure (by ref)"))
  (if (`ActorComponent.ComponentHasTag` OtherComp "Eyes_Bomber")
    (bind _asbomber_projectiles_counter_bp (cast `/Game/Léo/Blueprint/EyesBombers/Bomber_Projectiles_Counter_BP` OtherActor))
    (`/Game/Léo/Blueprint/EyesBombers/Bomber_Projectiles_Counter_BP.Set_Homing` _asbomber_projectiles_counter_bp (`self.Target`))))

(fn `UserConstructionScript`)