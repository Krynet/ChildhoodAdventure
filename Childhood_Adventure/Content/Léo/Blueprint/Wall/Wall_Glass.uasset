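; Breakable glass wall actor that the player destroys by punching it.
; On begin play it sets its life to the maximum and caches the player's ThirdPersonCharacter.
; A box overlap with a component tagged PunchBox deals damage, provided that character's Punch flag is set.
; Each hit decrements life, and the actor destroys itself once life reaches zero or below.
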(event `self.ReceiveBeginPlay`
  (set `self.Life` (`self.Life_Max`))
  (bind _asthird_person_character (cast `/Game/ThirdPersonBP/Blueprints/ThirdPersonCharacter` (`GameplayStatics.GetPlayerCharacter` 0)))
  (set `self.Character` _asthird_person_character))

(event `self.Box.OnComponentBeginOverlap`
  (params (OverlappedComponent :type "PrimitiveComponent Object Reference") (OtherActor :type "Actor Object Reference") (OtherComp :type "PrimitiveComponent Object Reference") (OtherBodyIndex :type Integer) (bFromSweep :type Boolean) (SweepResult :type "HitResult Structure (by ref)"))
  (if (`ActorComponent.ComponentHasTag` OtherComp "PunchBox")
    (if (`/Game/ThirdPersonBP/Blueprints/ThirdPersonCharacter.Punch` (`self.Character`))
      (`self.Deal_Damage`))))

(event `Deal_Damage`
  (bind _result (`/Engine/EditorBlueprintResources/StandardMacros.DecrementFloat` (`self.Life`))
    (:`  `
      (if (<= _result 0.0)
        (`self.K2_DestroyActor`)))))

(fn `UserConstructionScript`)