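; Punchable wall actor that breaks after taking enough hits from the player's punch.
; Box overlaps with a "PunchBox"-tagged component deal damage while the ThirdPersonCharacter, found by class lookup, has Punch set.
; Each hit decrements Life, which starts at LifeMax.
; At zero it hides, disables Cube collision, spawns Destructible_Wall_2 in its place and destroys itself after a brief delay.
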(event `self.ReceiveBeginPlay`
  (set `self.Life` (`self.Life_Max`)))

(event `Deal_Damage`
  (bind _result (`/Engine/EditorBlueprintResources/StandardMacros.DecrementFloat` (`self.Life`))
    (:`  `
      (if (<= _result 0.0)
        (`|ExecutionSequence`
          (:`then_0`
            (`self.SetActorHiddenInGame` true)
            (`|SpawnActorFromClass` "/Game/Léo/Destructible_mesh/Destructible_Wall_2.Destructible_Wall_2_C" (`KismetMathLibrary.MakeTransform` (`self.K2_GetActorLocation`) (`self.K2_GetActorRotation`)) "Undefined" "OverrideRootScale" null null)
            (`KismetSystemLibrary.Delay` 0.02)
            (`self.K2_DestroyActor`))
          (:`then_1`
            (`PrimitiveComponent.SetCollisionEnabled` (`self.Cube`) "NoCollision")))))))

(event `self.Box.OnComponentBeginOverlap`
  (params (OverlappedComponent :type "PrimitiveComponent Object Reference") (OtherActor :type "Actor Object Reference") (OtherComp :type "PrimitiveComponent Object Reference") (OtherBodyIndex :type Integer) (bFromSweep :type Boolean) (SweepResult :type "HitResult Structure (by ref)"))
  (if (`ActorComponent.ComponentHasTag` OtherComp "PunchBox")
    (bind _returnvalue (`GameplayStatics.GetActorOfClass` "/Game/ThirdPersonBP/Blueprints/ThirdPersonCharacter.ThirdPersonCharacter_C"))
    (if (`/Game/ThirdPersonBP/Blueprints/ThirdPersonCharacter.Punch` _returnvalue)
      (`self.Deal_Damage`))))

(fn `UserConstructionScript`)