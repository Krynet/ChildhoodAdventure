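; Ground piece, apparently for a boss fight, that swaps itself for a destructible classroom floor once activated.
; ActivateGround arms it, and Tick checks that flag along with whether time accumulated since play began, not since activation, exceeds Delay.
; It then hides, disables the cube's collision, spawns Destructible_Classroom_Ground at its transform and destroys itself shortly after.
; The overlap handler is empty, and older physics and destroyer-zone logic is disconnected.
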(event `self.ReceiveBeginPlay`
  ;[1 1 1] aaah
  (if (and (> (stale `self.ReceiveTick` _output_get) (`self.Delay`)) (`self.Set_Active`)) :!label _label
    (`/Engine/EditorBlueprintResources/StandardMacros.DoOnce` false
      (:`Completed`
        (`|ExecutionSequence`
          (:`then_0`
            (`self.SetActorHiddenInGame` true)
            (`|SpawnActorFromClass` "/Game/Matteo/LD_Meshes/DestructiblesMeshes/Destructible_Classroom_Ground.Destructible_Classroom_Ground_C" (`KismetMathLibrary.MakeTransform` (`self.K2_GetActorLocation`) (`self.K2_GetActorRotation`)) "Undefined" "OverrideRootScale" null null)
            (`KismetSystemLibrary.Delay` 0.02)
            (`self.K2_DestroyActor`))
          (:`then_1`
            (`PrimitiveComponent.SetCollisionEnabled` (`self.Cube`) "NoCollision")))))))

(event `self.ReceiveTick`
  (params (DeltaSeconds :type "Float (single-precision)"))
  (bind _output_get (set `self.temp` (+ (`self.temp`) DeltaSeconds)))
  (goto _label))

(event `ActivateGround`
  (`/Engine/EditorBlueprintResources/StandardMacros.DoOnce` false
    (:`Completed`
      (set `self.Set_Active` true))))

(event `self.Box.OnComponentBeginOverlap`
  (params (OverlappedComponent :type "PrimitiveComponent Object Reference") (OtherActor :type "Actor Object Reference") (OtherComp :type "PrimitiveComponent Object Reference") (OtherBodyIndex :type Integer) (bFromSweep :type Boolean) (SweepResult :type "HitResult Structure (by ref)")))

(fn `UserConstructionScript`)