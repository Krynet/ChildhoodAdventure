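; Double gate actor that swings its two leaves open when a component tagged PlayerHit enters its trigger box.
; BeginPlay caches each leaf's world rotation, and the overlap restarts a timeline that lerps both a quarter turn in opposite yaw directions.
; No closing logic runs.
; An interact-prompt widget and a FlipFlop open/close toggle remain as disconnected logic, and OpenGate is an empty event.
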(event `Key|E`
  (params (Key :type "Key Structure")))

(event `OpenGate`)

(event `self.ReceiveTick`
  (params (DeltaSeconds :type "Float (single-precision)")))

(event `self.ReceiveBeginPlay`
  (set `self.InitRotationLeft` (`SceneComponent.K2_GetComponentRotation` (`self.lp`)))
  (set `self.InitRotationRight` (`SceneComponent.K2_GetComponentRotation` (`self.rp`))))

(event `self.Box.OnComponentBeginOverlap`
  (params (OverlappedComponent :type "PrimitiveComponent Object Reference") (OtherActor :type "Actor Object Reference") (OtherComp :type "PrimitiveComponent Object Reference") (OtherBodyIndex :type Integer) (bFromSweep :type Boolean) (SweepResult :type "HitResult Structure (by ref)"))
  (bind _initrotationleft (`self.InitRotationLeft`))
  (bind _initrotationright (`self.InitRotationRight`))
  (if (`ActorComponent.ComponentHasTag` OtherComp "PlayerHit")
    (bind (_direction _newtrack_0) (`Timeline|Timeline_0` :!via `PlayFromStart`)
      (:`Update`
        (`|ExecutionSequence`
          (:`then_0`
            (`SceneComponent.K2_SetWorldRotation` (`self.lp`) (`KismetMathLibrary.RLerp` _initrotationleft (`KismetMathLibrary.MakeRotator` (.roll _initrotationleft) (.pitch _initrotationleft) (+ (.yaw _initrotationleft) 90.0)) _newtrack_0) false false))
          (:`then_1`
            (`SceneComponent.K2_SetWorldRotation` (`self.rp`) (`KismetMathLibrary.RLerp` _initrotationright (`KismetMathLibrary.MakeRotator` (.roll _initrotationright) (.pitch _initrotationright) (- (.yaw _initrotationright) 90.0)) _newtrack_0) false false)))))))

(fn `UserConstructionScript`)