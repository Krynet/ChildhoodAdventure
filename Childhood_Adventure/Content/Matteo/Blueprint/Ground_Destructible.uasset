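; Destructible ground piece whose cube breaks loose and falls in a randomized way once its Physics flag is true.
; Tick polls the flag and fires a one-shot sequence that waits up to a second at random, then enables physics simulation on the cube.
; Short delayed follow-ups add a small random X/Y force and a random roll and pitch rotation to vary the fall.
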(event `self.ReceiveTick`
  (params (DeltaSeconds :type "Float (single-precision)"))
  (bind _returnvalue (`KismetMathLibrary.RandomFloatInRange` 0.0 45.0))
  (bind _returnvalue_2 (`KismetMathLibrary.RandomFloatInRange` 0.0 45.0))
  (bind _physics (`self.physics`))
  (bind _cube (`self.Cube`))
  ;[1 1 1] chute aléatoire du mesh
  (if _physics
    (`/Engine/EditorBlueprintResources/StandardMacros.DoOnce` false
      (:`Completed`
        (`KismetSystemLibrary.Delay` (`KismetMathLibrary.RandomFloatInRange` 0.0 1.0))
        (`PrimitiveComponent.SetSimulatePhysics` _cube _physics)
        (`KismetSystemLibrary.Delay` 0.3)
        (`PrimitiveComponent.AddForce` _cube (`KismetMathLibrary.MakeVector` _returnvalue _returnvalue_2) "None" false)
        (`KismetSystemLibrary.Delay` 0.3)
        (`SceneComponent.K2_AddLocalRotation` _cube (`KismetMathLibrary.MakeRotator` _returnvalue_2 _returnvalue) false false)))))

(fn `UserConstructionScript`)