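; Spawner actor that makes a Tentacle_Mat periodically appear at its own location.
; After BeginPlay and a configurable starting delay, it runs an endless delay-driven loop that spawns the tentacle, destroys it a few seconds later, then pauses before repeating.
; A single Scale variable sets both the tentacle's size and its radial force radius.
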(event `self.ReceiveBeginPlay`
  (bind _scale (`self.Scale`))
  (`KismetSystemLibrary.Delay` (+ (`self.StartingDelay`) 0.1))
  (bind _returnvalue (`|SpawnActorFromClass` "/Game/Matteo/Blueprint/Tentacle_Mat.Tentacle_Mat_C" (`KismetMathLibrary.MakeTransform` (`self.K2_GetActorLocation`) (`KismetMathLibrary.MakeRotator` 0.0) (`KismetMathLibrary.MakeVector` _scale _scale _scale)) "AlwaysSpawn" "OverrideRootScale" null null :!label _label))
  (set `RadialForceComponent.Radius` (* 100 _scale) (`/Game/Matteo/Blueprint/Tentacle_Mat.RadialForce` _returnvalue))
  (`KismetSystemLibrary.Delay` 3.0)
  (`self.K2_DestroyActor` _returnvalue)
  (`KismetSystemLibrary.Delay` 4.0)
  (goto _label))

(fn `UserConstructionScript`)