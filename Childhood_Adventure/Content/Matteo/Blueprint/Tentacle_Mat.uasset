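; Tentacle enemy that turns to face the player and loses Life when countered, destroying itself with a sound at zero.
; A trigger sphere gates the smoothed Tick look-at rotation, and a closer push trigger fires a delayed radial impulse.
; Damage comes from the Attacked event or CounterBox overlaps while the player's CanRedHit is set.
; The Shoot event is empty, leaving the laser bullet spawn disconnected.
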(event `self.CapsuleComponent.OnComponentBeginOverlap`
  (params (OverlappedComponent :type "PrimitiveComponent Object Reference") (OtherActor :type "Actor Object Reference") (OtherComp :type "PrimitiveComponent Object Reference") (OtherBodyIndex :type Integer) (bFromSweep :type Boolean) (SweepResult :type "HitResult Structure (by ref)"))
  ;[0 0 0] Détection de la tentacule par rapport au Player et appel de l'attaque du Player
  (if (`ActorComponent.ComponentHasTag` OtherComp "CounterBox")
    (bind _returnvalue (`GameplayStatics.GetActorOfClass` "/Game/Alexandre/Blueprint/ThirdPersonCharacter_Alexandre_BP.ThirdPersonCharacter_Alexandre_BP_C"))
    (if (`/Game/Alexandre/Blueprint/ThirdPersonCharacter_Alexandre_BP.CanRedHit` _returnvalue)
      (`self.Receive Damage` :!label _label))))

(event `Attacked`
  ;[0 0 0] Détection de la tentacule par rapport au Player et appel de l'attaque du Player
  (goto _label))

(event `self.ReceiveTick`
  (params (DeltaSeconds :type "Float (single-precision)"))
  ;[0 0 0] Rotation de la tentacule par rapport au Player
  (if (`self.CanRotate`)
    (bind _returnvalue (`GameplayStatics.GetActorOfClass` "/Game/ThirdPersonBP/Blueprints/ThirdPersonCharacter.ThirdPersonCharacter_C"))
    (bind _output_get (set `self.Rotation` (`KismetMathLibrary.FindLookAtRotation` (`self.K2_GetActorLocation`) (`SceneComponent.K2_GetComponentLocation` (`Actor.RootComponent` _returnvalue)))))
    (`self.K2_SetActorRotation` (`KismetMathLibrary.RLerp` (`self.K2_GetActorRotation`) (`KismetMathLibrary.MakeRotator` (.roll _output_get) 0.0 (.yaw _output_get)) (* DeltaSeconds 10.0)))))

(event `Shoot`
  ;[0 0 0] Tir à distance de l'ennemi
)

(event `self.TriggerSphere.OnComponentBeginOverlap`
  (params (OverlappedComponent :type "PrimitiveComponent Object Reference") (OtherActor :type "Actor Object Reference") (OtherComp :type "PrimitiveComponent Object Reference") (OtherBodyIndex :type Integer) (bFromSweep :type Boolean) (SweepResult :type "HitResult Structure (by ref)"))
  ;[0 0 0] Rotation par rapport à la position du joueur
  (if (`ActorComponent.ComponentHasTag` OtherComp "PlayerCapsule")
    (set `self.CanRotate` true)))

(event `self.TriggerSphere.OnComponentEndOverlap`
  (params (OverlappedComponent :type "PrimitiveComponent Object Reference") (OtherActor :type "Actor Object Reference") (OtherComp :type "PrimitiveComponent Object Reference") (OtherBodyIndex :type Integer))
  ;[0 0 0] Rotation par rapport à la position du joueur
  (if (`ActorComponent.ComponentHasTag` OtherComp "PlayerCapsule")
    (set `self.CanRotate` false)))

(event `self.TriggerPush.OnComponentBeginOverlap`
  (params (OverlappedComponent :type "PrimitiveComponent Object Reference") (OtherActor :type "Actor Object Reference") (OtherComp :type "PrimitiveComponent Object Reference") (OtherBodyIndex :type Integer) (bFromSweep :type Boolean) (SweepResult :type "HitResult Structure (by ref)"))
  ;[0 0 0] Bump du joueur si il est trop près de l'ennemi
  (if (`ActorComponent.ComponentHasTag` OtherComp "PlayerCapsule")
    (`KismetSystemLibrary.Delay` 0.1)
    (`RadialForceComponent.FireImpulse` (`self.RadialForce`))
    (`KismetSystemLibrary.PrintString` "Hello")))

(fn `UserConstructionScript`)